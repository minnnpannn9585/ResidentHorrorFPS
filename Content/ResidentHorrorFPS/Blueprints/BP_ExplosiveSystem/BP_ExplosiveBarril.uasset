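; Explosive barrel actor that blows up when hit by damage, hides its mesh, destroys itself after a delay and saves that state for loading.
; Explode triggers the explosive component and sphere-traces the radius to hurt the player, break wooden boxes, and damage AI enemies with hit montages before resuming their strafing.
; Nearby barrels get SelfExplode, which detonates them without their own trace or save, so area effects do not chain.
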(event LoadedData(BP_SaveLoadRHFps)
  (params (Save%20Loaded%20Data :type ST%20Save%20Load%20Structure))
  ;[0 0 0 0.5] Load
  (if (Utilities|Struct|BreakST_SaveLoad Save%20Loaded%20Data)
    (Actor|DestroyActor)))

(event Custom|Explode
  (bind _returnvalue (Transformation|GetActorLocation))
  (bind _barril_mesh (Variables|Default|GetBarril%20Mesh))
  (bind _hit_montage_ia_enemy (Variables|Default|GetHit%20Montage%20IA%20Enemy))
  ;[0 0 0 0.5] Explode Barril
  (Utilities|FlowControl|Sequence
    (:then_0
      (Collision|SetCollisionEnabled _barril_mesh "NoCollision")
      (Collision|SetCollisionResponsetoAllChannels _barril_mesh "ECR_Ignore")
      (Development|SetHiddeninGame (Variables|Default|GetBarril%20Mesh) true false)
      (Utilities|FlowControl|Delay 5.0)
      (Actor|DestroyActor))
    (:then_1
      (Collision|SetCollisionResponsetoAllChannels (Variables|Default|GetBarril%20Mesh) "ECR_Ignore")
      (Default|SaveData (Variables|Default|GetBP_SaveLoadRHFps) (Utilities|Struct|MakeST_SaveLoad true))
      (Variables|Default|SetOff? true)
      (Default|Explode (Variables|Default|GetExplosiveComponet))
      (bind _outhits (Collision|MultiSphereTraceForObjects _returnvalue _returnvalue (Variables|Default|GetRadius%20Explose) (Utilities|Array|MakeArray "ObjectTypeQuery3" "ObjectTypeQuery1") false 0 (Variables|Default|GetDraw%20Debug%20Type)))
      (bind _array_element (Utilities|Array|ForEachLoopwithBreak _outhits)
        (:LoopBody
          (bind _asbp_explosive_barril (Utilities|Casting|CastToBP_ExplosiveBarril (.HitActor (Collision|BreakHitResult _array_element)))
            (:then
              (CallFunction|SelfExplode _asbp_explosive_barril))
            (:CastFailed
              _))
          (bind _asbp_box_wood_broken (Utilities|Casting|CastToBP_BoxWood_Broken (.HitActor (Collision|BreakHitResult _array_element)))
            (:then
              (Default|BoxBroken _asbp_box_wood_broken))
            (:CastFailed
              _))
          (if (== (.HitActor (Collision|BreakHitResult _array_element)) (CallFunction|RHVFPSPlayerRef))
            (Default|TakeDamage (Variables|/Game/ResidentHorrorFPS/Character/BP_Character/BP_RHV_FPS_Player.BP_RHV_FPS_Player_C|GetHealthComponent (CallFunction|RHVFPSPlayerRef)) (Variables|Default|Get%20Damage%20In%20Player)))
          (bind _aienemy (Class|BPIIA|ReceiveAIEnemy(Message) (.HitActor (Collision|BreakHitResult _array_element))))
          (bind _output_get (Variables|Default|SetAi%20Enemy _aienemy))
          (Utilities|IsValid _output_get
            (:Is%20Valid
              (Variables|Default|SetOff? true)
              (Class|BPIMasterIAEnemy|BPIDamage(Message) :self _output_get :DamageCauser (.HitActor (Collision|BreakHitResult _array_element)) :Base%20Damage (Variables|Default|GetDamage%20Explose) :ForceHeavyHit true)
              (Animation|Montage|PlayMontage (Variables|/Script/Engine.Character|GetMesh _output_get) (Utilities|Array|Get(acopy) _hit_montage_ia_enemy (Math|Random|RandomIntegerinRange 0 (- (Utilities|Array|Length _hit_montage_ia_enemy) 1)))
                (:OnCompleted
                  _)
                (:OnNotifyBegin
                  _))
              (Utilities|IsValid _output_get
                (:Is%20Valid
                  (bind _currentstrafetask (Variables|/Game/ResidentHorrorFPS/Blueprints/BP_MasterAI/Enemy/MasterAIBase/BP_AIMaster.BP_AIMaster_C|GetCurrentStrafeTask _output_get)
                    (:then
                      (Default|ContinueStrafing _currentstrafetask))
                    (:else)))))))))))

(event Custom|Break
  (bind _hit_montage_ia_enemy (Variables|Default|GetHit%20Montage%20IA%20Enemy))
  ;[0 0 0 0.5] Explode Barril
  (Utilities|Array|ForEachLoopwithBreak (stale Custom|Explode _outhits)) ; enters at Break
)

(event Custom|Self%20Explode
  (bind _barril_mesh (Variables|Default|GetBarril%20Mesh))
  ;[0.15 0.15 0.15 0.5] Self Explode
  (Collision|SetCollisionEnabled _barril_mesh "NoCollision")
  (Collision|SetCollisionResponsetoAllChannels _barril_mesh "ECR_Ignore")
  (Development|SetHiddeninGame (Variables|Default|GetBarril%20Mesh) true false)
  (Default|Explode (Variables|Default|GetExplosiveComponet))
  (Utilities|FlowControl|Delay 5.0)
  (Actor|DestroyActor))

(event EventEventDamageRHFPS
  (params (Damage :type Float%20%28double-precision%29) (Hitresult :type Hit%20Result%20Structure) (Preparator :type Actor%20Object%20Reference))
  ;[0 0 0 0.5] Damage
  (if (not (Variables|Default|GetOff?))
    (if (== (.HitActor (Collision|BreakHitResult Hitresult)) self)
      (CallFunction|Explode))))

(fn ConstructionScript)