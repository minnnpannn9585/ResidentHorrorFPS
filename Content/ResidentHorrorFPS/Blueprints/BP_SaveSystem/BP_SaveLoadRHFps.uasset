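; BP_SaveLoadRHFps is a save/load helper that persists per-object data for its owner in Resident Horror FPS.
; On BeginPlay it caches its world location and the game instance, then looks up stored data keyed by that location.
; It broadcasts the loaded data, or a no-data event for a new game, missing save slot or missing entry.
; SaveData writes object data back to the game instance under the initial location.
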(event EventBeginPlay
  ;[0 0 0 0.5] Begin Play Save System
  (Variables|Default|SetInit%20Location (Transformation|GetWorldLocation))
  (CallFunction|InitGameInstance)
  (CallFunction|LoadeData))

(fn LoadeData
  (bind _returnvalue (Transformation|GetWorldLocation))
  (bind _game_instance_resident_horror (Variables|Default|GetGame%20Instance%20Resident%20Horror))
  (bind _objectsavedata (Variables|/Game/ResidentHorrorFPS/Blueprints/BP_MainMenu/GameInstanceResidentHorror.GameInstanceResidentHorror_C|GetObjectSaveData _game_instance_resident_horror))
  (bind (_value _returnvalue_2) (Utilities|Map|Find _objectsavedata _returnvalue))
  (bind _gameinstanceresidenthorror (Class|BPIGameInstance|RetrieveGameInstance(Message) (Game|GetGameInstance)))
  (if (Variables|/Game/ResidentHorrorFPS/Blueprints/BP_MainMenu/GameInstanceResidentHorror.GameInstanceResidentHorror_C|GetNewGame? _gameinstanceresidenthorror)
    (Default|CallNoLoadedData)
    (else
      (bind _returnvalue_3 (SaveGame|DoesSaveGameExist "ResidentHorrorGlobal"))
      (if _returnvalue_3
        (if _returnvalue_2
          (bind _output_get (Variables|Default|SetSt%20Stored%20data _value))
          (Default|CallLoadedData _output_get)
          (else
            (Default|CallNoLoadedData)))
        (else
          (Default|CallNoLoadedData))))))

(fn SaveData
  (params (Object%20Data :type ST%20Save%20Load%20Structure))
  (Default|SaveObjectData (Variables|Default|GetGame%20Instance%20Resident%20Horror) Object%20Data (Variables|Default|GetInit%20Location)))

(fn InitGameInstance
  (bind _gameinstanceresidenthorror (Class|BPIGameInstance|RetrieveGameInstance(Message) (Game|GetGameInstance)))
  (Variables|Default|SetGame%20Instance%20Resident%20Horror _gameinstanceresidenthorror))