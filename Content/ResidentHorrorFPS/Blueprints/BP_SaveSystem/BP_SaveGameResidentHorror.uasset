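; BP_SaveGameResidentHorror is the save data Blueprint for Resident Horror FPS, holding a snapshot of the player's inventory and equipment.
; A setter and getter pair writes and reads the snapshot as a whole: inventory entries, item information, equipment indices, current equipped index and a has-data flag.
; RegisterActorSave and SecureRescue are stubs that only return false, so no actor saving or rescue logic runs here.
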(fn SetInventorySaveSnapshot
  (params (InventorySaveEntries :type Array%20of%20ST%20Inventory%20Save%20Entry%20Structures) (InventoryItemInformation :type Array%20of%20ST%20Item%20Information%20Structures) (EquipmentItemIndices :type Array%20of%20Integers) (CurrentEquipmentItemIndex :type Integer) (HasInventorySaveData :type Boolean))
  (Variables|Default|SetInventorySaveEntries InventorySaveEntries)
  (Variables|Default|SetInventoryItemInformation InventoryItemInformation)
  (Variables|Default|SetEquipmentItemIndices EquipmentItemIndices)
  (Variables|Default|SetCurrentEquipmentItemIndex CurrentEquipmentItemIndex)
  (Variables|Default|SetHasInventorySaveData HasInventorySaveData))

(fn GetInventorySaveSnapshot
  (return (Variables|Default|GetInventorySaveEntries) (Variables|Default|GetInventoryItemInformation) (Variables|Default|GetEquipmentItemIndices) (Variables|Default|GetCurrentEquipmentItemIndex) (Variables|Default|GetHasInventorySaveData)))

(fn RegisterActorSave
  (params (ActoSave :type Actor%20Object%20Reference) (SaveName :type String))
  (return false))

(fn SecureRescue
  (params (SaveName :type String))
  (return false))