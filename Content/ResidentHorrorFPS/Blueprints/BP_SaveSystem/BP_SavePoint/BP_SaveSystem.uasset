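; BP_SaveSystem is an interactable save point that opens the in-game save menu with its own camera view and music.
; On interaction it fades out, disables player input, shows WBP_SaveIngame, blends to its CineCamera, hides the player and HUD, and starts save-room music.
; CloseCamera reverses this behind another fade, returning view and input to the player and restoring ambient music taken from the Game Instance.
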(event Custom|Initial%20Camera
  ;[0 0 0] have a camera
  (Game|Player|SetViewTargetwithBlend (Game|GetPlayerController 0) (Components|GetOwner (Variables|Default|GetCineCamera)) 0.0 "VTBlend_Cubic" 1.0 false)
  (Widget|SetVisibility (Variables|/Game/ResidentHorrorFPS/Character/BP_Character/BP_RHV_FPS_Player.BP_RHV_FPS_Player_C|GetWBP%20Main%20Hud (CallFunction|RHVFPSPlayerRef)) "Hidden"))

(event Custom|Close%20Camera
  ;[0 0 0] Close Camera
  (CameraFades|StartCameraFade :self (Game|GetPlayerCameraManager 0) :ToAlpha 1.0 :Duration 0.3 :bHoldWhenFinished true)
  (Utilities|FlowControl|Delay 0.4)
  (Game|Player|SetViewTargetwithBlend (Game|GetPlayerController 0) (Game|Player|GetPlayerPawn 0) 0.0 "VTBlend_Cubic" 0.0 false)
  (Widget|SetVisibility (Variables|/Game/ResidentHorrorFPS/Character/BP_Character/BP_RHV_FPS_Player.BP_RHV_FPS_Player_C|GetWBP%20Main%20Hud (CallFunction|RHVFPSPlayerRef)) "Visible")
  (bind _gameinstanceresidenthorror (Class|BPIGameInstance|RetrieveGameInstance(Message) (Game|GetGameInstance)))
  (Utilities|IsValid (Variables|/Game/ResidentHorrorFPS/Character/BP_Character/BP_RHV_FPS_Player.BP_RHV_FPS_Player_C|GetMusic%20manage%20ref (CallFunction|RHVFPSPlayerRef))
    (:Is%20Valid
      (Default|StartMusicAmbient (Variables|/Game/ResidentHorrorFPS/Character/BP_Character/BP_RHV_FPS_Player.BP_RHV_FPS_Player_C|GetMusic%20manage%20ref (CallFunction|RHVFPSPlayerRef)) (Variables|/Game/ResidentHorrorFPS/Blueprints/BP_MainMenu/GameInstanceResidentHorror.GameInstanceResidentHorror_C|GetAmbient%20Music _gameinstanceresidenthorror) 2.0 1.0 0.0 true)
      (Rendering|SetActorHiddenInGame (CallFunction|RHVFPSPlayerRef) false)
      (Rendering|SetVisibility (Variables|Default|GetInteractWidget) true false)
      (CameraFades|StartCameraFade :self (Game|GetPlayerCameraManager 0) :FromAlpha 1.0 :Duration 0.4)
      (Input|EnableInput (Game|Player|GetPlayerPawn 0) (Game|GetPlayerController 0)))))

(event EventBeginPlay
  (|CallParentFunction) ; This node is disabled and will not be called.\nDrag off pins to build functionality.
)

(event EventInteraction
  (params (Player :type BP%20RHV%20FPS%20Player%20Object%20Reference) (AutoInteraction%28Non-Player%29 :type Boolean))
  (bind _returnvalue (Game|GetPlayerController 0))
  (bind _player (CallFunction|RHVFPSPlayerRef))
  (bind _music_manage_ref (Variables|/Game/ResidentHorrorFPS/Character/BP_Character/BP_RHV_FPS_Player.BP_RHV_FPS_Player_C|GetMusic%20manage%20ref _player))
  ;[0 0 0 0.5] Start Interact
  (CameraFades|StartCameraFade :self (Game|GetPlayerCameraManager 0) :ToAlpha 1.0 :Duration 0.3 :bHoldWhenFinished true)
  (Input|DisableInput (Game|Player|GetPlayerPawn 0) (Game|GetPlayerController 0))
  (Utilities|FlowControl|Delay 0.4)
  (bind _returnvalue_2 (UserInterface|CreateWidget "/Game/ResidentHorrorFPS/Blueprints/BP_SaveSystem/WBP/WBP_SaveIngame.WBP_SaveIngame_C" 0 self))
  (bind _output_get (Variables|Default|SetWB%20Load%20Slots _returnvalue_2))
  (UserInterface|Viewport|AddtoViewport _output_get 0)
  (Variables|/Script/Engine.PlayerController|SetbShowMouseCursor _returnvalue true)
  (Input|SetInputModeUIOnly _returnvalue _returnvalue_2 "DoNotLock" false)
  (CallFunction|InitialCamera)
  (Utilities|IsValid _music_manage_ref
    (:Is%20Valid
      (Default|StartMusicAmbient _music_manage_ref (Variables|Default|GetMusic%20Save%20load) 0.5 0.5 0.0 false)
      (Rendering|SetVisibility (Variables|Default|GetInteractWidget) false false)
      (Rendering|SetActorHiddenInGame (CallFunction|RHVFPSPlayerRef) true)
      (CameraFades|StartCameraFade :self (Game|GetPlayerCameraManager 0) :FromAlpha 1.0 :Duration 1.0))))

(fn ConstructionScript
  (|CallParentFunction))