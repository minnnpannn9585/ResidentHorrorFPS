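; Base weapon projectile for the Resident Horror FPS weapon system that resolves its impact on hit, then destroys itself.
; Hit pushes physics-simulating components, spawns impact effects, applies damage and reports it to AI damage sensing.
; Sound, particle and fading decal come from a map keyed by physical material, with randomized scale, roll and decal frame.
; An uncalled Splatter function only runs a debug-drawn forward trace.
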(event Collision|EventHit
  (params (MyComp :type Primitive%20Component%20Object%20Reference) (Other :type Actor%20Object%20Reference) (OtherComp :type Primitive%20Component%20Object%20Reference) (bSelfMoved :type Boolean) (HitLocation :type Vector :default "0, 0, 0") (HitNormal :type Vector :default "0, 0, 0") (NormalImpulse :type Vector :default "0, 0, 0") (Hit :type Hit%20Result%20Structure%20%28by%20ref%29))
  (bind _ownerprojectile (Variables|Default|GetOwnerProjectile))
  (Variables|Default|SetHitActor Other)
  (Variables|Default|SetHitResult Hit)
  (Variables|Default|SetHitPhysMat (.PhysMat (Collision|BreakHitResult (Variables|Default|GetHitResult))))
  (Variables|Default|SetImpact%20Point (.ImpactPoint (Collision|BreakHitResult (Variables|Default|GetHitResult))))
  (Variables|Default|SetNormal (.Normal (Collision|BreakHitResult (Variables|Default|GetHitResult))))
  (Variables|Default|SetHit%20Component (.HitComponent (Collision|BreakHitResult (Variables|Default|GetHitResult))))
  (Variables|Default|SetHit%20Bone%20Name (.HitBoneName (Collision|BreakHitResult (Variables|Default|GetHitResult))))
  (CallFunction|AddPhysicImpulse)
  (CallFunction|CreateHitVSFX)
  (bind _returnvalue (Game|Damage|ApplyDamage (Variables|Default|GetHitActor) (Variables|Default|GetCurrent%20Damage) (Pawn|GetController (Variables|Actor|GetInstigator)) _ownerprojectile))
  (Class|AISenseDamage|ReportDamageEvent (Variables|Default|GetHitActor) _ownerprojectile _returnvalue (Transformation|GetActorLocation _ownerprojectile) (Variables|Default|GetImpact%20Point) "None")
  (Actor|DestroyActor))

(event Collision|EventActorBeginOverlap
  (params (OtherActor :type Actor%20Object%20Reference)))

(event EventTick
  (params (DeltaSeconds :type Float%20%28single-precision%29)))

(event EventBeginPlay)

(fn ConstructionScript)

(fn CreateHitVSFX
  (bind _hitinformation (Variables|Default|GetHitInformation))
  (bind _normal (Variables|Default|GetNormal))
  (bind _hitphysmat (Variables|Default|GetHitPhysMat))
  (bind _returnvalue (* _normal -1))
  (bind (_value _returnvalue_2) (Utilities|Map|Find _hitinformation _hitphysmat))
  (bind _returnvalue_3 (Math|Conversions|RotationFromXVector _returnvalue))
  (bind (_roll _pitch _yaw) (Math|Rotator|BreakRotator _returnvalue_3))
  (LocalVariables|SetHitInfo _value)
  (LocalVariables|SetIsFindPhysMat _returnvalue_2)
  (Audio|PlaySoundatLocation (select (LocalVariables|GetIsFindPhysMat) (.HitSound (Utilities|Struct|BreakST_HitInformation (LocalVariables|GetHitInfo))) 0) (Variables|Default|GetImpact%20Point) "0, 0, 0" 1.0 1.0 0.0 "/Game/ResidentHorrorFPS/Audio/Attenuation/Att_ImpactsAttenuation.Att_ImpactsAttenuation" 0 0 0)
  (Effects|SpawnEmitterAttached (select (LocalVariables|GetIsFindPhysMat) (.HitParticle (Utilities|Struct|BreakST_HitInformation (LocalVariables|GetHitInfo))) 0) (Variables|Default|GetHit%20Component) "None" (Variables|Default|GetImpact%20Point) (Math|Rotator|MakeRotfromZ (Variables|Default|GetNormal)) (Math|Conversions|ToVector(Float) (Math|Random|RandomFloatinRange 0.2 0.5)) "KeepWorldPosition")
  (bind _returnvalue_4 (Class|GameplayStatics|SpawnDecalAttached (select (LocalVariables|GetIsFindPhysMat) (.Decal (Utilities|Struct|BreakST_HitInformation (LocalVariables|GetHitInfo))) 0) (* (* "2.000000,2.000000,2.000000" (Math|Random|RandomFloatinRange 0.75 1.25)) "0.800000,0.800000,0.800000") (Variables|Default|GetHit%20Component) (Variables|Default|GetHit%20Bone%20Name) (Variables|Default|GetImpact%20Point) (Math|Rotator|MakeRotator (Math|Random|RandomFloatinRange 0.0 3.6e+02) _pitch _yaw) "KeepWorldPosition" 15.0))
  (bind _output_get (LocalVariables|SetL_DecalRef _returnvalue_4))
  (Utilities|IsValid _output_get
    (:Is%20Valid
      (bind _returnvalue_5 (Rendering|Material|CreateDynamicMaterialInstance _output_get :!class /Script/Engine.DecalComponent))
      (Rendering|Material|SetScalarParameterValue _returnvalue_5 "Frame" (Math|Random|RandomFloatinRange 0.0 5.0) :!class /Script/Engine.MaterialInstanceDynamic)
      (Rendering|Components|Decal|SetFadeScreenSize (LocalVariables|GetL_DecalRef) 0.0)
      (Rendering|Components|Decal|SetFadeOut (LocalVariables|GetL_DecalRef) 15.0 5.0 false))))

(fn AddPhysicImpulse
  (if (Physics|IsSimulatingPhysics (Variables|Default|GetHit%20Component) "None")
    (Physics|AddImpulseatLocation (Variables|Default|GetHit%20Component) (* (Transformation|GetActorForwardVector) (+ (/ (Math|Vector|VectorLength (Transformation|GetVelocity)) 1e+02) 2e+02)) (Transformation|GetActorLocation) "None")))

(fn Splatter
  (bind _hitresult (Variables|Default|GetHitResult))
  (bind _location (Collision|BreakHitResult _hitresult))
  (Collision|LineTraceByChannel _location (+ _location (* (Transformation|GetActorForwardVector) 1.5e+02)) "TraceTypeQuery1" false (Utilities|Array|MakeArray self) "ForDuration"))