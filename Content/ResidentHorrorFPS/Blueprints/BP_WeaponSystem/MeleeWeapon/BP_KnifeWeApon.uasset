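; Player knife melee weapon that plays one of two random attack montages on use, unless a montage is already playing.
; A montage notify plays the swing sound and runs a short sphere trace from the camera.
; Hits send a hit reaction impulse, apply damage, report it to AI perception and attach a knife decal rolled per montage.
; Surface-type macros then spawn Cascade or Niagara effects and impact sounds from a settings data asset.
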(event Custom|StartTraceAttack
  (bind _returnvalue (Game|GetPlayerCharacter 0))
  (bind _player (Variables|Default|GetPlayer))
  (bind _camera (Variables|/Game/ResidentHorrorFPS/Character/BP_Character/BP_RHV_FPS_Player.BP_RHV_FPS_Player_C|GetCamera _player))
  (bind _returnvalue_2 (Transformation|GetWorldLocation _camera))
  ;[0 0 0 0.5] StartTraceAttack
  (bind (_outhit _returnvalue_3) (Collision|SphereTraceByChannel _returnvalue_2 (+ _returnvalue_2 (* (Math|Vector|GetForwardVector _camera) 1e+02)) 4.0 "TraceTypeQuery3" false (Utilities|Array|MakeArray (Variables|Default|GetPlayer) self) "None"))
  (Variables|Default|SetOut%20Hit _outhit)
  (Variables|Default|SetLastTraceLocation (.TraceEnd (Collision|BreakHitResult (Variables|Default|GetOut%20Hit))))
  (Variables|Default|SetLocation (.Location (Collision|BreakHitResult (Variables|Default|GetOut%20Hit))))
  (Variables|Default|SetHit%20Bone%20Name (.HitBoneName (Collision|BreakHitResult (Variables|Default|GetOut%20Hit))))
  (Variables|Default|SetHit%20Component (.HitComponent (Collision|BreakHitResult (Variables|Default|GetOut%20Hit))))
  (Variables|Default|SetImpact%20Point (.ImpactPoint (Collision|BreakHitResult (Variables|Default|GetOut%20Hit))))
  (Variables|Default|SetHit%20Actor (.HitActor (Collision|BreakHitResult (Variables|Default|GetOut%20Hit))))
  (Variables|Default|SetNormal (.Normal (Collision|BreakHitResult (Variables|Default|GetOut%20Hit))))
  (if _returnvalue_3
    ;[0 0 0 0.5] Activate Physic Controll Npc Test
    (Class|BPIBulletPhysics|HitReaction(Message) (Variables|Default|GetHit%20Actor) (* (Math|Vector|GetUnitDirection(Vector) (Transformation|GetWorldLocation (Variables|/Game/ResidentHorrorFPS/Character/BP_Character/BP_RHV_FPS_Player.BP_RHV_FPS_Player_C|GetCamera (CallFunction|RHVFPSPlayerRef))) "0, 0, 0") -5.6e+03) (Variables|Default|GetHit%20Bone%20Name))
    (bind _returnvalue_4 (Game|Damage|ApplyDamage (Variables|Default|GetHit%20Actor) (Variables|Default|GetDamage) (Game|GetPlayerController 0) self))
    (Class|AISenseDamage|ReportDamageEvent (Variables|Default|GetHit%20Actor) _returnvalue _returnvalue_4 (Transformation|GetActorLocation _returnvalue) (Variables|Default|GetImpact%20Point) "None")
    (Class|GameplayStatics|SpawnDecalAttached "/Game/ResidentHorrorFPS/Demo/Materials/M_Decal_KnifeHit.M_Decal_KnifeHit" (* (* "2.000000,2.000000,2.000000" (Math|Random|RandomFloatinRange 0.75 1.75)) "0.800000,0.800000,0.800000") (Variables|Default|GetHit%20Component) (Variables|Default|GetHit%20Bone%20Name) (Variables|Default|GetImpact%20Point) (Math|Rotator|MakeRotator (.Value (Utilities|Map|Find (Variables|Default|GetRotationDecal) (Variables|Default|GetCurrentAttack))) (.Pitch (Math|Rotator|BreakRotator (Math|Conversions|RotationFromXVector (* (Variables|Default|GetNormal) -1)))) (.Yaw (Math|Rotator|BreakRotator (Math|Conversions|RotationFromXVector (* (Variables|Default|GetNormal) -1))))) "KeepWorldPosition" 15.0)
    (|PhysicalSurface (Variables|/Script/PhysicsCore.PhysicalMaterial|GetSurfaceType (.PhysMat (Collision|BreakHitResult (Variables|Default|GetOut%20Hit)))) (Variables|Default|GetLocation)
      (:Out
        (Class|BPIWeaponDamage|EventDamageRHFPS(Message) (Variables|Default|GetHit%20Actor) (Variables|/Game/ResidentHorrorFPS/Blueprints/BP_DataAsset/DA_WeaponSettings.DA_WeaponSettings_C|GetDamage (Utilities|Struct|BreakST_CustomWeapon (Utilities|Struct|BreakST_ItemInformation (Variables|/Game/ResidentHorrorFPS/Blueprints/BP_ItemBase/DataAsset/PDA_InventoryItem.PDA_InventoryItem_C|GetItem%20Information (Variables|/Game/ResidentHorrorFPS/Blueprints/BP_Inventory/Inventory/ItemData/BP_ItemObject.BP_ItemObject_C|GetPrimaryItemData (Variables|Default|GetItemObject)))))) (Variables|Default|GetOut%20Hit) (CallFunction|RHVFPSPlayerRef))))))

(event EventBeginPlay
  ;[0.15 0.15 0.15 0.5] Begin Play
  (|CallParentFunction)
  (bind _player (Class|BPIPlayerReference|GetPlayer(Message) (Game|GetPlayerCharacter 0)))
  (Variables|Default|SetPlayer _player))

(event Collision|EventActorBeginOverlap
  (params (OtherActor :type Actor%20Object%20Reference))
  (|CallParentFunction OtherActor) ; This node is disabled and will not be called.\nDrag off pins to build functionality.
)

(event EventTick
  (params (DeltaSeconds :type Float%20%28single-precision%29))
  (|CallParentFunction DeltaSeconds) ; This node is disabled and will not be called.\nDrag off pins to build functionality.
)

(event EventUpdateItemInfo
  (params (EquipmentComponent :type BPC%20Equipment%20Object%20Reference) (DataTableRowHandle :type Data%20Table%20Row%20Handle%20Structure))
  (bind (_datatable _rowname) (Utilities|Struct|BreakDataTableRowHandle DataTableRowHandle))
  ;[0 0 0 0.5] Update Infor
  (bind _returnvalue (Utilities|GetDataTableRow _datatable _rowname)
    (:then
      (Variables|Default|SetAnimation (.Animation (Utilities|Struct|BreakST_MeleeInfo _returnvalue)))
      (Variables|Default|SetInteract%20Animation_0 (.InteractAnimation (Utilities|Struct|BreakST_MeleeInfo _returnvalue))))))

(event EventGetConstantUse
  (params (Start? :type Boolean))
  (bind _player (CallFunction|RHVFPSPlayerRef))
  (bind _as_abp_rhplayer (Variables|/Game/ResidentHorrorFPS/Character/BP_Character/BP_RHV_FPS_Player.BP_RHV_FPS_Player_C|GetAs%20ABP%20RHPlayer _player))
  (bind _da_animationstate (Variables|/Game/ResidentHorrorFPS/Character/BP_Character/ABP_RHPlayer.ABP_RHPlayer_C|GetDA_AnimationState _as_abp_rhplayer))
  ;[0 0 0 0.5] Start Attack
  (if (not (Class|AnimInstance|IsAnyMontagePlaying (Variables|/Game/ResidentHorrorFPS/Character/BP_Character/BP_RHV_FPS_Player.BP_RHV_FPS_Player_C|GetABP%20RHFPS (Variables|Default|GetPlayer))))
    (bind _output_get (Variables|Default|SetCurrentAttack (.OutItem (Utilities|Array|Random (Utilities|Array|MakeArray (Variables|/Game/ResidentHorrorFPS/Blueprints/BP_DataAsset/DA_CustomCharacter/Weapons/DA_AnimationState.DA_AnimationState_C|GetAnimation%20Attack%20Melle%20Weapon _da_animationstate) (Variables|/Game/ResidentHorrorFPS/Blueprints/BP_DataAsset/DA_CustomCharacter/Weapons/DA_AnimationState.DA_AnimationState_C|GetAnimation%20Attack%20Melle%20Weapon%202 _da_animationstate))))))
    (bind _notifyname (Utilities|PlayMontage _output_get)
      (:On%20Notify%20Begin
        (switch name _notifyname
          (:StartAttack
            (CallFunction|StartTraceAttack)
            (Audio|PlaySoundatLocation "/Game/ResidentHorrorFPS/Audio/Cue/CUE_AttackSound_Cue.CUE_AttackSound_Cue" (Transformation|GetActorLocation) "0, 0, 0" 1.0 1.0 0.0 "/Game/ResidentHorrorFPS/Audio/Attenuation/Att_ImpactsAttenuation.Att_ImpactsAttenuation" 0 0 0)))))))

(fn ConstructionScript
  (|CallParentFunction))

(fn GetInteractAnimation
  (return (Variables|Default|GetInteract%20Animation_0)))

(fn EffectsImpact
  (params (bRoll :type Boolean) (Location :type Vector) (Cascader%20Effects :type Particle%20System%20Object%20Reference) (Niagara%20Effects :type Niagara%20System%20Object%20Reference) (Niagara? :type Boolean) (Scale%20Particle%20Casacde :type Vector) (Scale%20Particle%20Niagara :type Vector))
  (bind _returnvalue (Math|Random|RandomRotator bRoll))
  (if Niagara?
    (Niagara|SpawnSystematLocation Niagara%20Effects Location _returnvalue Scale%20Particle%20Niagara)
    (else
      (Effects|SpawnEmitteratLocation Cascader%20Effects Location _returnvalue Scale%20Particle%20Casacde))))

(fn ApplyDamageWeapon
  (params (Acto :type Object%20Object%20Reference) (InputPin :type Hit%20Result%20Structure))
  (if (Utilities|DoesObjectImplementInterface Acto "/Game/ResidentHorrorFPS/Blueprints/BP_WeaponSystem/Structure/BPI_WeaponDamage.BPI_WeaponDamage_C")
    (Class|BPIWeaponDamage|EventDamageRHFPS(Message) Acto (Variables|/Game/ResidentHorrorFPS/Blueprints/BP_DataAsset/DA_WeaponSettings.DA_WeaponSettings_C|GetDamage (Utilities|Struct|BreakST_CustomWeapon (Utilities|Struct|BreakST_ItemInformation (Variables|/Game/ResidentHorrorFPS/Blueprints/BP_ItemBase/DataAsset/PDA_InventoryItem.PDA_InventoryItem_C|GetItem%20Information (Variables|/Game/ResidentHorrorFPS/Blueprints/BP_Inventory/Inventory/ItemData/BP_ItemObject.BP_ItemObject_C|GetPrimaryItemData (Variables|Default|GetItemObject)))))) InputPin (CallFunction|RHVFPSPlayerRef))))