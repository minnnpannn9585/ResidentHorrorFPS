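; BP_Rifle is a rifle weapon Blueprint in the ResidentHorrorFPS weapon system, inheriting its firing behavior from a parent class.
; It overrides FireMainWeapon to limit fire rate, using the AutoFire flag as a gate around the parent call.
; The flag blocks further shots until a Delay of GunFireRate from DAWeaponSettings ends.
; Other events are disabled stubs, and construction only calls the parent.
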(event EventBeginPlay
  (|CallParentFunction) ; This node is disabled and will not be called.\nDrag off pins to build functionality.
)

(event Collision|EventActorBeginOverlap
  (params (OtherActor :type Actor%20Object%20Reference))
  (|CallParentFunction OtherActor) ; This node is disabled and will not be called.\nDrag off pins to build functionality.
)

(event EventTick
  (params (DeltaSeconds :type Float%20%28single-precision%29))
  (|CallParentFunction DeltaSeconds) ; This node is disabled and will not be called.\nDrag off pins to build functionality.
)

(event EventFireMainWeapon
  ;[0.15 0.15 0.15 0.5] Firing Rate
  (if (not (Variables|Default|GetAutoFire))
    (Variables|Default|SetAutoFire true)
    (|CallParentFunction)
    (Utilities|FlowControl|Delay (Variables|/Game/ResidentHorrorFPS/Blueprints/BP_DataAsset/DA_WeaponSettings.DA_WeaponSettings_C|GetGun%20Fire%20Rate (Variables|Default|GetDA%20WeaponSettings)))
    (Variables|Default|SetAutoFire false)))

(fn ConstructionScript
  (|CallParentFunction))