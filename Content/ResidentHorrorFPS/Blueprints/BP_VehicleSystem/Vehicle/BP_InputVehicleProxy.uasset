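; Input proxy for the vehicle system that receives player driving input and forwards it to its OwnerVehicle.
; Movement and look axes, handbrake, engine start and exit each call a matching function on the vehicle.
; Holding the right mouse button plays a timeline that offsets the vehicle's spring arm socket for a dashboard focus view, reversing on release.
; GetInputProxyActor returns the proxy itself.
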(event Input|ActionEvents|InputActionJump
  (params (Key :type Key%20Structure))
  (bind _ownervehicle (Variables|Default|GetOwnerVehicle))
  (:Pressed
    (Default|Handbrake _ownervehicle true))
  (:Released
    (Default|Handbrake _ownervehicle false)))

(event Input|AxisEvents|InputAxisLookUp/Down
  (params (AxisValue :type Float%20%28single-precision%29))
  (Default|LookUp/Down (Variables|Default|GetOwnerVehicle) AxisValue))

(event Input|AxisEvents|InputAxisLookLeft/Right
  (params (AxisValue :type Float%20%28single-precision%29))
  (Default|LookRight/Left (Variables|Default|GetOwnerVehicle) AxisValue))

(event Input|AxisEvents|InputAxisVehicle_Move_Forward/Backward
  (params (AxisValue :type Float%20%28single-precision%29))
  (Default|MoveForward/Backward (Variables|Default|GetOwnerVehicle) AxisValue))

(event Input|AxisEvents|InputAxisVehicle_Move_Right/Left
  (params (AxisValue :type Float%20%28single-precision%29))
  (Default|MoveRight/Left (Variables|Default|GetOwnerVehicle) AxisValue))

(event Input|KeyboardEvents|F
  (params (Key :type Key%20Structure))
  (:Pressed
    (Default|ExitVehicle (Variables|Default|GetOwnerVehicle))))

(event Input|KeyboardEvents|G
  (params (Key :type Key%20Structure))
  (:Pressed
    (Default|StartEngine (Variables|Default|GetOwnerVehicle))))

(event Input|MouseEvents|RightMouseButton
  (params (Key :type Key%20Structure))
  (:Pressed
    (bind _alpha (Timeline|FocuseDeashbord Play)
      (:Update
        (Variables|/Script/Engine.SpringArmComponent|SetSocketOffset (Variables|/Game/ResidentHorrorFPS/Blueprints/BP_VehicleSystem/Vehicle/BP_Vehicle.BP_Vehicle_C|GetSpringArm (Variables|Default|GetOwnerVehicle)) (Math|Vector|Lerp(Vector) "0, 0, 0" "15.000000,0.000000,15.000000" _alpha)))))
  (:Released
    (Timeline|FocuseDeashbord Reverse)))

(fn ConstructionScript)

(fn GetInputProxyActor
  (return self))