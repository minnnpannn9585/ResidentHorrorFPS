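; BP_DeshboardElement is a dashboard gauge element for the vehicle system, made of a base mesh and an arrow needle mesh.
; The construction script applies the configurable meshes, offsets the arrow and sets its yaw to the minimum rotation.
; The SetValue event turns the arrow by writing the incoming value directly as its relative yaw, with no scaling or clamping.
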(event EventBeginPlay)

(event Collision|EventActorBeginOverlap
  (params (OtherActor :type Actor%20Object%20Reference)))

(event EventTick
  (params (DeltaSeconds :type Float%20%28single-precision%29)))

(event EventSetValue
  (params (Value :type Float%20%28double-precision%29))
  (Transformation|SetRelativeRotation (Variables|Default|GetArrow) (Math|Rotator|MakeRotator 0.0 0.0 Value) false false))

(fn ConstructionScript
  (bind _arrow (Variables|Default|GetArrow))
  (Components|StaticMesh|SetStaticMesh (Variables|Default|GetBase) (Variables|Default|GetNewBaseMesh))
  (Components|StaticMesh|SetStaticMesh _arrow (Variables|Default|GetNewArrowMash))
  (Transformation|SetRelativeRotation (Variables|Default|GetArrow) (Math|Rotator|MakeRotator 0.0 0.0 (Variables|Default|GetMinRotation)) false false)
  (Transformation|SetRelativeLocation _arrow (Variables|Default|GetNewArrowLocation) false false))