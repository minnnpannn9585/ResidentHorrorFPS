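; BP_FastInspectV2 is an interactable that opens a close-up inspection view with a titled message widget and page navigation.
; Interaction, gated by AmIInspecting, creates WBP_FastInspect, hides the player, disables their input, blends to WhichCamera's owner and enables the mouse cursor.
; CloseInspection fades out the widget and restores the player's view and input.
; Optional comment audio plays after a delay and is cleared on close, so it is one-shot.
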(event Custom|RIGHT%20PAGE
  ;[0 0 0] Here, you can skip to the page number stored in the variable. In this case, it's the page on the right.
  (Default|NextPage (Variables|Default|GetWB%20Inspect) true))

(event Custom|LEFT%20PAGE
  ;[0 0 0] Here, you can skip to the page you specified in the variable. In this case, it's the page on the left.
  (Default|NextPage (Variables|Default|GetWB%20Inspect) false))

(event Custom|Open%20Inspection
  (bind _returnvalue (Game|GetPlayerController 0))
  ;[0 0 0 1 56] Logic
  ;;[0 0 0] Start Inspection
  (Utilities|FlowControl|Sequence
    (:then_0
      (bind _returnvalue_2 (UserInterface|CreateWidget "/Game/ResidentHorrorFPS/Blueprints/BP_FastInspect/WB/WBP_FastInspect.WBP_FastInspect_C" 0 self))
      (bind _output_get (Variables|Default|SetWB%20Inspect _returnvalue_2))
      (Audio|PlaySound2D (Variables|Default|GetSound%20on%20Opening%20Inspection) 1.0 1.0 0.0 0 0)
      (UserInterface|Viewport|AddtoViewport _output_get 0)
      (Variables|/Game/ResidentHorrorFPS/Blueprints/BP_FastInspect/WB/WBP_FastInspect.WBP_FastInspect_C|SetWrite%20your%20message%20here (Variables|Default|GetWB%20Inspect) (Variables|Default|GetWrite%20your%20message%20here))
      (Variables|/Game/ResidentHorrorFPS/Blueprints/BP_FastInspect/WB/WBP_FastInspect.WBP_FastInspect_C|SetTitle (Variables|Default|GetWB%20Inspect) (Variables|Default|GetPage%20Title))
      (Default|Fadin (Variables|Default|GetWB%20Inspect))
      (Rendering|SetActorHiddenInGame (CallFunction|RHVFPSPlayerRef) true)
      (Game|Player|SetViewTargetwithBlend (Game|GetPlayerController 0) (Components|GetOwner (Variables|/Script/Engine.Actor|GetRootComponent (Variables|Default|GetWhich%20camera?))) 1.0 "VTBlend_Cubic" 1.0 false)
      (Input|DisableInput (CallFunction|RHVFPSPlayerRef) (Game|GetPlayerController 0))
      (Utilities|FlowControl|Delay 1.0)
      (Variables|/Script/Engine.PlayerController|SetbShowMouseCursor _returnvalue true)
      (Input|SetInputModeGameandUI _returnvalue (Variables|Default|GetWB%20Inspect) "DoNotLock" true false)
      (if (Variables|Default|GetComment:%20During%20the%20inspection?)
        (Utilities|FlowControl|Delay (Variables|Default|GetTime%20to%20play%20the%20audio%20clip))
        (Audio|SpawnSoundatLocation (Variables|Default|GetSound%20Coment%20inspect) (Transformation|GetWorldLocation (Variables|/Script/Engine.Actor|GetRootComponent (Variables|Default|GetWhich%20camera?))) "0, 0, 0" 1.0 1.0 0.0 "/Game/ResidentHorrorFPS/Audio/Attenuation/Att_LocalVoice.Att_LocalVoice" 0 false)))
    (:then_1
      (CallFunction|VisibilityWidgetChange true))))

(event Custom|Close%20Inspection
  (bind _returnvalue (Game|GetPlayerController 0))
  ;[0 0 0 1 56] Logic
  ;;[0 0 0 1 56] Exit inspection
  (Utilities|FlowControl|Sequence
    (:then_0
      (Variables|Default|SetAm%20I%20inspecting? true)
      (if (Variables|Default|GetAm%20I%20inspecting?)
        (Variables|Default|SetAm%20I%20inspecting? false)
        (Default|FadOut (Variables|Default|GetWB%20Inspect)))
      (Audio|PlaySound2D (Variables|Default|GetSound%20when%20closing%20the%20window) 1.0 1.0 0.0 0 0)
      (Rendering|SetActorHiddenInGame (CallFunction|RHVFPSPlayerRef) false)
      (Game|Player|SetViewTargetwithBlend (Game|GetPlayerController 0) (Game|Player|GetPlayerPawn 0) 1.0 "VTBlend_Cubic" 0.0 false)
      (Input|EnableInput (CallFunction|RHVFPSPlayerRef) (Game|GetPlayerController 0))
      (Utilities|FlowControl|Delay 1.0)
      (Widget|RemovefromParent (Variables|Default|GetWB%20Inspect))
      (Variables|Default|SetAm%20I%20inspecting? true)
      (Variables|/Script/Engine.PlayerController|SetbShowMouseCursor _returnvalue false)
      (Input|SetInputModeGameOnly _returnvalue false)
      (if (Variables|Default|GetComment:%20During%20the%20inspection?)
        (Class|AudioLinkBlueprintInterface|StopLink(Message) (Variables|Default|GetSound%20Coment%20inspect))
        (Variables|Default|SetComment:%20During%20the%20inspection? false)))
    (:then_1
      (CallFunction|VisibilityWidgetChange false))))

(event EventInteraction
  (params (Player :type BP%20RHV%20FPS%20Player%20Object%20Reference) (AutoInteraction%28Non-Player%29 :type Boolean))
  ;[0 0 0 1 45] START INTERACTION
  (if (Variables|Default|GetAm%20I%20inspecting?)
    (CallFunction|OpenInspection)))

(event EventBeginPlay
  ;[0 0 0] BEGIN PLAY
  (|CallParentFunction))

(fn ConstructionScript
  (|CallParentFunction))