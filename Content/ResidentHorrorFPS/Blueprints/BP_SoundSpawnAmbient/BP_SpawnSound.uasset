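; Trigger-box actor that plays an ambient sound at a set world location when the player walks into it.
; After a configurable delay, the overlap asks the player to spawn the sound with its attenuation and volume.
; An optional Destroy flag removes the trigger and saves that state, so it destroys itself again when save data loads.
; A play-once guard exists but is left unconnected.
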(event OnComponentBeginOverlap(Box)
  (params (OverlappedComponent :type Primitive%20Component%20Object%20Reference) (OtherActor :type Actor%20Object%20Reference) (OtherComp :type Primitive%20Component%20Object%20Reference) (OtherBodyIndex :type Integer) (bFromSweep :type Boolean) (SweepResult :type Hit%20Result%20Structure%20%28by%20ref%29))
  (bind _player (CallFunction|RHVFPSPlayerRef))
  ;[0 0 0 0.5 60] THIS CODE PLAYS THE AUDIO AT A SPECIFIC LOCATION
  (if (== OtherActor _player)
    (Utilities|FlowControl|Delay (Variables|Default|GetWhen%20will%20it%20play?))
    (Class|BPISoundWorld|SpawnEffectSoundWorlds(Message) _player (Variables|Default|GetSound) (Variables|Default|GetSound%20Loction) (Variables|Default|GetAttenuation) (Variables|Default|GetVolume%20Sound))
    ;;[0.15 0 0 0.5] Demo (Delete)
    (if (Variables|Default|GetDestroy?)
      (Actor|DestroyActor)
      (Default|SaveData (Variables|Default|GetBP_SaveLoadRHFps) (Utilities|Struct|MakeST_SaveLoad true 0 0)))))

(event LoadedData(BP_SaveLoadRHFps)
  (params (Save%20Loaded%20Data :type ST%20Save%20Load%20Structure))
  ;[0 0 0 0.5] Load
  (if (.Boolean2 (Utilities|Struct|BreakST_SaveLoad Save%20Loaded%20Data))
    (Actor|DestroyActor)))

(fn ConstructionScript)