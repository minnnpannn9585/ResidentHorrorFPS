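; BP_MasterVoiceGameplay is a trigger volume that plays a character voice line during gameplay when the player walks into it.
; Its Box overlap checks that the other actor is the player reference and that it has not fired yet.
; It then passes the configured sound, attenuation and volume to the player pawn's GameplayDialogueMessage and destroys itself, so each placed trigger plays only once.
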(event OnComponentBeginOverlap(Box)
  (params (OverlappedComponent :type Primitive%20Component%20Object%20Reference) (OtherActor :type Actor%20Object%20Reference) (OtherComp :type Primitive%20Component%20Object%20Reference) (OtherBodyIndex :type Integer) (bFromSweep :type Boolean) (SweepResult :type Hit%20Result%20Structure%20%28by%20ref%29))
  ;[0 0 0 1 30] THIS CODE PLAYS THE CHARACTER'S AUDIO
  (if (== OtherActor (CallFunction|RHVFPSPlayerRef))
    (if (not (Variables|Default|GetHas%20it%20played%20yet?😡😡))
      (Variables|Default|SetHas%20it%20played%20yet?😡😡 true)
      (Class|BPISoundWorld|GameplayDialogue(Message) (Game|Player|GetPlayerPawn 0) (Variables|Default|GetSound%20Play🐭😼👍) (Variables|Default|GetAttenuation) (Variables|Default|GetVolume%20Sound))
      (Actor|DestroyActor))))

(fn ConstructionScript)