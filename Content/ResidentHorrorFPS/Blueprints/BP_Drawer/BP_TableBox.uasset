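; Interactive table drawer that the player opens and closes, spawning a random item on first opening.
; In animated mode it holsters equipped gear, glides the player into place at a distance-scaled rate, then plays a montage whose notify moves the drawer.
; Without animation, the drawer slides directly via a reversible timeline.
; Drawer position and spawned item persist through the save component, and item widget visibility follows the drawer state.
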(event LoadedData(BP_SaveLoadRHFps)
  (params (Save%20Loaded%20Data :type ST%20Save%20Load%20Structure))
  (bind (_vvector _boolean2 _boolean4 _itemsdropped) (Utilities|Struct|BreakST_SaveLoad Save%20Loaded%20Data))
  (bind _spawnitem (Variables|Default|GetSpawnItem))
  ;[0 0 0 0.5] Load
  (if _boolean2
    (Transformation|SetRelativeLocation (Variables|Default|GetStaticMesh_0) _vvector false false)
    (Variables|Default|SetClose? false))
  (if _boolean4
    (bind _itemobject (Class|BPIItemObject|GetItemObject(Message) (Variables|/Game/ResidentHorrorFPS/Character/BP_Character/BP_RHV_FPS_Player.BP_RHV_FPS_Player_C|GetBPC_Equipment (CallFunction|RHVFPSPlayerRef))))
    (bind _returnvalue (Game|SpawnActorfromClass "/Game/ResidentHorrorFPS/Blueprints/BP_ItemBase/BP_ItemBaseRHFPS.BP_ItemBaseRHFPS_C" (Math|Transform|MakeTransform (Transformation|GetWorldLocation _spawnitem) (Transformation|GetWorldRotation _spawnitem) "1.000000,1.000000,1.000000") "Undefined" "MultiplyWithRoot" 0 false _itemobject _itemsdropped (CallFunction|RHVFPSPlayerRef)))
    (Variables|Default|SetBP%20Item _returnvalue)))

(event Custom|SetPlayerLocationAndRotation
  (bind _returnvalue (Game|GetPlayerController 0))
  (bind _player (CallFunction|RHVFPSPlayerRef))
  (bind _playertransform (Variables|Default|GetPlayerTransform))
  (bind _returnvalue_2 (Transformation|GetActorLocation _player))
  (bind _returnvalue_3 (Transformation|GetWorldLocation _playertransform))
  ;[0 0 0 0.5] Set Player Location And Rotation
  (bind _alpha (Timeline|PlayerPosition PlayFromStart)
    (:Update
      (Transformation|SetActorLocation (CallFunction|RHVFPSPlayerRef) (Math|Vector|Lerp(Vector) _returnvalue_2 (Math|Vector|MakeVector (.x _returnvalue_3) (.y _returnvalue_3) (.Z (Math|Vector|BreakVector _returnvalue_2))) _alpha) false false)
      (Pawn|SetControlRotation _returnvalue (Math|Rotator|Lerp(Rotator) (Pawn|GetControlRotation _returnvalue :!class /Script/Engine.Controller) (Transformation|GetWorldRotation (Variables|Default|GetPlayerTransform)) _alpha true)))
    (:Finished
      (CallFunction|PlayMontageInteraction)
      (Variables|/Script/Engine.CameraComponent|SetbUsePawnControlRotation (Variables|/Game/ResidentHorrorFPS/Character/BP_Character/BP_RHV_FPS_Player.BP_RHV_FPS_Player_C|GetCamera (CallFunction|RHVFPSPlayerRef)) false)
      (Input|SetIgnoreLookInput (Game|GetPlayerController 0) true))))

(event Custom|TableInteraction
  (bind _returnvalue (Transformation|GetActorLocation))
  ;[0 0 0 0.5] Table Interaction
  (if (not (Variables|Default|GetIn%20Open?))
    (if (Variables|Default|GetClose?)
      (Audio|PlaySoundatLocation "/Game/ResidentHorrorFPS/Audio/Wavs/WAV_DrawerClose.WAV_DrawerClose" _returnvalue "0, 0, 0" 4.0 1.0 0.0 "/Game/ResidentHorrorFPS/Audio/Attenuation/Att_WorldSound.Att_WorldSound" 0 0 0)
      (Collision|SetCollisionResponsetoChannel (Variables|Default|GetStaticMesh_0) "ECC_Pawn" "ECR_Ignore")
      (bind (_direction _alpha) (Timeline|Open/Close PlayFromStart)
        (:Update
          (Variables|Default|SetIn%20Open? true)
          (Transformation|SetRelativeLocation (Variables|Default|GetStaticMesh_0) (Math|Vector|Lerp(Vector) "-6.239888,-58.362144,75.689849" "37.337505,-58.362144,75.689849" _alpha) false false))
        (:Finished
          ;[0 0 0 0.5] Set Variables
          (switch Utilities|FlowControl|Switch|SwitchonETimelineDirection _direction
            (:Forward
              (Variables|Default|SetClose? false))
            (:Backward
              (Variables|Default|SetClose? true)))
          (Variables|Default|SetIn%20Open? false)
          (Collision|SetCollisionResponsetoChannel (Variables|Default|GetStaticMesh_0) "ECC_Pawn" "ECR_Block")
          ;[0 0 0 0.5] Save
          (Utilities|Struct|SetmembersinST_SaveLoad (Variables|Default|GetObject%20Data) (Variables|/Script/Engine.SceneComponent|GetRelativeLocation (Variables|Default|GetStaticMesh_0)) true)
          (Default|SaveData (Variables|Default|GetBP_SaveLoadRHFps) (Variables|Default|GetObject%20Data))))
      (else
        (Audio|PlaySoundatLocation "/Game/ResidentHorrorFPS/Audio/Wavs/WAV_DrawerOpen.WAV_DrawerOpen" _returnvalue "0, 0, 0" 4.0 1.0 0.0 "/Game/ResidentHorrorFPS/Audio/Attenuation/Att_WorldSound.Att_WorldSound" 0 0 0)
        (Collision|SetCollisionResponsetoChannel (Variables|Default|GetStaticMesh_0) "ECC_Pawn" "ECR_Ignore")
        (Timeline|Open/Close ReverseFromEnd)))))

(event Custom|Verification%20Item%20equipped
  (bind _player (CallFunction|RHVFPSPlayerRef))
  (bind _bpc_equipment (Variables|/Game/ResidentHorrorFPS/Character/BP_Character/BP_RHV_FPS_Player.BP_RHV_FPS_Player_C|GetBPC_Equipment _player))
  ;[0 0 0 0.5] Verification Item equipped
  (if (not (Variables|/Game/ResidentHorrorFPS/Blueprints/BP_Inventory/Inventory/Equipment/BPC_Equipment.BPC_Equipment_C|GetEquip%20Item? _bpc_equipment))
    (if (Variables|Default|GetDid%20you%20have%20the%20item%20equipped?)
      (Default|ActivateEquipment/UseItem _bpc_equipment (Variables|/Game/ResidentHorrorFPS/Blueprints/BP_Inventory/Inventory/Equipment/BPC_Equipment.BPC_Equipment_C|GetCurrentIndex _bpc_equipment))
      (Variables|Default|SetDid%20you%20have%20the%20item%20equipped? false))))

(event Custom|PlayMontageInteraction
  (bind _player (CallFunction|RHVFPSPlayerRef))
  (bind _interactioninfo (Variables|Default|GetInteractionInfo))
  (bind _spawnitem (Variables|Default|GetSpawnItem))
  (bind (_closemontage _openmontage) (Utilities|Struct|BreakST_TableInteractionInfo _interactioninfo))
  (bind _camera (Variables|/Game/ResidentHorrorFPS/Character/BP_Character/BP_RHV_FPS_Player.BP_RHV_FPS_Player_C|GetCamera _player))
  (bind _returnvalue (Transformation|GetWorldRotation _camera))
  ;[0 0 0 0.5] Play Montage Interaction
  (if (Variables|Default|GetClose?)
    (if (Variables|Default|GetItem%20Dropped?)
      (bind _bp_item (Variables|Default|GetBP%20Item :!label _label)
        (:then
          ;[0 0 0 0.5] Switch Visibility Widget Main
          (if (Variables|Default|GetClose?)
            (Utilities|FlowControl|Sequence
              (:then_0
                (Utilities|FlowControl|Delay 0.8)
                (Default|VisibilityWidgetChange _bp_item false))
              (:then_1
                (switch Utilities|FlowControl|Switch|SwitchonE_TypeInteraction (Variables|Default|Get%20TypeInteraction) :!label _label_2
                  (:NewEnumerator1
                    ;[0 0 0 0.5] Play monte Type Ineraction
                    (bind _notifyname (Animation|Montage|PlayMontage (Variables|/Script/Engine.Character|GetMesh (CallFunction|RHVFPSPlayerRef)) (select (Variables|Default|GetClose?) _openmontage _closemontage))
                      (:OnCompleted
                        ;[0 0 0 0.5] Set Rotation Player
                        (Pawn|SetControlRotation (Game|GetPlayerController 0) (Math|Rotator|MakeRotator 0.0 (.pitch _returnvalue) (.yaw _returnvalue)))
                        ;[0 0 0 0.5] Settings Controller
                        (Variables|/Script/Engine.CameraComponent|SetbUsePawnControlRotation _camera true)
                        (Input|ResetIgnoreLookInput (Game|GetPlayerController 0))
                        (Input|EnableInput (CallFunction|RHVFPSPlayerRef) (Game|GetPlayerController 0))
                        (Utilities|FlowControl|Delay 0.8)
                        (CallFunction|VerificationItemEquipped))
                      (:OnNotifyBegin
                        (switch name _notifyname
                          (:StartAnimation
                            (CallFunction|TableInteraction)))))))))
            (else
              (Utilities|FlowControl|Sequence
                (:then_0
                  (Utilities|FlowControl|Delay 0.8)
                  (Default|VisibilityWidgetChange _bp_item true))
                (:then_1
                  (goto _label_2))))))
        (:else
          (goto _label_2)))
      (else
        (Variables|Default|SetItem%20Dropped? true)
        (bind _itemobject (Class|BPIItemObject|GetItemObject(Message) (Variables|/Game/ResidentHorrorFPS/Character/BP_Character/BP_RHV_FPS_Player.BP_RHV_FPS_Player_C|GetBPC_Equipment (CallFunction|RHVFPSPlayerRef))))
        (bind _returnvalue_2 (Game|SpawnActorfromClass "/Game/ResidentHorrorFPS/Blueprints/BP_ItemBase/BP_ItemBaseRHFPS.BP_ItemBaseRHFPS_C" (Math|Transform|MakeTransform (Transformation|GetWorldLocation _spawnitem) (Transformation|GetWorldRotation _spawnitem) "1.000000,1.000000,1.000000") "Undefined" "MultiplyWithRoot" 0 false _itemobject (.OutItem (Utilities|Array|Random (Variables|Default|GetItems%20Dropped))) (CallFunction|RHVFPSPlayerRef)))
        (bind _output_get (Variables|Default|SetBP%20Item _returnvalue_2))
        ;[0 0 0 0.5] SAVE
        (Utilities|Struct|SetmembersinST_SaveLoad (Variables|Default|GetObject%20Data) true (Variables|/Game/ResidentHorrorFPS/Blueprints/BP_InteractMaster/BP_RHMasterInteract.BP_RHMasterInteract_C|GetPrymaryDataAsset _output_get))
        (Default|SaveData (Variables|Default|GetBP_SaveLoadRHFps) (Variables|Default|GetObject%20Data))
        (goto _label_2)))
    (else
      (goto _label))))

(event EventBeginPlay
  ;[0 0 0 0.5] Begin Play
  (|CallParentFunction))

(event EventInteraction
  (params (Player :type BP%20RHV%20FPS%20Player%20Object%20Reference) (AutoInteraction%28Non-Player%29 :type Boolean))
  (bind _player (CallFunction|RHVFPSPlayerRef))
  (bind _bpc_equipment (Variables|/Game/ResidentHorrorFPS/Character/BP_Character/BP_RHV_FPS_Player.BP_RHV_FPS_Player_C|GetBPC_Equipment _player))
  ;[0 0 0 0.5] Inicial Interact
  (switch Utilities|FlowControl|Switch|SwitchonE_TypeInteraction (Variables|Default|Get%20TypeInteraction)
    (:NewEnumerator1
      ;[0 0 0 0.5] Verificiation Item Equippeds
      (if (Variables|/Game/ResidentHorrorFPS/Blueprints/BP_Inventory/Inventory/Equipment/BPC_Equipment.BPC_Equipment_C|GetEquip%20Item? (Variables|/Game/ResidentHorrorFPS/Character/BP_Character/BP_RHV_FPS_Player.BP_RHV_FPS_Player_C|GetBPC_Equipment (CallFunction|RHVFPSPlayerRef)))
        (Default|ActivateEquipment/UseItem _bpc_equipment (Variables|/Game/ResidentHorrorFPS/Blueprints/BP_Inventory/Inventory/Equipment/BPC_Equipment.BPC_Equipment_C|GetCurrentIndex _bpc_equipment))
        (Utilities|FlowControl|Delay 1.0)
        (Variables|Default|SetDid%20you%20have%20the%20item%20equipped? true))
      (Input|DisableInput Player (Game|GetPlayerController 0))
      (CallFunction|CheckDistanceto)
      (CallFunction|SetPlayerLocationandRotation))
    (:NewEnumerator2
      ;[0 0 0 0.5] Type Interaction No animation
      (CallFunction|TableInteraction)
      (CallFunction|PlayMontageInteraction))))

(fn ConstructionScript)

(fn CheckDistanceto
  (Components|Timeline|SetPlayRate (Variables|Default|GetPlayerPosition) (Math|Float|MapRangeClamped (Math|Vector|Distance(Vector) (Transformation|GetActorLocation (CallFunction|RHVFPSPlayerRef)) (Transformation|GetWorldLocation (Variables|Default|GetPlayerTransform))) 0.0 2e+02 5.0 1.0))
  (return))

(fn UpdateAnimation)