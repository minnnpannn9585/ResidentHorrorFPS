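; Master interactable item Blueprint that shows a world widget with the item's name from its data asset when the player comes near.
; Overlapping InteractableAlert creates WBP_SingleInteraction in InteractWidget; leaving it removes the widget.
; DefineActor crossfades between alert and interaction displays based on a hit flag.
; The data asset configures SphereItem's trace blocking, collision is enabled after a startup delay, and VisibilityWidgetChange toggles widget and collision together.
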(event OnComponentBeginOverlap(InteractableAlert)
  (params (OverlappedComponent :type Primitive%20Component%20Object%20Reference) (OtherActor :type Actor%20Object%20Reference) (OtherComp :type Primitive%20Component%20Object%20Reference) (OtherBodyIndex :type Integer) (bFromSweep :type Boolean) (SweepResult :type Hit%20Result%20Structure%20%28by%20ref%29))
  ;[0 0 0 0.5 50] Begin Overlap
  (CallFunction|ForceCreateWidgetBeginOveralp OtherActor))

(event OnComponentEndOverlap(InteractableAlert)
  (params (OverlappedComponent :type Primitive%20Component%20Object%20Reference) (OtherActor :type Actor%20Object%20Reference) (OtherComp :type Primitive%20Component%20Object%20Reference) (OtherBodyIndex :type Integer))
  ;[0 0 0 0.5 50] End Overlap
  (bind _wbp_interact (Variables|Default|GetWBP%20Interact)
    (:then
      (Widget|RemovefromParent _wbp_interact)
      (Rendering|SetVisibility (Variables|Default|GetInteractWidget) false false))
    (:else)))

(event Custom|Visibility%20Widget%20Change
  (params (Visibility%20Of%20widget%20Interaction? :type Boolean))
  ;[0 0 0 0.5 50] Visibility Widget Change
  (if Visibility%20Of%20widget%20Interaction?
    (Rendering|SetVisibility (Variables|Default|GetInteractWidget) false false)
    (Collision|SetCollisionEnabled (Variables|Default|GetSphereItem) "NoCollision")
    ;[0 0 0 0.5] ensuring the widget disappears
    (Collision|SetCollisionResponsetoAllChannels (Variables|Default|GetInteractableAlert) "ECR_Ignore")
    (Collision|SetCollisionObjectType (Variables|Default|GetSphereItem) "ECC_Pawn")
    (else
      (Rendering|SetVisibility (Variables|Default|GetInteractWidget) true false)
      (Collision|SetCollisionEnabled (Variables|Default|GetSphereItem) "QueryAndPhysics")
      ;[0 0 0 0.5] ensuring the widget appears
      (Collision|SetCollisionResponsetoAllChannels (Variables|Default|GetInteractableAlert) "ECR_Overlap")
      (Collision|SetCollisionResponsetoChannel (Variables|Default|GetSphereItem) "ECC_GameTraceChannel2" "ECR_Block"))))

(event Custom|Collsion%20Enable
  ;[0 0 0 1 50] Collsion Enable Item
  (Utilities|FlowControl|Delay 1.0)
  (Collision|SetCollisionEnabled (Variables|Default|GetSphereItem) "QueryAndPhysics")
  (Collision|SetCollisionEnabled (Variables|Default|GetInteractableAlert) "QueryOnly"))

(event EventBeginPlay
  (bind _sphereitem (Variables|Default|GetSphereItem))
  ;[0 0 0 0.5 50] Begin Play
  (Utilities|FlowControl|Sequence
    (:then_0
      (if (Utilities|Struct|BreakST_ItemInformation (Variables|/Game/ResidentHorrorFPS/Blueprints/BP_ItemBase/DataAsset/PDA_InventoryItem.PDA_InventoryItem_C|GetItem%20Information (Variables|Default|GetPrymaryDataAsset)))
        (Collision|SetCollisionEnabled _sphereitem "QueryAndPhysics")
        (Collision|SetCollisionResponsetoChannel _sphereitem "ECC_GameTraceChannel2" "ECR_Block")
        (else
          (Collision|SetCollisionEnabled (Variables|Default|GetSphereItem) "NoCollision")
          (Collision|SetCollisionResponsetoChannel (Variables|Default|GetSphereItem) "ECC_GameTraceChannel2" "ECR_Ignore"))))
    (:then_1
      (CallFunction|CollsionEnable))))

(event EventDefineActor
  (params (Hit? :type Boolean))
  ;[0 0 0 0.5 50] Define Acto Visibility Widget
  (if Hit?
    (bind _wbp_interact (Variables|Default|GetWBP%20Interact)
      (:then
        (Default|FadOutAlert _wbp_interact)
        (Default|FadinInteraction _wbp_interact))
      (:else))
    (else
      (bind _wbp_interact_2 (Variables|Default|GetWBP%20Interact)
        (:then
          (Default|FadinAlert _wbp_interact_2)
          (Default|FadOutInteraction _wbp_interact_2))
        (:else)))))

(fn ConstructionScript)

(fn RemoveWidgetEndOverlap
  (params (Get%20component%20By%20Class :type Actor%20Object%20Reference))
  (bind _wbp_interact (Variables|Default|GetWBP%20Interact)
    (:then
      (Default|FadOutAlert _wbp_interact)
      (if (Utilities|IsValid (Actor|GetComponentbyClass Get%20component%20By%20Class "/Game/ResidentHorrorFPS/Blueprints/BP_InteractMaster/InteractionSystem/BPC_Interaction.BPC_Interaction_C"))
        _))
    (:else)))

(fn ForceCreateWidgetBeginOveralp
  (params (PlayerRef :type Object%20Object%20Reference))
  (if (== PlayerRef (CallFunction|RHVFPSPlayerRef))
    (bind _returnvalue (UserInterface|CreateWidget "/Game/ResidentHorrorFPS/Blueprints/BP_InteractMaster/InteractionSystem/WBP_SingleInteraction.WBP_SingleInteraction_C" 0 (Utilities|Struct|BreakST_ItemVisualization (Utilities|Struct|BreakST_ItemInformation (Variables|/Game/ResidentHorrorFPS/Blueprints/BP_ItemBase/DataAsset/PDA_InventoryItem.PDA_InventoryItem_C|GetItem%20Information (Variables|Default|GetPrymaryDataAsset))))))
    (bind _output_get (Variables|Default|SetWBP%20Interact _returnvalue))
    (Rendering|SetVisibility (Variables|Default|GetInteractWidget) true true)
    (UserInterface|SetWidget (Variables|Default|GetInteractWidget) _output_get)
    (Default|FadinAlert (Variables|Default|GetWBP%20Interact))))