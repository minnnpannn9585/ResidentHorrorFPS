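; Physics-driven interactable item actor that plays impact and sliding sounds as it moves around the world.
; Hits above a mass-scaled impulse threshold play a pitch-randomized impact sound with volume scaled by force, gated until a weaker hit resets it.
; Each impact starts a looping timer that fades in the slide sound while horizontal speed is high, then fades it out and clears itself when movement slows.
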(event Custom|CalculateSlideSound
  (bind _returnvalue (Transformation|GetVelocity))
  (bind _slidesound (Variables|Default|GetSlideSound))
  (if (> (Math|Vector|VectorLength (Math|Vector|MakeVector (.x _returnvalue) (.y _returnvalue) 0.0)) 1e+02)
    (Utilities|FlowControl|DoOnce false :!label _label
      (:Completed
        (Audio|Components|Audio|Play _slidesound 0.0)
        (Audio|Components|Audio|FadeIn _slidesound 0.1 0.2 0.0 "Linear" :!class /Script/Engine.AudioComponent)))
    (else
      (Audio|Components|Audio|FadeOut (Variables|Default|GetSlideSound) 0.25 0.1 "Linear" :!class /Script/Engine.AudioComponent)
      (Utilities|Time|ClearandInvalidateTimerbyHandle (Variables|SoundPhysic|GetCheckSlideTimer))
      (goto _label Reset))))

(event Custom|StartSlide
  (bind _returnvalue (Utilities|Time|SetTimerbyEvent (delegate Custom|CalculateSlideSound) 0.01 true))
  (Variables|SoundPhysic|SetCheckSlideTimer _returnvalue))

(event EventBeginPlay
  ;[0.15 0.15 0.15 0.5] Comment
  (|CallParentFunction)
  (Audio|Components|Audio|SetSound (Variables|Default|GetSlideSound) (Variables|Default|GetSlideSoundCue)))

(event EventTick
  (params (DeltaSeconds :type Float%20%28single-precision%29))
  ;[0.15 0.15 0.15 0.5] Event Tick
  (|CallParentFunction DeltaSeconds))

(event Collision|EventHit
  (params (MyComp :type Primitive%20Component%20Object%20Reference) (Other :type Actor%20Object%20Reference) (OtherComp :type Primitive%20Component%20Object%20Reference) (bSelfMoved :type Boolean) (HitLocation :type Vector :default "0, 0, 0") (HitNormal :type Vector :default "0, 0, 0") (NormalImpulse :type Vector :default "0, 0, 0") (Hit :type Hit%20Result%20Structure%20%28by%20ref%29))
  (bind _returnvalue (Math|Vector|VectorLength NormalImpulse))
  (if (> _returnvalue (* (Physics|GetMass (Variables|Default|GetitemMesh)) 1e+02))
    (Utilities|FlowControl|DoOnce false :!label _label
      (:Completed
        (Variables|SoundPhysic|SetHit%20Location HitLocation)
        (Variables|SoundPhysic|SetForce (Math|Float|NormalizetoRange _returnvalue 15.0 2e+03))
        (Audio|PlaySoundatLocation (Variables|Default|GetHitSound) (Variables|SoundPhysic|GetHit%20Location) "0, 0, 0" (* (* 1.0 (Variables|SoundPhysic|GetForce)) (Variables|SoundPhysic|GetItemVolumeMult)) (Math|Random|RandomFloatinRange 0.9 1.0) 0.0 "/Game/ResidentHorrorFPS/Audio/Attenuation/Att_ImpactsAttenuation.Att_ImpactsAttenuation" 0 self 0)
        (CallFunction|StartSlide)))
    (else
      (goto _label Reset))))

(fn ConstructionScript)