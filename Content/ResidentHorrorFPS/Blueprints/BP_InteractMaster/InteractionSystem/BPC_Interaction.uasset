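; Player interaction component for a first-person horror game, which also seeds the inventory with starting items on BeginPlay.
; Each tick a short camera sphere trace finds BPI_Interaction actors, toggles their focus state and resizes the HUD crosshair.
; Interact, blocked during montages, messages the focused actor, forwards it to the puzzle component and opens inspection for inspectable items not yet recorded.
; Helpers compute a clamped hand-reach location; depth-of-field autofocus is disconnected.
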(event EventBeginPlay
  (bind _player (CallFunction|RHVFPSPlayerRef))
  ;[0 0 0 0.5] Begin Play
  (bind _player_2 (Class|BPIPlayerReference|GetPlayer(Message) (Components|GetOwner)))
  (Variables|Reference|SetPlayer _player_2)
  (if (Variables|/Game/ResidentHorrorFPS/Blueprints/BP_Inventory/Inventory/BPC_Inventory.BPC_Inventory_C|GetAdd%20Item%20Begin%20Play%20Inventory? (Variables|/Game/ResidentHorrorFPS/Character/BP_Character/BP_RHV_FPS_Player.BP_RHV_FPS_Player_C|GetBPC_Inventory (CallFunction|RHVFPSPlayerRef)))
    ;[0 0 0 0.5] No remove
    (Utilities|FlowControl|Delay 0.2)
    ;[0 0 0 0.5] Add Item Inventory
    (for _array_element (Variables|/Game/ResidentHorrorFPS/Blueprints/BP_Inventory/Inventory/BPC_Inventory.BPC_Inventory_C|GetAdd%20Items%20Inicialize%20Inventory (Variables|/Game/ResidentHorrorFPS/Character/BP_Character/BP_RHV_FPS_Player.BP_RHV_FPS_Player_C|GetBPC_Inventory (CallFunction|RHVFPSPlayerRef)))
      (bind _returnvalue (Default|ConstructItemObject (Variables|/Game/ResidentHorrorFPS/Character/BP_Character/BP_RHV_FPS_Player.BP_RHV_FPS_Player_C|GetBPC_Equipment _player) (Variables|/Game/ResidentHorrorFPS/Blueprints/BP_ItemBase/DataAsset/PDA_InventoryItem.PDA_InventoryItem_C|GetItemObjectClass _array_element) (Variables|/Game/ResidentHorrorFPS/Blueprints/BP_ItemBase/DataAsset/PDA_InventoryItem.PDA_InventoryItem_C|GetItem%20Information _array_element) _array_element))
      (Default|AddItemforInventory (Variables|/Game/ResidentHorrorFPS/Character/BP_Character/BP_RHV_FPS_Player.BP_RHV_FPS_Player_C|GetBPC_Equipment _player) _returnvalue false))
    ;;[0 0 0 0.5] No Remove
    (Variables|/Game/ResidentHorrorFPS/Blueprints/BP_Inventory/Inventory/BPC_Inventory.BPC_Inventory_C|SetItem%20Object (Variables|/Game/ResidentHorrorFPS/Character/BP_Character/BP_RHV_FPS_Player.BP_RHV_FPS_Player_C|GetBPC_Inventory (CallFunction|RHVFPSPlayerRef)) 0)))

(event EventTick
  (params (DeltaSeconds :type Float%20%28single-precision%29))
  ;[0 0 0 0.5] Event Tick
  (Variables|Interaction|Parametr|SetDelta%20seconds DeltaSeconds)
  (Interaction|TraceInteraction)
  (Effect|InitializateDepthOfField)
  (Effect|InitializateDepthOfField))

(fn Interact
  (if (not (Class|AnimInstance|IsAnyMontagePlaying (Variables|/Game/ResidentHorrorFPS/Character/BP_Character/BP_RHV_FPS_Player.BP_RHV_FPS_Player_C|GetABP%20RHFPS (Variables|Reference|GetPlayer))))
    (bind _currentinteractableitem (Variables|Interaction|GetCurrentInteractableItem)
      (:then
        (Class|BPIInteraction|Interaction(Message) _currentinteractableitem (Variables|Reference|GetPlayer) false)
        (Variables|Interaction|Parametr|SetCurrentTemporaryItem _currentinteractableitem)
        (Default|Use (Variables|/Game/ResidentHorrorFPS/Character/BP_Character/BP_RHV_FPS_Player.BP_RHV_FPS_Player_C|GetPuzzleComponent (CallFunction|RHVFPSPlayerRef)) _currentinteractableitem (Variables|Default|GetHit%20Component))
        (Variables|/Game/ResidentHorrorFPS/Blueprints/BP_Inventory/Inventory/BPC_Inventory.BPC_Inventory_C|GetItem%20Object (Variables|/Game/ResidentHorrorFPS/Character/BP_Character/BP_RHV_FPS_Player.BP_RHV_FPS_Player_C|GetBPC_Inventory (CallFunction|RHVFPSPlayerRef))
          (:then
            (bind _sucess (CallFunction|CheckInspect))
            (if _sucess
              (bind _item_object (Variables|/Game/ResidentHorrorFPS/Blueprints/BP_Inventory/Inventory/BPC_Inventory.BPC_Inventory_C|GetItem%20Object (Variables|/Game/ResidentHorrorFPS/Character/BP_Character/BP_RHV_FPS_Player.BP_RHV_FPS_Player_C|GetBPC_Inventory (CallFunction|RHVFPSPlayerRef)))
                (:then
                  (if (Variables|/Game/ResidentHorrorFPS/Blueprints/BP_ItemBase/DataAsset/PDA_InventoryItem.PDA_InventoryItem_C|GetItem%20inspect? (Variables|/Game/ResidentHorrorFPS/Blueprints/BP_Inventory/Inventory/ItemData/BP_ItemObject.BP_ItemObject_C|GetPrimaryItemData _item_object))
                    (if (Variables|/Game/ResidentHorrorFPS/Blueprints/BP_ItemBase/DataAsset/PDA_InventoryItem.PDA_InventoryItem_C|GetInspect%20item%20Hand? (Variables|/Game/ResidentHorrorFPS/Blueprints/BP_Inventory/Inventory/ItemData/BP_ItemObject.BP_ItemObject_C|GetPrimaryItemData _item_object))
                      (if (Variables|/Game/ResidentHorrorFPS/Blueprints/BP_Inventory/Inventory/Equipment/BPC_Equipment.BPC_Equipment_C|GetEquip%20Item? (Variables|/Game/ResidentHorrorFPS/Character/BP_Character/BP_RHV_FPS_Player.BP_RHV_FPS_Player_C|GetBPC_Equipment (CallFunction|RHVFPSPlayerRef)))
                        (Default|Inspect (Variables|/Game/ResidentHorrorFPS/Character/BP_Character/BP_RHV_FPS_Player.BP_RHV_FPS_Player_C|GetBPC_Inventory (CallFunction|RHVFPSPlayerRef)) :!label _label)
                        (else
                          (Default|ActivateInspectItem :self (Variables|/Game/ResidentHorrorFPS/Character/BP_Character/BP_RHV_FPS_Player.BP_RHV_FPS_Player_C|GetBPC_Inventory (CallFunction|RHVFPSPlayerRef)) :InspectItem? true :ItemObject _item_object)
                          (Variables|/Script/Engine.PlayerController|SetbShowMouseCursor (Game|GetPlayerController 0) true)
                          (Variables|Default|SetInspect%20Hand%20Inventory? true)))
                      (else
                        (goto _label)))))
                (:else))))
          (:else)))
      (:else))))

(fn InitializateDepthOfField)

(fn CheckDistancetoInteract
  (bind _player (Variables|Reference|GetPlayer))
  (bind _currentinteractableitem (Variables|Interaction|GetCurrentInteractableItem))
  (bind _returnvalue (Transformation|GetActorLocation _currentinteractableitem))
  (bind _mesh (Variables|/Script/Engine.Character|GetMesh _player))
  (bind _returnvalue_2 (Transformation|GetSocketTransform _mesh "root" "RTS_World"))
  (bind _returnvalue_3 (Math|Transform|MakeTransform _returnvalue))
  (bind _returnvalue_4 (Math|Transform|MakeRelativeTransform _returnvalue_3 _returnvalue_2))
  (bind (_x _y _z) (Math|Vector|BreakVector (.location _returnvalue_4)))
  (bind _returnvalue_5 (Math|Float|Clamp(Float) _y 0.0 1e+02))
  (bind _returnvalue_6 (Math|Float|Clamp(Float) _x -1e+02 1e+02))
  (bind _output (UsableInteraction|CircleClamp (Math|Vector2D|MakeVector2D _returnvalue_6 _returnvalue_5)))
  (Variables|Interaction|Parametr|SetRelativeHandLocation (+ (Math|Vector|MakeVector (.x _output) (.y _output) _z) "0.000000,0.000000,5.000000"))
  (return))

(fn CircleClamp
  (params (Input :type Vector%202D%20Structure))
  (bind _returnvalue (>= (.x Input) 0.0))
  (return (Math|Vector2D|MakeVector2D (* (Math|Float|SelectFloat 1.0 -1.0 _returnvalue) (Math|Float|Clamp(Float) (Math|Float|SelectFloat 1.0 -1.0 _returnvalue) (UsableInteraction|CircleCalculation 3e+01 (.y Input)) (UsableInteraction|CircleCalculation 1e+02 (.y Input)))) (Math|Float|Clamp(Float) (.y Input) (UsableInteraction|CircleCalculation 3e+01 (.x Input)) (UsableInteraction|CircleCalculation 1e+02 (.x Input))))))

(fn CircleCalculation
  (params (Radius :type Float%20%28double-precision%29) (Input :type Float%20%28double-precision%29))
  (return (Math|Float|Sqrt (- (* Radius Radius) (* Input Input)))))

(fn SetInteractable
  (params (InteractableActor :type Actor%20Object%20Reference))
  (Utilities|IsValid InteractableActor
    (:Is%20Valid
      (if (!= InteractableActor (Variables|Interaction|GetCurrentInteractableItem))
        (bind _currentinteractableitem (Variables|Interaction|GetCurrentInteractableItem)
          (:then
            (Class|BPIInteraction|DefineActor(Message) _currentinteractableitem false)
            (bind _output_get (Variables|Interaction|SetCurrentInteractableItem InteractableActor))
            (Class|BPIInteraction|DefineActor(Message) _output_get true))
          (:else
            (bind _output_get_2 (Variables|Interaction|SetCurrentInteractableItem InteractableActor :!label _label))
            (Class|BPIInteraction|DefineActor(Message) _output_get_2 true)))
        (else
          (goto _label))))
    (:Is%20Not%20Valid
      (bind _currentinteractableitem_2 (Variables|Interaction|GetCurrentInteractableItem)
        (:then
          (Class|BPIInteraction|DefineActor(Message) _currentinteractableitem_2 false)
          (Variables|Interaction|SetCurrentInteractableItem 0))
        (:else)))))

(fn TraceInteraction
  (bind _player (CallFunction|RHVFPSPlayerRef))
  (bind _player_2 (Variables|Reference|GetPlayer))
  (bind _camera (Variables|/Game/ResidentHorrorFPS/Character/BP_Character/BP_RHV_FPS_Player.BP_RHV_FPS_Player_C|GetCamera _player_2))
  (bind _wbp_main_hud (Variables|/Game/ResidentHorrorFPS/Character/BP_Character/BP_RHV_FPS_Player.BP_RHV_FPS_Player_C|GetWBP%20Main%20Hud _player))
  (bind _returnvalue (Transformation|GetWorldLocation _camera))
  (bind (_outhit _returnvalue_2) (Collision|SphereTraceByChannel _returnvalue (+ _returnvalue (* (Math|Vector|GetForwardVector _camera) 95.0)) 2.0 "TraceTypeQuery4" false (Utilities|Array|MakeArray (Game|GetPlayerCharacter 0)) "None" true "(R=1.000000,G=0.583200,B=0.000000,A=1.000000)" "(R=0.000000,G=1.000000,B=0.000000,A=1.000000)" 0.1))
  (if _returnvalue_2
    (if (Utilities|DoesObjectImplementInterface (.HitActor (Collision|BreakHitResult _outhit)) "/Game/ResidentHorrorFPS/Blueprints/BP_InteractMaster/InteractionSystem/BPI_Interaction.BPI_Interaction_C")
      (Interaction|SetInteractable (.HitActor (Collision|BreakHitResult _outhit)))
      (Variables|Default|SetHit%20Component (.HitComponent (Collision|BreakHitResult _outhit)))
      (Default|Size12PointInteract _wbp_main_hud)
      (else
        (Interaction|SetInteractable :!label _label)
        (Default|Size8PointInteract _wbp_main_hud)))
    (else
      (goto _label))))

(fn EndInteraction
  (bind _currenttemporaryitem (Variables|Interaction|Parametr|GetCurrentTemporaryItem))
  (Utilities|IsValid _currenttemporaryitem
    (:Is%20Valid
      (Class|BPIInteraction|EndInteraction(Message) _currenttemporaryitem)
      (Variables|Interaction|SetCurrentInteractableItem 0)
      (return))))

(fn CheckInspect
  (bind _player (CallFunction|RHVFPSPlayerRef))
  (bind _bpc_inventory (Variables|/Game/ResidentHorrorFPS/Character/BP_Character/BP_RHV_FPS_Player.BP_RHV_FPS_Player_C|GetBPC_Inventory _player))
  (bind _itemobjectbase (Variables|/Game/ResidentHorrorFPS/Blueprints/BP_Inventory/Inventory/BPC_Inventory.BPC_Inventory_C|GetItemObjectBase _bpc_inventory))
  (bind _item_object (Variables|/Game/ResidentHorrorFPS/Blueprints/BP_Inventory/Inventory/BPC_Inventory.BPC_Inventory_C|GetItem%20Object _bpc_inventory))
  (bind _primaryitemdata (Variables|/Game/ResidentHorrorFPS/Blueprints/BP_Inventory/Inventory/ItemData/BP_ItemObject.BP_ItemObject_C|GetPrimaryItemData _item_object))
  (Utilities|IsValid _item_object
    (:Is%20Valid
      (if (Utilities|Array|ContainsItem _itemobjectbase _primaryitemdata)
        (return false)
        (else
          (Utilities|Array|Add _itemobjectbase _primaryitemdata)
          (return true))))))