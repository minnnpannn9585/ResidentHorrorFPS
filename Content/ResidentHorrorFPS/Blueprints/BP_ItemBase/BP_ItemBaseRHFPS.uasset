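; Base pickup item actor for the horror FPS, taking its mesh, optional shiny overlay, montage and hand offsets from a primary data asset.
; Interaction adds an existing or newly constructed item object to the player's equipment inventory, then plays a pickup montage with an IK hand target.
; Montage notifies attach it to the free hand and destroy it.
; Pickup state is saved, so collected items destroy themselves on load.
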(event LoadedData(BP_SaveLoadRHFps)
  (params (Save%20Loaded%20Data :type ST%20Save%20Load%20Structure))
  ;[0 0 0 0.5] Load
  (if (Utilities|Struct|BreakST_SaveLoad Save%20Loaded%20Data)
    (Actor|DestroyActor)))

(event EventBeginPlay
  ;[0 0 0 0.5] Begin Play
  (|CallParentFunction)
  (CallFunction|UpdateMesh))

(event EventInteraction
  (params (Player :type BP%20RHV%20FPS%20Player%20Object%20Reference) (AutoInteraction%28Non-Player%29 :type Boolean))
  ;[0 0 0] Inveraction Item
  ;;[0 0 0 0.5] Inicial Interact
  (Variables|Reference|SetPlayer Player)
  (if (not (Class|AnimInstance|IsAnyMontagePlaying (Variables|/Game/ResidentHorrorFPS/Character/BP_Character/BP_RHV_FPS_Player.BP_RHV_FPS_Player_C|GetABP%20RHFPS (Variables|Reference|GetPlayer))))
    ;;[0.15 0.15 0.15 0.5] Add To inventory Item
    (bind _add_ (CallFunction|AddtoInventory))
    (if _add_
      ;;[0.15 0.15 0.15 0.5] InteractionEnable
      (Interactable|InteractionEnable false)
      ;;[0.15 0.15 0.15 0.5] Check distance interact
      (Default|CheckDistancetoInteract (Variables|/Game/ResidentHorrorFPS/Character/BP_Character/BP_RHV_FPS_Player.BP_RHV_FPS_Player_C|GetBPC_Interaction (Variables|Reference|GetPlayer)))
      (Utilities|IsValid (Default|GetCurrentHandItem (Variables|/Game/ResidentHorrorFPS/Character/BP_Character/BP_RHV_FPS_Player.BP_RHV_FPS_Player_C|GetBPC_Equipment (Variables|Reference|GetPlayer)))
        (:Is%20Valid
          ;;[0.15 0.15 0.15 0.5] Interface Animation
          (bind _interactanimation (Class|BPIConstantUse|GetInteractAnimation(Message) (Default|GetCurrentHandItem (Variables|/Game/ResidentHorrorFPS/Character/BP_Character/BP_RHV_FPS_Player.BP_RHV_FPS_Player_C|GetBPC_Equipment (Variables|Reference|GetPlayer))))))
        (:Is%20Not%20Valid
          _))
      (Utilities|PlayInteractionMontage (select (Utilities|IsValid (Default|GetCurrentHandItem (Variables|/Game/ResidentHorrorFPS/Character/BP_Character/BP_RHV_FPS_Player.BP_RHV_FPS_Player_C|GetBPC_Equipment (Variables|Reference|GetPlayer)))) (Utilities|Struct|BreakST_InteractionAnimation _interactanimation) (Utilities|Struct|BreakST_InteractionOffsets (.Interaction (Utilities|Struct|BreakST_ItemInformation (Variables|/Game/ResidentHorrorFPS/Blueprints/BP_ItemBase/DataAsset/PDA_InventoryItem.PDA_InventoryItem_C|GetItem%20Information (Variables|Default|GetPrymaryDataAsset))))))
        (:then
          (Rendering|SetRenderCustomDepth (Variables|Default|GetitemMesh) false)
          (Interactable|SetIkHandPosition)
          (Rendering|SetVisibility (Variables|Default|GetInteractWidget) false false)
          (Default|SaveData (Variables|Default|GetBP_SaveLoadRHFps) (Utilities|Struct|MakeST_SaveLoad true)))
        (:Interact
          (Interactable|AttachtoHand))
        (:false
          (Interactable|InteractionEnable true))
        (:Destroy
          (Actor|DestroyActor))))))

(event EventEndInteraction
  ;[0 0 0] Inveraction Item
)

(fn ConstructionScript
  (if (Variables|Information|GetRefresh)
    _
    (else
      _))
  (CallFunction|UpdateMesh)
  (Variables|Information|SetRefresh false)
  (if (Variables|/Game/ResidentHorrorFPS/Blueprints/BP_ItemBase/DataAsset/PDA_InventoryItem.PDA_InventoryItem_C|GetBrigtness%20Item? (Variables|Default|GetPrymaryDataAsset))
    (Rendering|Material|SetOverlayMaterial (Variables|Default|GetitemMesh) "/Game/ResidentHorrorFPS/Demo/Materials/M_ShinyOverlay.M_ShinyOverlay" :!class /Script/Engine.MeshComponent)
    (else
      (Rendering|Material|SetOverlayMaterial (Variables|Default|GetitemMesh) 0 :!class /Script/Engine.MeshComponent))))

(fn SetIkHandPosition
  (Variables|/Game/ResidentHorrorFPS/Character/BP_Character/ABP_RHPlayer.ABP_RHPlayer_C|SetHandLocationInteraction (Variables|/Game/ResidentHorrorFPS/Character/BP_Character/BP_RHV_FPS_Player.BP_RHV_FPS_Player_C|GetABP%20RHFPS (Variables|Reference|GetPlayer)) (Transformation|GetWorldLocation (Variables|Default|GetitemMesh))))

(fn InteractionEnable
  (params (Enable? :type Boolean))
  (Physics|SetSimulatePhysics (Variables|Default|GetitemMesh) Enable?)
  (Collision|SetActorEnableCollision Enable?)
  (return))

(fn AttachtoHand
  (bind _player (Variables|Reference|GetPlayer))
  (bind _prymarydataasset (Variables|Default|GetPrymaryDataAsset))
  (bind _bpc_equipment (Variables|/Game/ResidentHorrorFPS/Character/BP_Character/BP_RHV_FPS_Player.BP_RHV_FPS_Player_C|GetBPC_Equipment _player))
  (bind _item_information (Variables|/Game/ResidentHorrorFPS/Blueprints/BP_ItemBase/DataAsset/PDA_InventoryItem.PDA_InventoryItem_C|GetItem%20Information _prymarydataasset))
  (bind _interaction (Utilities|Struct|BreakST_ItemInformation _item_information))
  (bind _child_actor (Default|GetCurrentHandItem _bpc_equipment))
  (bind (_offsetrighthand _offsetlefthand) (Utilities|Struct|BreakST_InteractionOffsets _interaction))
  (bind _returnvalue (Utilities|IsValid _child_actor))
  (Transformation|AttachComponentToComponent (Variables|/Script/Engine.Character|GetMesh _player) (select _returnvalue "weapon_l" "weapon_r") "SnapToTarget" "SnapToTarget" "KeepRelative" true)
  (Transformation|SetRelativeTransform (Variables|Default|GetitemMesh) (select _returnvalue _offsetlefthand _offsetrighthand) false false)
  (Audio|PlaySoundatLocation "/Engine/VREditor/Sounds/UI/Object_PickUp.Object_PickUp" (Transformation|GetActorLocation) "0, 0, 0" 1.0 1.0 0.0 "/Game/ResidentHorrorFPS/Audio/Attenuation/Att_SA_SoundRHFPS.Att_SA_SoundRHFPS" 0 0 0)
  (return))

(fn GetPrimaryDataAsset
  (return (Variables|Default|GetPrymaryDataAsset)))

(fn UpdateMesh
  (bind _prymarydataasset (Variables|Default|GetPrymaryDataAsset)
    (:then
      (Components|StaticMesh|SetStaticMesh (Variables|Default|GetitemMesh) (Utilities|Struct|BreakST_ItemVisualization (Utilities|Struct|BreakST_ItemInformation (Variables|/Game/ResidentHorrorFPS/Blueprints/BP_ItemBase/DataAsset/PDA_InventoryItem.PDA_InventoryItem_C|GetItem%20Information _prymarydataasset)))))
    (:else)))

(fn AddtoInventory
  (bind _player (Variables|Reference|GetPlayer))
  (bind _prymarydataasset (Variables|Default|GetPrymaryDataAsset))
  (bind _bpc_equipment (Variables|/Game/ResidentHorrorFPS/Character/BP_Character/BP_RHV_FPS_Player.BP_RHV_FPS_Player_C|GetBPC_Equipment _player))
  (Variables|Default|GetItemObject
    (:then
      (bind _add_ (Default|AddItemforInventory _bpc_equipment (Variables|Default|GetItemObject) false))
      (return _add_))
    (:else
      (bind _returnvalue (Default|ConstructItemObject _bpc_equipment (Variables|/Game/ResidentHorrorFPS/Blueprints/BP_ItemBase/DataAsset/PDA_InventoryItem.PDA_InventoryItem_C|GetItemObjectClass _prymarydataasset) (Variables|/Game/ResidentHorrorFPS/Blueprints/BP_ItemBase/DataAsset/PDA_InventoryItem.PDA_InventoryItem_C|GetItem%20Information _prymarydataasset) _prymarydataasset))
      (bind _add__2 (Default|AddItemforInventory _bpc_equipment _returnvalue false))
      (return _add__2))))

(fn GetDroppedItemObject
  (return (Variables|Default|GetItemObject)))