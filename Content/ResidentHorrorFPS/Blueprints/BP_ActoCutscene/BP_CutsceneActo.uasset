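; Trigger actor that plays a one-shot level sequence cutscene when the player enters its box.
; On overlap it glides the capsule to an arrow marker while disabling input, stopping aiming, hiding the HUD and setting InCutscene for full-body animation.
; After the sequence's duration it restores control and HUD, then destroys itself.
; Separate timeline events shrink and restore the player's capsule and mesh offset, with no caller in this graph.
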(event OnComponentBeginOverlap(OverlapBoxPlaySequence)
  (params (OverlappedComponent :type Primitive%20Component%20Object%20Reference) (OtherActor :type Actor%20Object%20Reference) (OtherComp :type Primitive%20Component%20Object%20Reference) (OtherBodyIndex :type Integer) (bFromSweep :type Boolean) (SweepResult :type Hit%20Result%20Structure%20%28by%20ref%29))
  (bind _player (CallFunction|RHVFPSPlayerRef))
  (bind _position_player (Variables|Default|GetPosition%20Player))
  ;[0 0 0 0.5] Overlap Player
  (if (== OtherActor (Game|Player|GetPlayerPawn 0))
    (Utilities|FlowControl|Sequence
      (:then_0
        ;[0 0 0] Move to character Arrow
        (bind _output_get (Variables|Default|SetIn%20Cutscene? true))
        (Variables|/Game/ResidentHorrorFPS/Character/BP_Character/BP_RHV_FPS_Player.BP_RHV_FPS_Player_C|SetIn%20Cutscene? _player _output_get)
        (Components|MoveComponentTo (Variables|/Script/Engine.Character|GetCapsuleComponent _player) (Transformation|GetWorldLocation _position_player) (Transformation|GetWorldRotation _position_player) false true 1.0 false))
      (:then_1
        (CallFunction|DisableInputCreateCutscene))
      (:then_2
        (CallFunction|PlayCutscene)))))

(event Custom|Back%20Capsule
  ;[0 0 0 0.5] Decrise Capsule
  (bind _camlength (Timeline|Timeline ReverseFromEnd)
    (:Update
      (Transformation|SetRelativeLocation (Variables|/Script/Engine.Character|GetMesh (CallFunction|RHVFPSPlayerRef)) (Math|Vector|MakeVector 0.0 0.0 (Math|Float|Lerp -89.0 -55.0 _camlength)) false false)
      (Components|Capsule|SetCapsuleHalfHeight (Variables|/Script/Engine.Character|GetCapsuleComponent (CallFunction|RHVFPSPlayerRef)) (Math|Float|Lerp 9e+01 55.0 _camlength) true))))

(event Custom|Play%20Cutscene
  (bind _returnvalue (Game|GetPlayerController 0))
  (bind _player (CallFunction|RHVFPSPlayerRef))
  (bind _player_2 (CallFunction|RHVFPSPlayerRef))
  (bind _player_3 (CallFunction|RHVFPSPlayerRef))
  (bind _player_4 (CallFunction|RHVFPSPlayerRef))
  (bind _levelsequence_player (Variables|Default|GetLevelSequence%20Player))
  ;[0 0 0] Play Cutscene
  (if (Variables|/Game/ResidentHorrorFPS/Character/BP_Character/BP_RHV_FPS_Player.BP_RHV_FPS_Player_C|GetAiming _player_3)
    (Default|Disiring _player_3))
  (Sequencer|Player|Play _levelsequence_player :!class /Script/MovieScene.MovieSceneSequencePlayer)
  (Widget|SetVisibility (Variables|/Game/ResidentHorrorFPS/Character/BP_Character/BP_RHV_FPS_Player.BP_RHV_FPS_Player_C|GetWBP%20Main%20Hud _player_4) "Hidden")
  (Collision|SetCollisionEnabled (Variables|/Script/Engine.Character|GetCapsuleComponent _player_4) "QueryAndPhysics")
  (Variables|/Script/Engine.CameraComponent|SetbUsePawnControlRotation (Variables|/Game/ResidentHorrorFPS/Character/BP_Character/BP_RHV_FPS_Player.BP_RHV_FPS_Player_C|GetCamera (CallFunction|RHVFPSPlayerRef)) false)
  (Utilities|FlowControl|Delay (Class|TimeManagementBlueprintLibrary|ToSeconds(QualifiedFrameTime) (Media|MediaPlayer|GetDuration _levelsequence_player)))
  (Sequencer|Player|Stop (Variables|Default|GetLevelSequence%20Player) :!class /Script/MovieScene.MovieSceneSequencePlayer)
  (Widget|SetVisibility (Variables|/Game/ResidentHorrorFPS/Character/BP_Character/BP_RHV_FPS_Player.BP_RHV_FPS_Player_C|GetWBP%20Main%20Hud _player) "Visible")
  (Utilities|FlowControl|Sequence
    (:then_0
      (Collision|SetCollisionEnabled (Variables|/Script/Engine.Character|GetCapsuleComponent _player) "QueryAndPhysics")
      (bind _output_get (Variables|Default|SetIn%20Cutscene? false))
      (Variables|/Game/ResidentHorrorFPS/Character/BP_Character/BP_RHV_FPS_Player.BP_RHV_FPS_Player_C|SetIn%20Cutscene? _player_2 _output_get)
      (Input|EnableInput _player_2 _returnvalue)
      (Input|SetInputModeGameOnly _returnvalue false)
      (Variables|/Script/Engine.CameraComponent|SetbUsePawnControlRotation (Variables|/Game/ResidentHorrorFPS/Character/BP_Character/BP_RHV_FPS_Player.BP_RHV_FPS_Player_C|GetCamera (CallFunction|RHVFPSPlayerRef)) true))
    (:then_1
      (CallFunction|DestroyCutscene))))

(event Custom|Disable%20Input%20Create%20Cutscene
  ;[0 0 0 0.5] Disable Input Create Cutscene
  (bind (_outactor _returnvalue) (Sequencer|Player|CreateLevelSequencePlayer (Variables|Default|GetWhich%20cutscene?)))
  (Variables|Default|SetLevelSequence%20acto _outactor)
  (Variables|Default|SetLevelSequence%20Player _returnvalue)
  (Input|DisableInput (CallFunction|RHVFPSPlayerRef) (Game|GetPlayerController 0)))

(event Custom|Destroy%20Cutscene
  ;[0 0 0 0.5] Destroy Cutscene
  (Utilities|FlowControl|Delay 0.2)
  (Actor|DestroyActor))

(event Custom|Decrise%20Capsule
  ;[0 0 0 0.5] Decrise Capsule
  (bind _camlength (Timeline|Timeline PlayFromStart)
    (:Update
      (Transformation|SetRelativeLocation (Variables|/Script/Engine.Character|GetMesh (CallFunction|RHVFPSPlayerRef)) (Math|Vector|MakeVector 0.0 0.0 (Math|Float|Lerp -89.0 -55.0 _camlength)) false false)
      (Components|Capsule|SetCapsuleHalfHeight (Variables|/Script/Engine.Character|GetCapsuleComponent (CallFunction|RHVFPSPlayerRef)) (Math|Float|Lerp 9e+01 55.0 _camlength) true))))

(fn ConstructionScript
  (Development|SetHiddeninGame (Variables|Default|GetPosition%20Player) (not (Variables|Default|GetVisibility%20Arrow%20Position)) false))