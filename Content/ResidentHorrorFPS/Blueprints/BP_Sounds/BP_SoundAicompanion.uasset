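; BP_SoundAicompanion is an animation notify that plays a sound by random chance, named for the AI companion's sounds.
; When received, it compares ChanceDeTocarSom against a random integer from 0 to 100.
; If the chance value is higher, it plays SomParaTocar at the mesh component's world location with configurable attenuation and concurrency settings.
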(fn ReceivedNotify
  (params (MeshComp :type Skeletal%20Mesh%20Component%20Object%20Reference) (Animation :type Anim%20Sequence%20Base%20Object%20Reference) (EventReference :type Anim%20Notify%20Event%20Reference%20Structure%20%28by%20ref%29))
  (if (> (Variables|Default|GetChance%20de%20tocar%20som) (Math|Random|RandomIntegerinRange 0 100))
    (Audio|PlaySoundatLocation (Variables|Default|GetSom%20para%20tocar) (Transformation|GetWorldLocation MeshComp) "0, 0, 0" 1.0 1.0 0.0 (Variables|Default|GetConfig%20Attenuation) (Variables|Default|GetConfig%20Concurrency) 0 0)
    (return false)))