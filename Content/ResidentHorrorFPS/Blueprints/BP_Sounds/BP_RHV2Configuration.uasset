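; BP_RHV2Configuration is an animation notify that triggers chance-based effects, sound and camera shake during animations.
; When enabled, a percentage roll spawns a particle emitter attached to the mesh at a configurable point.
; A separate roll plays a sound at the mesh location with configurable attenuation and concurrency.
; The same sound roll fires a world camera shake centred on the first player's pawn, regardless of mesh distance.
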(fn ReceivedNotify
  (params (MeshComp :type Skeletal%20Mesh%20Component%20Object%20Reference) (Animation :type Anim%20Sequence%20Base%20Object%20Reference) (EventReference :type Anim%20Notify%20Event%20Reference%20Structure%20%28by%20ref%29))
  (if (Variables|EffectSpawn|GetSpawn%20Effects?)
    (if (> (Variables|Effectspawn|GetChance%20Spawn%20Effects) (Math|Random|RandomIntegerinRange 0 100))
      (Effects|SpawnEmitterAttached (Variables|Effectspawn|GetEffect%20spawn) MeshComp (Variables|EffectSpawn|GetAttach%20Point%20Name%20Effects) "0, 0, 0" (Variables|EffectSpawn|GetRotation%20Effects) (Variables|EffectSpawn|GetScale%20Effects))))
  (if (> (Variables|Default|GetA%20chance%20to%20play%20Sound) (Math|Random|RandomIntegerinRange 0 100))
    (Audio|PlaySoundatLocation (Variables|Default|GetSound%20Play) (Transformation|GetWorldLocation MeshComp) "0, 0, 0" (Variables|Default|GetVolume%20Sound) (Variables|Default|GetPitch%20Sound) 0.0 (Variables|Default|GetConfig%20Attenuation) (Variables|Default|GetConfig%20Concurrency) 0 0)
    (Camera|PlayWorldCameraShake (Variables|Default|GetShake) (Transformation|GetActorLocation (Game|Player|GetPlayerPawn 0)) 9999.0 9999.0)
    (return false)))