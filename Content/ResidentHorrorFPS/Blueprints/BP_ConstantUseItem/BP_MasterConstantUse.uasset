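; BP_MasterConstantUse is, by its name, the master Blueprint for constant-use items in a horror FPS.
; It stores an item object through SetItemObject and exposes getters for that object, an interact animation, a socket and a mesh.
; The socket and mesh getters return empty results, and Tick only calls the parent, so the class holds no use logic itself.
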(event EventBeginPlay)

(event Collision|EventActorBeginOverlap
  (params (OtherActor :type Actor%20Object%20Reference)))

(event EventTick
  (params (DeltaSeconds :type Float%20%28single-precision%29))
  (|CallParentFunction DeltaSeconds))

(event EventSetItemObject
  (params (ItemObject :type BP%20Item%20Object%20Object%20Reference))
  (Variables|Default|SetItemObject ItemObject))

(fn ConstructionScript)

(fn GetInteractAnimation
  (return (Variables|Default|GetInteract%20Animation)))

(fn GetInteractSocket
  (return "None"))

(fn GetItemObject
  (return (Variables|Default|GetItemObject)))

(fn GetMesh
  (return 0))