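; Base actor for single-use items, which plays the player's use animation and then destroys itself.
; PushItemObject looks up the item's data table row, holsters any held equipment, then plays paired character and item montage/animation, with sound on notify.
; The empty Use hook, presumably for child classes, fires on montage blend out.
; On completion it re-equips the previous item or resets the player's action state.
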(event EventBeginPlay
  ;[0 0 0 0.5] Begin Play
  (bind _player (Class|BPIPlayerReference|GetPlayer(Message) (Game|GetPlayerCharacter 0)))
  (Variables|Default|SetPlayer _player))

(event EventPushItemObject
  (params (ItemObject :type BP%20Item%20Object%20Object%20Reference))
  (bind _player (Variables|Default|GetPlayer))
  (bind _bpc_equipment (Variables|/Game/ResidentHorrorFPS/Character/BP_Character/BP_RHV_FPS_Player.BP_RHV_FPS_Player_C|GetBPC_Equipment _player))
  ;[0 0 0 0.5] Push Item object Usable
  (Variables|Default|SetItem%20Object ItemObject)
  (bind _output_get (Variables|Default|SetDataTableRowHandle (.Information (Utilities|Struct|BreakST_UsableInfo (Default|GetUsableInformation (Variables|Default|GetItem%20Object))))))
  (bind _returnvalue (Utilities|GetDataTableRow (.DataTable (Utilities|Struct|BreakDataTableRowHandle _output_get)) (.RowName (Utilities|Struct|BreakDataTableRowHandle _output_get)))
    (:then
      (Variables|Default|SetItemInfo _returnvalue)
      (Utilities|IsValid (Default|GetCurrentHandItem _bpc_equipment)
        (:Is%20Valid
          (Variables|Default|SetHandItemValid? true)
          (Animation|Montage|PlayMontage (Variables|/Script/Engine.Character|GetMesh (Variables|Default|GetPlayer)) (.Holster (Utilities|Struct|BreakST_Base_Info (.BaseInfo (Utilities|GetClassDefaults (.AsBP%20Master%20Constant%20Use (Utilities|Casting|CastToBP_MasterConstantUseClass (.UsableClass (Utilities|Struct|BreakST_UsableInfo (Default|GetUsableInformation (Variables|/Game/ResidentHorrorFPS/Blueprints/BP_Inventory/Inventory/Equipment/BPC_Equipment.BPC_Equipment_C|GetCurrentActivateEquipmentFromIndex _bpc_equipment))))))))))
            (:OnCompleted
              (Components|SkeletalMesh|SetSkeletalMeshAsset (Variables|Default|GetItemMesh) (.SkeletalMesh (Utilities|Struct|BreakST_UsableItemInfo (Variables|Default|GetItemInfo))) :!label _label)
              (Animation|Montage|PlayMontage (Variables|/Script/Engine.Character|GetMesh (Variables|Default|GetPlayer)) (.CharacterUsableMontage (Utilities|Struct|BreakST_UsableAnimation (.Animation (Utilities|Struct|BreakST_UsableItemInfo (Variables|Default|GetItemInfo)))))
                (:then
                  (Components|Animation|PlayAnimation (Variables|Default|GetItemMesh) (.ItemUsableAnimation (Utilities|Struct|BreakST_UsableAnimation (.Animation (Utilities|Struct|BreakST_UsableItemInfo (Variables|Default|GetItemInfo))))) false)
                  (Variables|/Game/ResidentHorrorFPS/Blueprints/BP_Inventory/Inventory/Equipment/BPC_Equipment.BPC_Equipment_C|SetUsableItemState? (Variables|/Game/ResidentHorrorFPS/Character/BP_Character/BP_RHV_FPS_Player.BP_RHV_FPS_Player_C|GetBPC_Equipment (Variables|Default|GetPlayer)) true)
                  (Default|UpdateActionState (Variables|Default|GetPlayer) "NewEnumerator5"))
                (:OnCompleted
                  (Variables|/Game/ResidentHorrorFPS/Blueprints/BP_Inventory/Inventory/Equipment/BPC_Equipment.BPC_Equipment_C|SetUsableItemState? (Variables|/Game/ResidentHorrorFPS/Character/BP_Character/BP_RHV_FPS_Player.BP_RHV_FPS_Player_C|GetBPC_Equipment (Variables|Default|GetPlayer)) false)
                  (if (Variables|Default|GetHandItemValid?)
                    (Utilities|FlowControl|Delay 0.2)
                    (Default|LoadCurrentEquip (Variables|/Game/ResidentHorrorFPS/Character/BP_Character/BP_RHV_FPS_Player.BP_RHV_FPS_Player_C|GetBPC_Equipment (Variables|Default|GetPlayer)))
                    (else
                      (Default|UpdateActionState (Variables|Default|GetPlayer) "NewEnumerator0")))
                  (Actor|DestroyActor))
                (:OnBlendOut
                  (CallFunction|Use))
                (:OnNotifyBegin
                  (Audio|SpawnSoundAttached (.SFX (Utilities|Struct|BreakST_UsableItemInfo (Variables|Default|GetItemInfo))) (Variables|Default|GetItemMesh) "Root" (Transformation|GetActorLocation) "0, 0, 0" "SnapToTarget" false 1.0 1.0 0.0 "/Game/ResidentHorrorFPS/Audio/Attenuation/att_Attenuation.att_Attenuation" 0))))
            (:OnBlendOut
              (Default|ClearHandItem (Variables|/Game/ResidentHorrorFPS/Character/BP_Character/BP_RHV_FPS_Player.BP_RHV_FPS_Player_C|GetBPC_Equipment (Variables|Default|GetPlayer))))))
        (:Is%20Not%20Valid
          (Variables|Default|SetHandItemValid? false)
          (goto _label))))
    (:RowNotFound
      (Actor|DestroyActor))))

(fn ConstructionScript)

(fn Use)

(fn HideInventory
  (bind _player (Variables|Default|GetPlayer))
  (bind _bpc_equipment (Variables|/Game/ResidentHorrorFPS/Character/BP_Character/BP_RHV_FPS_Player.BP_RHV_FPS_Player_C|GetBPC_Equipment _player))
  (if (Variables|/Game/ResidentHorrorFPS/Blueprints/BP_Inventory/Inventory/Equipment/BPC_Equipment.BPC_Equipment_C|GetInventoryOpen? _bpc_equipment)
    (Default|HideInventoryOnly _bpc_equipment)))