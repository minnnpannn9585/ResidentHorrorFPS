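; Puzzle interaction component that routes use actions to puzzle actors and relays input to security monitors.
; Use casts the hit actor, calling Use on a puzzle master with the player character, or caching padlock, security monitor and picture frame references.
; Camera input handlers forward movement, stop and camera-swap requests to the cached monitor after a validity check.
; The puzzle-completed function is an empty stub.
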(event EventBeginPlay)

(event EventTick
  (params (DeltaSeconds :type Float%20%28single-precision%29)))

(fn Use
  (params (HitActor :type Actor%20Object%20Reference) (Hit%20Component :type Primitive%20Component%20Object%20Reference))
  (bind _output_get (Variables|Reference|SetHit%20Actor HitActor))
  (bind _asbp_puzzle_master (Utilities|Casting|CastToBP_PuzzleMaster _output_get)
    (:then
      (Default|Use _asbp_puzzle_master (Game|GetPlayerCharacter 0)))
    (:CastFailed
      _))
  (bind _asbp_pad_lock (Utilities|Casting|CastToBP_PadLock (Variables|Reference|GetHit%20Actor))
    (:then
      (Variables|Reference|Setref%20Pad%20Lock _asbp_pad_lock))
    (:CastFailed
      _))
  (bind _asbp_security_monitor_01 (Utilities|Casting|CastToBP_SecurityMonitor01 (Variables|Reference|GetHit%20Actor))
    (:then
      (Variables|Reference|SetRef%20Security%20Monitor _asbp_security_monitor_01))
    (:CastFailed
      _))
  (bind _asbp_frame (Utilities|Casting|CastToBP_Frame (Variables|Reference|GetHit%20Actor))
    (:then
      (Variables|Default|SetAs%20BP%20Frame _asbp_frame))
    (:CastFailed
      (return))))

(fn CameraActionX/Y
  (params (Action%20Value%20X :type Float%20%28double-precision%29) (Action%20Value%20Y :type Float%20%28double-precision%29))
  (bind _ref_security_monitor (Variables|Reference|GetRef%20Security%20Monitor)
    (:then
      (Default|NewPlayerInput _ref_security_monitor Action%20Value%20X Action%20Value%20Y))
    (:else)))

(fn CameraStop
  (bind _ref_security_monitor (Variables|Reference|GetRef%20Security%20Monitor)
    (:then
      (Default|PlayerStopInput _ref_security_monitor))
    (:else)))

(fn SwitchCameras
  (bind _ref_security_monitor (Variables|Reference|GetRef%20Security%20Monitor)
    (:then
      (Default|SwapCamera _ref_security_monitor))
    (:else)))

(fn OnPuzzleCompleted)