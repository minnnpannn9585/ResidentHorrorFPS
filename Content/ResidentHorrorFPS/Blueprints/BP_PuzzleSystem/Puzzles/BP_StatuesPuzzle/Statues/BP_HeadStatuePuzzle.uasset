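; BP_HeadStatuePuzzle is a head statue in the statues puzzle that sinks slightly when the puzzle is completed.
; On completion it calls the parent handler, stores its location, and after a short delay a Timeline lerps it downward.
; The parent completion handler is called again when the Timeline finishes.
; BeginPlay and construction only call the parent, and a delayed completion trigger is left unconnected.
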(event EventBeginPlay
  ;[0 0 0 0.5] Begin Play
  (|CallParentFunction))

(event EventOnPuzzleCompletion
  ;[0 0 0 0.5] Completation Puzzle
  (|CallParentFunction)
  (Variables|Default|SetPreCompletionLoc (Transformation|GetActorLocation))
  (Utilities|FlowControl|Delay 1.0)
  (bind _newtrack_0 (Timeline|Timeline PlayFromStart)
    (:Update
      (Transformation|SetActorLocation (Math|Vector|Lerp(Vector) (Variables|Default|GetPreCompletionLoc) (- (Variables|Default|GetPreCompletionLoc) "0.000000,0.000000,10.000000") _newtrack_0) false false))
    (:Finished
      (|CallParentFunction))))

(fn ConstructionScript
  (|CallParentFunction))