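; Inventory item placement puzzle: interacting switches to a puzzle camera and opens the inventory for item selection.
; SMC_PuzzleItemRequirement child components define the required item tags, and each accepted item reveals its hidden mesh with a timeline slide-in.
; PuzzleSaveLoad persists remaining requirements, filled tags and solved state, restoring placed items on BeginPlay.
; Completion broadcasts an event and, when unlock actors are assigned, restores the player view and sends them auto-interaction.
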(event Custom|OnPuzzleCompletion
  (bind _interactionactorstounlock (Variables|Default|GetInteractionActorsToUnlock))
  ;[0 0 0 0.5] On Puzzle Completion
  (Default|CallOnPuzzleCompleted)
  (if (Utilities|Array|IsNotEmpty _interactionactorstounlock)
    (for _array_element _interactionactorstounlock
      _)
    (Utilities|FlowControl|Delay (Variables|Default|GetDelay%20Remove%20Camera))
    (CallFunction|RemoveCamera)
    (CallFunction|VisibilityWidgetChange true)
    (Class|BPIInteraction|Interaction(Message) _array_element 0 true)
    (Default|OpenedInvPuzzle (Variables|/Game/ResidentHorrorFPS/Blueprints/BP_Inventory/Inventory/Equipment/BPC_Equipment.BPC_Equipment_C|GetWBP%20Inventory%20Main (Variables|/Game/ResidentHorrorFPS/Character/BP_Character/BP_RHV_FPS_Player.BP_RHV_FPS_Player_C|GetBPC_Equipment (CallFunction|RHVFPSPlayerRef))) false)))

(event Custom|AnimateItem
  (params (Component :type Primitive%20Component%20Object%20Reference) (Offset :type Vector))
  (bind _relativelocation (Variables|/Script/Engine.SceneComponent|GetRelativeLocation Component))
  ;[0 0 0 0.5] Animation Item Attached Puzzle
  (Utilities|Map|Add (Variables|Default|GetItemsBeingAnimated) Component _relativelocation)
  (Variables|Default|SetCurrentAnimationItem _relativelocation)
  (if (not (Audio|Components|Audio|IsPlaying (Variables|Default|GetItemAnimationTL)))
    (Transformation|SetRelativeLocation Component (+ _relativelocation Offset) false false)
    (Development|SetHiddeninGame Component false false)
    (bind _newtrack_0 (Timeline|ItemAnimationTL PlayFromStart)
      (:Update
        (Transformation|SetRelativeLocation Component (Math|Vector|Lerp(Vector) (+ (Variables|Default|GetCurrentAnimationItem) Offset) (Variables|Default|GetCurrentAnimationItem) _newtrack_0) false false))
      (:Finished
        (Utilities|Map|Remove (Variables|Default|GetItemsBeingAnimated) Component)
        (Audio|PlaySoundatLocation (Variables|Default|GetSound%20Puzzle%20End) (Transformation|GetActorLocation) "0, 0, 0" 1.0 1.0 0.0 "/Game/ResidentHorrorFPS/Audio/Attenuation/Att_AtenuationAll.Att_AtenuationAll" 0 0 0)))))

(event Custom|Posses%20Camera
  ;[0 0 0] Posses Camera
  (Game|Player|SetViewTargetwithBlend (Game|GetPlayerController 0) (Components|GetOwner (Variables|Default|GetCamera)) 0.0 "VTBlend_Cubic" 1.0 false)
  (Widget|SetVisibility (Variables|/Game/ResidentHorrorFPS/Character/BP_Character/BP_RHV_FPS_Player.BP_RHV_FPS_Player_C|GetWBP%20Main%20Hud (CallFunction|RHVFPSPlayerRef)) "Hidden")
  (Rendering|SetActorHiddenInGame (Game|Player|GetPlayerPawn 0) true))

(event Custom|Remove%20Camera
  ;[0 0 0] Remove Camera
  (Widget|RemovefromParent (Variables|Default|GetWBP%20Close))
  (Game|Player|SetViewTargetwithBlend (Game|GetPlayerController 0) (Game|Player|GetPlayerPawn 0) 0.0 "VTBlend_Cubic" 0.0 false)
  (Widget|SetVisibility (Variables|/Game/ResidentHorrorFPS/Character/BP_Character/BP_RHV_FPS_Player.BP_RHV_FPS_Player_C|GetWBP%20Main%20Hud (CallFunction|RHVFPSPlayerRef)) "Visible")
  (Rendering|SetActorHiddenInGame (Game|Player|GetPlayerPawn 0) false)
  (CallFunction|VisibilityWidgetChange false))

(event Custom|OnPuzzleSaveLoad
  (params (Save%20Loaded%20Data :type ST%20Save%20Load%20Structure))
  (bind (_puzzlesavedatavalid _puzzlesolved _puzzleremainingrequirements _puzzlefilleditemtags) (Utilities|Struct|BreakST_SaveLoad Save%20Loaded%20Data))
  ;[0 0 0 0.5] Puzzle Save Load
  (if _puzzlesavedatavalid
    (Variables|PuzzleConfiguration|SetRequirements _puzzleremainingrequirements)
    (Variables|PuzzleRuntime|SetFilledItemTags _puzzlefilleditemtags)
    (Variables|Default|SetbSolved _puzzlesolved)
    (for _array_element _puzzlefilleditemtags
      (CallFunction|ShowItemMesh _array_element))))

(event EventBeginPlay
  ;[0 0 0 0.5] Begin Play Puzzle
  (|CallParentFunction)
  (for _array_element (Components|GetChildrenComponents (Variables|Default|GetStaticMesh) false)
    (bind _assmc_puzzle_item_requirement (Utilities|Casting|CastToSMC_PuzzleItemRequirement _array_element))
    (Utilities|IsValid (Variables|/Game/ResidentHorrorFPS/Blueprints/BP_PuzzleSystem/Puzzles/BP_StatuesPuzzle/SMC_PuzzleItemRequirement.SMC_PuzzleItemRequirement_C|GetItemDataAsset _assmc_puzzle_item_requirement)
      (:Is%20Valid
        (Utilities|Array|Add (Variables|PuzzleConfiguration|GetRequirements) (Utilities|Struct|MakeST_InventoryPuzzleRequirement 1 (.ItemTag (Utilities|Struct|BreakST_Tags (Utilities|Struct|BreakST_ItemInformation (Variables|/Game/ResidentHorrorFPS/Blueprints/BP_ItemBase/DataAsset/PDA_InventoryItem.PDA_InventoryItem_C|GetItem%20Information (Variables|/Game/ResidentHorrorFPS/Blueprints/BP_PuzzleSystem/Puzzles/BP_StatuesPuzzle/SMC_PuzzleItemRequirement.SMC_PuzzleItemRequirement_C|GetItemDataAsset _assmc_puzzle_item_requirement))))))))))
  ;[0 0 0 0.5] Loaded
  (EventDispatchers|BindEventtoLoadedData (Variables|Default|GetPuzzleSaveLoad) (delegate Custom|OnPuzzleSaveLoad))
  (Default|LoadeData (Variables|Default|GetPuzzleSaveLoad)))

(event EventInteraction
  (params (Player :type BP%20RHV%20FPS%20Player%20Object%20Reference) (AutoInteraction%28Non-Player%29 :type Boolean))
  ;[0 0 0 0.5] Start Interact
  (if (not (Variables|Default|GetbSolved))
    (Default|BeginPuzzleItemSelection (Actor|GetComponentbyClass Player "/Game/ResidentHorrorFPS/Blueprints/BP_Inventory/Inventory/BPC_Inventory.BPC_Inventory_C") self)
    (Default|ForceOpenInv Player)
    (Default|OpenedInvPuzzle (Variables|/Game/ResidentHorrorFPS/Blueprints/BP_Inventory/Inventory/Equipment/BPC_Equipment.BPC_Equipment_C|GetWBP%20Inventory%20Main (Variables|/Game/ResidentHorrorFPS/Character/BP_Character/BP_RHV_FPS_Player.BP_RHV_FPS_Player_C|GetBPC_Equipment (CallFunction|RHVFPSPlayerRef))) true)
    (CallFunction|PossesCamera)
    (CallFunction|VisibilityWidgetChange true)
    (bind _returnvalue (UserInterface|CreateWidget "/Game/ResidentHorrorFPS/Blueprints/WBP/WBP_ClosePuzzle.WBP_ClosePuzzle_C" 0 self))
    (bind _output_get (Variables|Default|SetWBP%20Close _returnvalue))
    (UserInterface|Viewport|AddtoViewport _output_get 0)))

(fn ConstructionScript
  (|CallParentFunction)
  (for _array_element (Components|GetChildrenComponents (Variables|Default|GetStaticMesh) false)
    (bind _assmc_puzzle_item_requirement (Utilities|Casting|CastToSMC_PuzzleItemRequirement _array_element))
    (Default|RefreshPreview _assmc_puzzle_item_requirement)))

(fn ShowItemMesh
  (params (Tag :type Gameplay%20Tag%20Structure))
  (bind _array_element (Utilities|Array|ForEachLoopwithBreak (Components|GetChildrenComponents (Variables|Default|GetStaticMesh) false) :!label _label)
    (:LoopBody
      (bind _assmc_puzzle_item_requirement (Utilities|Casting|CastToSMC_PuzzleItemRequirement _array_element))
      (bind _itemdataasset (Variables|/Game/ResidentHorrorFPS/Blueprints/BP_PuzzleSystem/Puzzles/BP_StatuesPuzzle/SMC_PuzzleItemRequirement.SMC_PuzzleItemRequirement_C|GetItemDataAsset _assmc_puzzle_item_requirement)
        (:then
          (if (== (.ItemTag (Utilities|Struct|BreakST_Tags (Utilities|Struct|BreakST_ItemInformation (Variables|/Game/ResidentHorrorFPS/Blueprints/BP_ItemBase/DataAsset/PDA_InventoryItem.PDA_InventoryItem_C|GetItem%20Information _itemdataasset)))) Tag)
            (if (Variables|/Script/Engine.SceneComponent|GetbHiddenInGame _assmc_puzzle_item_requirement)
              (CallFunction|AnimateItem _assmc_puzzle_item_requirement (Variables|/Game/ResidentHorrorFPS/Blueprints/BP_PuzzleSystem/Puzzles/BP_StatuesPuzzle/SMC_PuzzleItemRequirement.SMC_PuzzleItemRequirement_C|GetAnimationOffset _assmc_puzzle_item_requirement))
              (goto _label Break))))
        (:else)))
    (:Completed
      (return))))

(fn SavePuzzleState
  (Default|SaveData (Variables|Default|GetPuzzleSaveLoad) (Utilities|Struct|MakeST_SaveLoad 0 true (Variables|Default|GetbSolved) (Variables|PuzzleConfiguration|GetRequirements) (Variables|PuzzleRuntime|GetFilledItemTags))))

(fn BPITryAcceptInventoryItem
  (params (ItemObject :type BP%20Item%20Object%20Object%20Reference))
  (bind _tags (Default|GetTags ItemObject))
  (bind _itemtag (Utilities|Struct|BreakST_Tags _tags))
  (if (not (Variables|Default|GetbSolved))
    (bind _output_get (LocalVariables|SetLocalRequirements (Variables|PuzzleConfiguration|GetRequirements)))
    (bind (_array_element _array_index) (Utilities|Array|ForEachLoopwithBreak _output_get :!label _label)
      (:LoopBody
        (if (GameplayTags|MatchesTag _itemtag (Utilities|Struct|BreakST_InventoryPuzzleRequirement _array_element) true)
          (Utilities|Array|RemoveIndex (Variables|PuzzleConfiguration|GetRequirements) _array_index)
          (Utilities|Array|Add (Variables|PuzzleRuntime|GetFilledItemTags) _itemtag)
          (CallFunction|SavePuzzleState)
          (CallFunction|ShowItemMesh _itemtag)
          (Default|CallOnSlotFilled)
          (LocalVariables|SetItemAccepted true)
          (goto _label Break)))
      (:Completed
        (if (Utilities|Array|IsEmpty (Variables|PuzzleConfiguration|GetRequirements))
          (bind _output_get_2 (Variables|Default|SetbSolved true))
          (CallFunction|SavePuzzleState)
          (CallFunction|OnPuzzleCompletion)
          (return _output_get_2 true)
          (else
            (return (LocalVariables|GetItemAccepted) false)))))))