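; Security camera actor for the security monitor puzzle, a scene capture view the player can pan and tilt.
; On begin play it hides its camera mesh and deactivates the capture component.
; RotateCamera applies sensitivity-scaled input to the capture's relative pitch and yaw, clamped to rotation limits.
; Horizontal and vertical movement each lazily create a reusable 2D motor sound, which StopSound halts immediately when input ceases.
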(event Custom|RotateCamera
  (params (LeftRightValue :type Float%20%28double-precision%29) (UpDownValue :type Float%20%28double-precision%29))
  (bind _scenecapturecomponent2d (Variables|Default|GetSceneCaptureComponent2D))
  (bind _relativerotation (Variables|/Script/Engine.SceneComponent|GetRelativeRotation _scenecapturecomponent2d))
  ;[0.03504 0.03714 0.15 0.5] Pivots the security camera in relative space. Speed can be adjusted with sensitivity variables, and maximum pivots with the max rotation variables
  (Variables|Floats|SetHorizontalValue LeftRightValue)
  (Variables|Floats|SetVerticalValue UpDownValue)
  (Transformation|SetRelativeRotation (Variables|Default|GetSceneCaptureComponent2D) (Math|Rotator|MakeRotator 0.0 (Math|Float|Clamp(Float) (+ (.pitch _relativerotation) (* (Variables|Floats|GetVerticalValue) (Variables|Floats|GetVerticalSensitivity))) (Variables|Floats|GetMaxDownRotation) (Variables|Floats|GetMaxUpRotation)) (Math|Float|Clamp(Float) (+ (.yaw _relativerotation) (* (Variables|Floats|GetHorizontalValue) (Variables|Floats|GetHorizontalSensitivity))) (Variables|Floats|GetMaxLeftRotation) (Variables|Floats|GetMaxRightRotation))) false false)
  ;[0.1657 0.4547 0.5625 0.5] Depending on which direction the player is adjusting the camera, you can have a different sound play
  (if (>= (Math|Float|Absolute(Float) (Variables|Floats|GetHorizontalValue)) 0.1)
    (CallFunction|MovementSoundHorizontal))
  (if (>= (Math|Float|Absolute(Float) (Variables|Floats|GetVerticalValue)) 0.1)
    (CallFunction|MovementSoundVertical)))

(event Custom|MovementSoundVertical
  ;[0.1451 0.15 0.04098 0.5] We will create a sound 2D variable so that we can play it and immediately stop it whenever player input ceases
  (Utilities|IsValid (Variables|Default|GetSoundVertical)
    (:Is%20Valid
      (if (not (Audio|Components|Audio|IsPlaying (Variables|Default|GetSoundVertical)))
        (Audio|Components|Audio|Play (Variables|Default|GetSoundVertical) 0.0)))
    (:Is%20Not%20Valid
      (bind _returnvalue (Audio|CreateSound2D "/Game/ResidentHorrorFPS/Audio/Wavs/WAV_Light02.WAV_Light02" 0.75 1.0 0.0 0))
      (Variables|Default|SetSoundVertical _returnvalue))))

(event Custom|StopSound
  (bind _soundvertical (Variables|Default|GetSoundVertical))
  (bind _soundhorizontal (Variables|Default|GetSoundHorizontal))
  ;[0.15 0.08572 0.04903 0.5] Called whenever the player stops moving the camera. Immediately stop the movement sound
  (Utilities|IsValid _soundhorizontal
    (:Is%20Valid
      (if (Audio|Components|Audio|IsPlaying _soundhorizontal)
        (Audio|Components|Audio|Stop (Variables|Default|GetSoundHorizontal))))
    (:Is%20Not%20Valid
      _))
  (Utilities|IsValid _soundvertical
    (:Is%20Valid
      (if (Audio|Components|Audio|IsPlaying _soundvertical)
        (Audio|Components|Audio|Stop (Variables|Default|GetSoundVertical))))))

(event Custom|MovementSoundHorizontal
  ;[0.1451 0.15 0.04098 0.5] We will create a sound 2D variable so that we can play it and immediately stop it whenever player input ceases
  (Utilities|IsValid (Variables|Default|GetSoundHorizontal)
    (:Is%20Valid
      (if (not (Audio|Components|Audio|IsPlaying (Variables|Default|GetSoundHorizontal)))
        (Audio|Components|Audio|Play (Variables|Default|GetSoundHorizontal) 0.0)))
    (:Is%20Not%20Valid
      (bind _returnvalue (Audio|CreateSound2D "/Game/ResidentHorrorFPS/Audio/Wavs/WAV_Light02.WAV_Light02" 0.75 1.0 0.0 0))
      (Variables|Default|SetSoundHorizontal _returnvalue))))

(event EventBeginPlay
  ;[0.15 0.15 0.15 0.5] Begin Play
  (Development|SetHiddeninGame (Variables|Default|GetCamera1) true false)
  (Components|Activation|Deactivate (Variables|Default|GetSceneCaptureComponent2D)))

(fn ConstructionScript)