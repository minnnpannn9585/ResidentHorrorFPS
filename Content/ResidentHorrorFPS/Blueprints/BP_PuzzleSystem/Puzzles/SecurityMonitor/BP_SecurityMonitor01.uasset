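; Security monitor puzzle actor that lets the player view, rotate and cycle through linked security cameras.
; Use blends the view to the monitor, locks the player, shows controls and activates scene captures until exit.
; Only the current camera feeds the screen's dynamic material, through a render target sized by viewport and camera quality, checked each Tick.
; Damage explodes the monitor, shuts off captures and blocks further entry.
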(event Custom|NewPlayerInput
  (params (LeftRightValue :type Float%20%28double-precision%29) (UpDownValue :type Float%20%28double-precision%29))
  ;[0.1262 0.06321 0.15 0.5] Called from the player character. Finds the active camera, and calls the appropriate functions in that class
  (Default|RotateCamera (Utilities|Array|Get(acopy) (.LinkedCameras (Utilities|Struct|BreakST_SecuritySsttings (Variables|Default|GetSecuritySsttings))) (Variables|Default|GetCurrentCamera)) LeftRightValue UpDownValue))

(event Custom|Exit%20Camera
  (bind _securityssttings (Variables|Default|GetSecuritySsttings))
  (bind (_cameratransitionspeed _sounds) (Utilities|Struct|BreakST_SecuritySsttings _securityssttings))
  (Variables|/Game/ResidentHorrorFPS/Character/BP_Character/BP_RHV_FPS_Player.BP_RHV_FPS_Player_C|Setin%20Interaction? (CallFunction|RHVFPSPlayerRef) false)
  (Variables|Default|SetIn%20Camera%20Security? false)
  (CallFunction|VisibilityWidgetChange false)
  ;[0.15 0.04897 0.1343 0.5] After the player is done interacting, we want to blend back from the monitor camera to the characters camera
  (Game|Player|SetViewTargetwithBlend (Game|GetPlayerController 0) (Game|GetPlayerCharacter 0) _cameratransitionspeed "VTBlend_Linear" 0.0 false)
  (Audio|PlaySound2D (.CameraExitSound (Utilities|Struct|BreakST_SecuritySounds _sounds)) 0.5 1.0 0.03 0 0)
  (bind _wbp_controls_camera (Variables|Default|GetWBP%20Controls%20Camera)
    (:then
      (Widget|RemovefromParent _wbp_controls_camera))
    (:else
      _))
  (Pawn|Components|CharacterMovement|SetMovementMode (Variables|/Script/Engine.Character|GetCharacterMovement (Game|GetPlayerCharacter 0)) "MOVE_Walking" 0)
  (Input|ResetIgnoreLookInput (Game|GetPlayerController 0))
  (Rendering|SetActorHiddenInGame (CallFunction|RHVFPSPlayerRef) false)
  (Utilities|FlowControl|Sequence
    (:then_0
      (Utilities|FlowControl|Delay (.CameraTransitionSpeed (Utilities|Struct|BreakST_SecuritySsttings (Variables|Default|GetSecuritySsttings))))
      (Input|DisableInput (Game|GetPlayerController 0))
      (Variables|Default|SetIsInteracting false))
    (:then_1
      (Utilities|FlowControl|Delay 0.2)
      (for _array_element (Utilities|Struct|BreakST_SecuritySsttings (Variables|Default|GetSecuritySsttings))
        (Components|Activation|Deactivate (Variables|/Game/ResidentHorrorFPS/Blueprints/BP_PuzzleSystem/Puzzles/SecurityMonitor/BP_SecurityCamera.BP_SecurityCamera_C|GetSceneCaptureComponent2D _array_element))))))

(event Custom|SwapCamera
  (bind _returnvalue (Viewport|GetViewportSize))
  ;[0.15 0.15 0.15 0.5] SwapCamera
  ;[0.03902 0.15 0.08479 0.5] Clear previous cameras render target, as there is no need for it while on a different camera
  (Variables|/Script/Engine.SceneCaptureComponent2D|SetTextureTarget (Variables|/Game/ResidentHorrorFPS/Blueprints/BP_PuzzleSystem/Puzzles/SecurityMonitor/BP_SecurityCamera.BP_SecurityCamera_C|GetSceneCaptureComponent2D (Utilities|Array|Get(acopy) (.LinkedCameras (Utilities|Struct|BreakST_SecuritySsttings (Variables|Default|GetSecuritySsttings))) (Variables|Default|GetCurrentCamera))) 0)
  (Math|Integer|IncrementInt (Variables|Default|GetCurrentCamera)
    (:%20%20
      (if (>= (Variables|Default|GetCurrentCamera) (Utilities|Array|Length (Utilities|Struct|BreakST_SecuritySsttings (Variables|Default|GetSecuritySsttings))))
        (Variables|Default|SetCurrentCamera 0))
      ;[0.15 0.15 0.15 0.5] Create new render target for new camera with size set to viewport size multiplied by the quality parameter. Lower values of quality will increase performance at the cost of quality
      (bind _returnvalue_2 (Rendering|CreateRenderTarget2D (Math|Float|Truncate (* (.x _returnvalue) (Variables|/Game/ResidentHorrorFPS/Blueprints/BP_PuzzleSystem/Puzzles/SecurityMonitor/BP_SecurityCamera.BP_SecurityCamera_C|GetCameraQualityLevel (Utilities|Array|Get(acopy) (Utilities|Struct|BreakST_SecuritySsttings (Variables|Default|GetSecuritySsttings)) (Variables|Default|GetCurrentCamera))))) (Math|Float|Truncate (* (.y _returnvalue) (Variables|/Game/ResidentHorrorFPS/Blueprints/BP_PuzzleSystem/Puzzles/SecurityMonitor/BP_SecurityCamera.BP_SecurityCamera_C|GetCameraQualityLevel (Utilities|Array|Get(acopy) (Utilities|Struct|BreakST_SecuritySsttings (Variables|Default|GetSecuritySsttings)) (Variables|Default|GetCurrentCamera))))) "RTF_RGBA16f"))
      (Variables|Default|SetCamera_RT _returnvalue_2)
      (bind _output_get (Variables|/Script/Engine.SceneCaptureComponent2D|SetTextureTarget (Variables|/Game/ResidentHorrorFPS/Blueprints/BP_PuzzleSystem/Puzzles/SecurityMonitor/BP_SecurityCamera.BP_SecurityCamera_C|GetSceneCaptureComponent2D (Utilities|Array|Get(acopy) (Utilities|Struct|BreakST_SecuritySsttings (Variables|Default|GetSecuritySsttings)) (Variables|Default|GetCurrentCamera))) (Variables|Default|GetCamera_RT)))
      (Rendering|Material|SetTextureParameterValue (Variables|Default|GetCamera_MAT) "Texture" _output_get)
      (Audio|PlaySound2D (Utilities|Struct|BreakST_SecuritySounds (Utilities|Struct|BreakST_SecuritySsttings (Variables|Default|GetSecuritySsttings))) 1.0 1.0 0.0 0 0))))

(event Custom|PlayerStopInput
  ;[0.1262 0.06321 0.15 0.5] Called from the player character. Finds the active camera, and calls the appropriate functions in that class
  (Default|StopSound (Utilities|Array|Get(acopy) (.LinkedCameras (Utilities|Struct|BreakST_SecuritySsttings (Variables|Default|GetSecuritySsttings))) (Variables|Default|GetCurrentCamera))))

(event EventBeginPlay
  (bind _returnvalue (Viewport|GetViewportSize))
  (bind _securityssttings (Variables|Default|GetSecuritySsttings))
  (bind _linkedcameras (Utilities|Struct|BreakST_SecuritySsttings _securityssttings))
  (bind _output (Utilities|Array|Get(acopy) _linkedcameras))
  (bind _cameraqualitylevel (Variables|/Game/ResidentHorrorFPS/Blueprints/BP_PuzzleSystem/Puzzles/SecurityMonitor/BP_SecurityCamera.BP_SecurityCamera_C|GetCameraQualityLevel _output))
  ;[0.04945 0.05439 0.15 0.5] Initial setup. We will start off on the first camera in the linked cameras list
  (|CallParentFunction)
  (Utilities|IsValid (Utilities|Array|Get(acopy) (Utilities|Struct|BreakST_SecuritySsttings (Variables|Default|GetSecuritySsttings)))
    (:Is%20Valid
      (bind _returnvalue_2 (Rendering|Material|CreateDynamicMaterialInstance "/Game/ResidentHorrorFPS/Demo/Materials/M_Camera_MAT.M_Camera_MAT" "None" "None" :!class /Script/Engine.KismetMaterialLibrary))
      (Variables|Default|SetCamera_MAT _returnvalue_2)
      (Rendering|Material|SetMaterial (Variables|Default|GetPlane) 0 (Variables|Default|GetCamera_MAT))
      ;;[0.15 0.005469 0.005469 0.5] No remove DELAY
      (Utilities|FlowControl|Delay 0.2)
      (bind _returnvalue_3 (Rendering|CreateRenderTarget2D (Math|Float|Truncate (* (.x _returnvalue) _cameraqualitylevel)) (Math|Float|Truncate (* (.y _returnvalue) _cameraqualitylevel)) "RTF_RGBA16f"))
      (Variables|Default|SetCamera_RT _returnvalue_3)
      (bind _output_get (Variables|/Script/Engine.SceneCaptureComponent2D|SetTextureTarget (Variables|/Game/ResidentHorrorFPS/Blueprints/BP_PuzzleSystem/Puzzles/SecurityMonitor/BP_SecurityCamera.BP_SecurityCamera_C|GetSceneCaptureComponent2D (Utilities|Array|Get(acopy) (Utilities|Struct|BreakST_SecuritySsttings (Variables|Default|GetSecuritySsttings)))) (Variables|Default|GetCamera_RT)))
      (Rendering|Material|SetTextureParameterValue (Variables|Default|GetCamera_MAT) "Texture" _output_get)
      (Rendering|Material|SetScalarParameterValue (Variables|Default|GetCamera_MAT) "ScreenBrightness" (Variables|Default|GetScreenBrightness) :!class /Script/Engine.MaterialInstanceDynamic))))

(event EventTick
  (params (DeltaSeconds :type Float%20%28single-precision%29))
  (|CallParentFunction DeltaSeconds)
  (CallFunction|CheckViewportSize))

(event EventEventDamageRHFPS
  (params (Damage :type Float%20%28double-precision%29) (Hitresult :type Hit%20Result%20Structure) (Preparator :type Actor%20Object%20Reference))
  ;[0.15 0.15 0.15 0.5] Explode
  (Effects|SpawnEmitteratLocation "/Game/ResidentHorrorFPS/Demo/Realistic_Starter_VFX_Pack_Vol2/Particles/Explosion/P_Explosion_Side.P_Explosion_Side" (Transformation|GetActorLocation))
  (Variables|Default|SetDestroyed? true)
  (CallFunction|VisibilityWidgetChange true)
  (Utilities|FlowControl|Delay 0.2)
  (for _array_element (Utilities|Struct|BreakST_SecuritySsttings (Variables|Default|GetSecuritySsttings))
    (Components|Activation|Deactivate (Variables|/Game/ResidentHorrorFPS/Blueprints/BP_PuzzleSystem/Puzzles/SecurityMonitor/BP_SecurityCamera.BP_SecurityCamera_C|GetSceneCaptureComponent2D _array_element))
    (Rendering|Material|SetMaterial (Variables|Default|GetPlane) 0 "/Engine/EngineMeshes/BackgroundMaterial.BackgroundMaterial"))
  (Effects|SpawnEmitteratLocation "/Game/ResidentHorrorFPS/Demo/Realistic_Starter_VFX_Pack_Vol2/Particles/Explosion/P_Explosion_Smoke.P_Explosion_Smoke" (Transformation|GetActorLocation)))

(event EventUse
  (params (Player%20Character :type Character%20Object%20Reference) (Hit%20Comp :type Primitive%20Component%20Object%20Reference))
  (bind _securityssttings (Variables|Default|GetSecuritySsttings))
  (bind _securityssttings_2 (Variables|Default|GetSecuritySsttings))
  (bind (_cameratransitionspeed _sounds) (Utilities|Struct|BreakST_SecuritySsttings _securityssttings_2))
  (bind (_cameratransitionspeed_2 _sounds_2) (Utilities|Struct|BreakST_SecuritySsttings _securityssttings))
  (if (Variables|Default|GetIn%20Camera%20Security?)
    (Variables|/Game/ResidentHorrorFPS/Character/BP_Character/BP_RHV_FPS_Player.BP_RHV_FPS_Player_C|Setin%20Interaction? (CallFunction|RHVFPSPlayerRef) false)
    (Variables|Default|SetIn%20Camera%20Security? false)
    (CallFunction|VisibilityWidgetChange false)
    ;[0.15 0.04897 0.1343 0.5] After the player is done interacting, we want to blend back from the monitor camera to the characters camera
    (Game|Player|SetViewTargetwithBlend (Game|GetPlayerController 0) (Game|GetPlayerCharacter 0) _cameratransitionspeed "VTBlend_Linear" 0.0 false)
    (Audio|PlaySound2D (.CameraExitSound (Utilities|Struct|BreakST_SecuritySounds _sounds)) 0.5 1.0 0.03 0 0)
    (bind _wbp_controls_camera (Variables|Default|GetWBP%20Controls%20Camera)
      (:then
        (Widget|RemovefromParent _wbp_controls_camera))
      (:else
        _))
    (Pawn|Components|CharacterMovement|SetMovementMode (Variables|/Script/Engine.Character|GetCharacterMovement (Game|GetPlayerCharacter 0)) "MOVE_Walking" 0)
    (Input|ResetIgnoreLookInput (Game|GetPlayerController 0))
    (Rendering|SetActorHiddenInGame (CallFunction|RHVFPSPlayerRef) false)
    (Utilities|FlowControl|Sequence
      (:then_0
        (Utilities|FlowControl|Delay (.CameraTransitionSpeed (Utilities|Struct|BreakST_SecuritySsttings (Variables|Default|GetSecuritySsttings))))
        (Input|DisableInput (Game|GetPlayerController 0))
        (Variables|Default|SetIsInteracting false))
      (:then_1
        (Utilities|FlowControl|Delay 0.2)
        (for _array_element (Utilities|Struct|BreakST_SecuritySsttings (Variables|Default|GetSecuritySsttings))
          (Components|Activation|Deactivate (Variables|/Game/ResidentHorrorFPS/Blueprints/BP_PuzzleSystem/Puzzles/SecurityMonitor/BP_SecurityCamera.BP_SecurityCamera_C|GetSceneCaptureComponent2D _array_element)))))
    (elif (not (Variables|Default|GetDestroyed?))
      (Variables|Default|SetIn%20Camera%20Security? true)
      (bind _returnvalue (UserInterface|CreateWidget "/Game/ResidentHorrorFPS/Blueprints/WBP/WBP_ControlCamera.WBP_ControlCamera_C"))
      (bind _output_get (Variables|Default|SetWBP%20Controls%20Camera _returnvalue))
      (UserInterface|Viewport|AddtoViewport _output_get 0)
      ;[0.15 0.03359 0.03359 0.5] When the player interacts, we will transfer his camera to the monitor's camera, and we will disable the input, to prevent him from walking around the map while viewing the monitor
      (Rendering|SetActorHiddenInGame (CallFunction|RHVFPSPlayerRef) true)
      (Game|Player|SetViewTargetwithBlend (Game|GetPlayerController 0) self _cameratransitionspeed_2 "VTBlend_Linear" 0.0 false)
      (Audio|PlaySound2D (.CameraEnterSound (Utilities|Struct|BreakST_SecuritySounds _sounds_2)) 0.5 1.0 0.03 0 0)
      (CallFunction|VisibilityWidgetChange true)
      (Variables|/Game/ResidentHorrorFPS/Character/BP_Character/BP_RHV_FPS_Player.BP_RHV_FPS_Player_C|Setin%20Interaction? (CallFunction|RHVFPSPlayerRef) true)
      (Pawn|Components|CharacterMovement|DisableMovement (Variables|/Script/Engine.Character|GetCharacterMovement (Game|GetPlayerCharacter 0)))
      (Input|SetIgnoreLookInput (Game|GetPlayerController 0) false)
      (Utilities|FlowControl|Delay (.CameraTransitionSpeed (Utilities|Struct|BreakST_SecuritySsttings (Variables|Default|GetSecuritySsttings))))
      (Input|EnableInput (Game|GetPlayerController 0))
      (Variables|Default|SetIsInteracting true)
      (for _array_element_2 (Utilities|Struct|BreakST_SecuritySsttings (Variables|Default|GetSecuritySsttings))
        (Components|Activation|Activate (Variables|/Game/ResidentHorrorFPS/Blueprints/BP_PuzzleSystem/Puzzles/SecurityMonitor/BP_SecurityCamera.BP_SecurityCamera_C|GetSceneCaptureComponent2D _array_element_2) false)))))

(event Input|KeyboardEvents|E
  (params (Key :type Key%20Structure :default "None"))
  ;[0.15 0.15 0.15 0.5] Interact
  (:Pressed
    (CallFunction|ExitCamera)))

(fn ConstructionScript
  (|CallParentFunction))

(fn CheckViewportSize
  (bind _returnvalue (Viewport|GetViewportSize))
  (bind _currentcamera (Variables|Default|GetCurrentCamera))
  (bind _securityssttings (Variables|Default|GetSecuritySsttings))
  (bind _linkedcameras (Utilities|Struct|BreakST_SecuritySsttings _securityssttings))
  (bind _output (Utilities|Array|Get(acopy) _linkedcameras _currentcamera))
  (bind _cameraqualitylevel (Variables|/Game/ResidentHorrorFPS/Blueprints/BP_PuzzleSystem/Puzzles/SecurityMonitor/BP_SecurityCamera.BP_SecurityCamera_C|GetCameraQualityLevel _output))
  (bind _returnvalue_2 (* (.y _returnvalue) _cameraqualitylevel))
  (bind _returnvalue_3 (* (.x _returnvalue) _cameraqualitylevel))
  (bind _returnvalue_4 (Math|Float|Truncate _returnvalue_3))
  (bind _returnvalue_5 (Math|Float|Truncate _returnvalue_2))
  ;[0.15 0.15 0.15 0.5] Adjust the size of the render target if the players screen resolution has changed
  (bind _camera_rt (Variables|Default|GetCamera_RT)
    (:then
      (if (or (!= (Variables|/Script/Engine.TextureRenderTarget2D|GetSizeX _camera_rt) _returnvalue_4) (!= (Variables|/Script/Engine.TextureRenderTarget2D|GetSizeY _camera_rt) _returnvalue_5))
        (Rendering|ResizeRenderTarget2D (Variables|Default|GetCamera_RT) _returnvalue_4 _returnvalue_5)))
    (:else)))