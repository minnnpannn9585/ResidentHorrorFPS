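; BP_Gasolina is a gasoline pickup in the generator puzzle folder, adding fuel to the player's puzzle component when used.
; Use adds FuelLevel to the component's Gasoline, clamped to its range, plays a pickup sound, saves a collected flag and destroys the actor.
; On load, a set flag restores FuelLevel and destroys the actor again.
; An optional debug display draws the fuel amount above it each tick.
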(event LoadedData(BP_SaveLoadRHFps)
  (params (Save%20Loaded%20Data :type ST%20Save%20Load%20Structure))
  (bind (_boolean4 _float1) (Utilities|Struct|BreakST_SaveLoad Save%20Loaded%20Data))
  (if _boolean4
    (Variables|Default|SetFuelLevel _float1)
    (Actor|DestroyActor)))

(event EventBeginPlay
  (|CallParentFunction))

(event Collision|EventActorBeginOverlap
  (params (OtherActor :type Actor%20Object%20Reference))
  (|CallParentFunction OtherActor) ; This node is disabled and will not be called.\nDrag off pins to build functionality.
)

(event EventTick
  (params (DeltaSeconds :type Float%20%28single-precision%29))
  (|CallParentFunction DeltaSeconds)
  (CallFunction|Debugs))

(event EventUse
  (params (Player%20Character :type Character%20Object%20Reference))
  (bind _returnvalue (Actor|GetComponentbyClass Player%20Character "/Game/ResidentHorrorFPS/Blueprints/BP_PuzzleSystem/BPC_PuzzleComponent.BPC_PuzzleComponent_C"))
  (bind _fuellevel (Variables|Default|GetFuelLevel))
  (Utilities|IsValid _returnvalue
    (:Is%20Valid
      (Variables|/Game/ResidentHorrorFPS/Blueprints/BP_PuzzleSystem/BPC_PuzzleComponent.BPC_PuzzleComponent_C|Setgasoline _returnvalue (Math|Float|Clamp(Float) (+ (Variables|/Game/ResidentHorrorFPS/Blueprints/BP_PuzzleSystem/BPC_PuzzleComponent.BPC_PuzzleComponent_C|Getgasoline _returnvalue) _fuellevel) 0.0 1e+02))
      (Audio|PlaySound2D "/Engine/VREditor/Sounds/UI/Object_PickUp.Object_PickUp" 1.0 1.0 0.0 0 0)
      (Default|SaveData (Variables|Default|GetBP_SaveLoadRHFps) (Utilities|Struct|MakeST_SaveLoad true _fuellevel))
      (Actor|DestroyActor))))

(fn ConstructionScript
  (|CallParentFunction))

(fn Debugs
  ;[0.15 0.025 0.025 0.5 100] Debug
  (if (Variables|Default|GetDebug)
    (Rendering|Debug|DrawDebugString (CallFunction|RelativePositionSystem "0.000000,0.000000,30.000000" self 0.0) (Utilities|String|Append "FUEL: " (Utilities|String|ToString(Float) (Variables|Default|GetFuelLevel))) 0 "(R=0.169322,G=0.661458,B=0.165365,A=1.000000)")))