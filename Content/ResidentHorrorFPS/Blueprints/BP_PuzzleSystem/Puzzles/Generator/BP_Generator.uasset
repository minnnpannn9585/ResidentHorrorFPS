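; Fuel-powered generator puzzle actor that switches linked actors on while it runs.
; Use transfers gasoline from the player's BPC_PuzzleComponent, starting the generator at full fuel, or shows a failure widget and sound if none is carried.
; A looping timer drains and saves fuel, closing linked actors when empty; loading re-enters the same start or shutdown paths.
; An overlap sphere shows the fuel-bar widget.
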(event LoadedData(BP_SaveLoadRHFps)
  (params (Save%20Loaded%20Data :type ST%20Save%20Load%20Structure))
  (bind (_boolean2 _float1) (Utilities|Struct|BreakST_SaveLoad Save%20Loaded%20Data))
  ;[0 0 0 0.5 50] Load
  (if _boolean2
    (Utilities|FlowControl|Delay 1.0)
    (if (<= _float1 0.0)
      (CallFunction|OFFGenerator)
      (else
        (Variables|Default|SetFuelLevel _float1)
        (CallFunction|LoadStateGenerator)))))

(event OnComponentBeginOverlap(SphereBarGasoline)
  (params (OverlappedComponent :type Primitive%20Component%20Object%20Reference) (OtherActor :type Actor%20Object%20Reference) (OtherComp :type Primitive%20Component%20Object%20Reference) (OtherBodyIndex :type Integer) (bFromSweep :type Boolean) (SweepResult :type Hit%20Result%20Structure%20%28by%20ref%29))
  ;[0 0 0 0.5 50] Begin Overlap
  (CallFunction|ForceCreateWidgetBeginOveralp0 OtherActor))

(event OnComponentEndOverlap(SphereBarGasoline)
  (params (OverlappedComponent :type Primitive%20Component%20Object%20Reference) (OtherActor :type Actor%20Object%20Reference) (OtherComp :type Primitive%20Component%20Object%20Reference) (OtherBodyIndex :type Integer))
  ;[0 0 0 0.5 50] End Overlap
  (bind _wbp_bargasoline (Variables|Default|GetWBP%20BarGasoline)
    (:then
      (Widget|RemovefromParent _wbp_bargasoline)
      (Rendering|SetVisibility (Variables|Default|GetGasolineBar) false false))
    (:else)))

(event Custom|Timer
  (bind _output_get (Variables|Default|SetFuelLevel (Math|Float|Clamp(Float) (- (Variables|Default|GetFuelLevel) (Utilities|Time|GetWorldDeltaSeconds)) 0.0 1e+02)))
  (Utilities|Struct|SetmembersinST_SaveLoad (Variables|Default|GetObject%20Data) true _output_get)
  (Default|SaveData (Variables|Default|GetBP_SaveLoadRHFps) (Variables|Default|GetObject%20Data))
  (if (<= (Variables|Default|GetFuelLevel) 0.0)
    (Utilities|FlowControl|Sequence
      (:then_0
        (bind _refsound (Variables|Default|GetRefSound)
          (:then
            (Audio|Components|Audio|Stop _refsound)
            (Variables|Default|SetIsItOn? false)
            (Rendering|Components|Light|SetIntensity (Variables|Default|GetLightOn) 0.0)
            (Rendering|Components|Light|SetIntensity (Variables|Default|GetLightOn) 5e+03))
          (:else)))
      (:then_1
        (for _array_element (Utilities|Struct|BreakST_GeneratorSettings (Variables|Default|GetGeneratorSettings))
          (Default|Close/Off _array_element))))))

(event Custom|I%20am%20Gasolina
  (bind _generatorsettings (Variables|Default|GetGeneratorSettings))
  (bind _soundsettings (Utilities|Struct|BreakST_GeneratorSettings _generatorsettings))
  (bind (_soundfailedgenerator _attenuation _volume _pitchmultiplier) (Utilities|Struct|BreakST_SoundGenerator _soundsettings))
  ;[0.15 0.15 0.15 0.5] I am Gasolina
  (if (not (Variables|Default|GetIsItOn?))
    (bind _returnvalue (UserInterface|CreateWidget "/Game/ResidentHorrorFPS/Blueprints/BP_PuzzleSystem/Puzzles/Generator/WBP_IamGasoline.WBP_IamGasoline_C"))
    (UserInterface|Viewport|AddtoViewport _returnvalue 0)
    (Audio|SpawnSoundatLocation _soundfailedgenerator (CallFunction|RelativePositionSystem "0, 0, 0" self 0.0) "0, 0, 0" _volume _pitchmultiplier 0.0 _attenuation 0)))

(event Custom|Load%20State%20Generator
  (bind _generatorsettings (Variables|Default|GetGeneratorSettings))
  (bind _generatorsettings_2 (Variables|Default|GetGeneratorSettings))
  (bind (_actorstouse _generatorstartupdelay) (Utilities|Struct|BreakST_GeneratorSettings _generatorsettings_2))
  (bind _soundsettings (Utilities|Struct|BreakST_GeneratorSettings _generatorsettings))
  (bind (_soundofthegeneratorrunning _soundfailedgenerator _attenuation _volume _pitchmultiplier) (Utilities|Struct|BreakST_SoundGenerator _soundsettings))
  (Utilities|Time|SetTimerbyFunctionName 0 "Timer" (Utilities|Struct|BreakST_GeneratorSettings (Variables|Default|GetGeneratorSettings)) true)
  (Variables|Default|SetIsItOn? true)
  (CallFunction|VisibilityWidgetChange true)
  (Utilities|FlowControl|Sequence
    (:then_0
      (bind _returnvalue (Audio|SpawnSoundatLocation _soundofthegeneratorrunning (CallFunction|RelativePositionSystem "0, 0, 0" self 0.0) "0, 0, 0" _volume _pitchmultiplier 0.0 _attenuation 0))
      (Variables|Default|SetRefSound _returnvalue))
    (:then_1
      (Utilities|FlowControl|Delay _generatorstartupdelay)
      (for _array_element _actorstouse
        (Utilities|IsValid _array_element
          (:Is%20Valid
            (Default|Open/On _array_element)))))
    (:then_2
      (Rendering|Components|Light|SetIntensity (Variables|Default|GetLightOn) 5e+03)
      (Rendering|Components|Light|SetIntensity (Variables|Default|GetLightOff) 0.0))))

(event Custom|oFF%20Generator
  (Utilities|FlowControl|Sequence
    (:then_0
      (bind _refsound (Variables|Default|GetRefSound)
        (:then
          (Audio|Components|Audio|Stop _refsound)
          (Variables|Default|SetIsItOn? false)
          (Rendering|Components|Light|SetIntensity (Variables|Default|GetLightOn) 0.0)
          (Rendering|Components|Light|SetIntensity (Variables|Default|GetLightOn) 5e+03))
        (:else)))
    (:then_1
      (for _array_element (Utilities|Struct|BreakST_GeneratorSettings (Variables|Default|GetGeneratorSettings))
        (Default|Close/Off _array_element)))))

(event EventBeginPlay
  ;[0.15 0.15 0.15 0.5] Begin Play
  (|CallParentFunction)
  (Variables|Default|SetFuelLevel (Utilities|Struct|BreakST_GeneratorSettings (Variables|Default|GetGeneratorSettings))))

(event EventUse
  (params (Player%20Character :type Character%20Object%20Reference) (Hit%20Comp :type Primitive%20Component%20Object%20Reference))
  (bind _returnvalue (Actor|GetComponentbyClass Player%20Character "/Game/ResidentHorrorFPS/Blueprints/BP_PuzzleSystem/BPC_PuzzleComponent.BPC_PuzzleComponent_C"))
  (bind _generatorsettings (Variables|Default|GetGeneratorSettings))
  (bind _generatorsettings_2 (Variables|Default|GetGeneratorSettings))
  (bind (_actorstouse _generatorstartupdelay) (Utilities|Struct|BreakST_GeneratorSettings _generatorsettings_2))
  (bind _soundsettings (Utilities|Struct|BreakST_GeneratorSettings _generatorsettings))
  (bind (_soundofthegeneratorrunning _soundfailedgenerator _attenuation _volume _pitchmultiplier) (Utilities|Struct|BreakST_SoundGenerator _soundsettings))
  (Utilities|IsValid _returnvalue
    (:Is%20Valid
      (if (> (Variables|/Game/ResidentHorrorFPS/Blueprints/BP_PuzzleSystem/BPC_PuzzleComponent.BPC_PuzzleComponent_C|Getgasoline _returnvalue) 0.0)
        (Utilities|FlowControl|DoOnce false :!label _label
          (:Completed
            (Audio|PlaySoundatLocation "/Game/ResidentHorrorFPS/Audio/Wavs/WAV_Gasline.WAV_Gasline" (Transformation|GetActorLocation) "0, 0, 0" 1.0 1.0 0.0 "/Game/ResidentHorrorFPS/Audio/Attenuation/Att_AI.Att_AI" 0 0 0)
            (Variables|Default|SetFuelLevel (Math|Float|Clamp(Float) (+ (Variables|Default|GetFuelLevel) (Variables|/Game/ResidentHorrorFPS/Blueprints/BP_PuzzleSystem/BPC_PuzzleComponent.BPC_PuzzleComponent_C|Getgasoline _returnvalue)) 0.0 1e+02))
            (Variables|/Game/ResidentHorrorFPS/Blueprints/BP_PuzzleSystem/BPC_PuzzleComponent.BPC_PuzzleComponent_C|Setgasoline _returnvalue 0.0)
            (Utilities|FlowControl|Sequence
              (:then_0
                (goto _label Reset))
              (:then_1
                (if (>= (Variables|Default|GetFuelLevel) 1e+02)
                  (Utilities|Time|SetTimerbyFunctionName 0 "Timer" (Utilities|Struct|BreakST_GeneratorSettings (Variables|Default|GetGeneratorSettings)) true)
                  (Variables|Default|SetIsItOn? true)
                  (CallFunction|VisibilityWidgetChange true)
                  (Utilities|FlowControl|Sequence
                    (:then_0
                      (bind _returnvalue_2 (Audio|SpawnSoundatLocation _soundofthegeneratorrunning (CallFunction|RelativePositionSystem "0, 0, 0" self 0.0) "0, 0, 0" _volume _pitchmultiplier 0.0 _attenuation 0))
                      (Variables|Default|SetRefSound _returnvalue_2))
                    (:then_1
                      (Utilities|FlowControl|Delay _generatorstartupdelay)
                      (for _array_element _actorstouse
                        (Utilities|IsValid _array_element
                          (:Is%20Valid
                            (Default|Open/On _array_element)))))
                    (:then_2
                      (Rendering|Components|Light|SetIntensity (Variables|Default|GetLightOn) 5e+03)
                      (Rendering|Components|Light|SetIntensity (Variables|Default|GetLightOff) 0.0))))))))
        (else
          (CallFunction|IAmGasolina))))))

(event EventTick
  (params (DeltaSeconds :type Float%20%28single-precision%29))
  ;[0.15 0.15 0.15 0.5] Event Tick
  (|CallParentFunction DeltaSeconds)
  (CallFunction|Debugs))

(fn ConstructionScript
  (|CallParentFunction))

(fn Debugs
  ;[0.15 0.02805 0.02655 0.5 100] DEBUG
  (if (Variables|Default|GetDebug)
    (Rendering|Debug|DrawDebugString (CallFunction|RelativePositionSystem "0.000000,0.000000,150.000000" self 0.0) (Utilities|String|Append "FUEL LEVEL: " (Utilities|String|ToString(Float) (Variables|Default|GetFuelLevel))) 0 "(R=0.051413,G=0.661458,B=0.014367,A=1.000000)")
    (Rendering|Debug|DrawDebugString (CallFunction|RelativePositionSystem "0.000000,0.000000,170.000000" self 0.0) (Utilities|String|Append "IS IT ON: " (select (Variables|Default|GetIsItOn?) "YES" "FALSE")) 0 "(R=0.198993,G=0.225611,B=0.661458,A=1.000000)")))

(fn ForceCreateWidgetBeginOveralp0
  (params (PlayerRef :type Object%20Object%20Reference))
  (if (== PlayerRef (CallFunction|RHVFPSPlayerRef))
    (bind _returnvalue (UserInterface|CreateWidget "/Game/ResidentHorrorFPS/Blueprints/BP_PuzzleSystem/Puzzles/Generator/WBP_BarGasoline.WBP_BarGasoline_C" 0 self))
    (bind _output_get (Variables|Default|SetWBP%20BarGasoline _returnvalue))
    (Rendering|SetVisibility (Variables|Default|GetGasolineBar) true true)
    (UserInterface|SetWidget (Variables|Default|GetGasolineBar) _output_get)))