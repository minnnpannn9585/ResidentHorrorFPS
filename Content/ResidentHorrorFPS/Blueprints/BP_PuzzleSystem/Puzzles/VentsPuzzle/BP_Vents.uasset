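; Vent cover puzzle in which the player clicks out four screws to open the vent.
; Interaction blends the view to the actor, hides and freezes the player, enables mouse clicks and highlights screws until exit.
; Timelines unscrew each bolt one at a time before it drops with physics; the fourth swings the cover open and optionally calls OpenOn on linked actors.
; Screw states and count persist through the save component and are restored on load.
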(event OnClicked(StaticMesh2)
  (params (TouchedComponent :type Primitive%20Component%20Object%20Reference) (ButtonPressed :type Key%20Structure :default "None"))
  ;[0 0 0 0.5] Click Object
  (if (not (Variables|Default|GetIn%20drop?))
    (CallFunction|SmoothTimiline TouchedComponent TouchedComponent 29.50434 63.482237 9.744208)
    ;[0 0 0 0.5] Save
    (Utilities|Struct|SetmembersinST_SaveLoad (Variables|Default|GetObject%20Data) true)
    (Variables|Default|SetIn%20drop? true)
    ;[0 0 0 0.5] Importante Node Focus mouse
    (Class|GameplayStatics|SetViewportMouseCaptureMode "CapturePermanently_IncludingInitialMouseDown")
    ;[0 0 0 0.5] Sound
    (Audio|PlaySound2D "/Game/ResidentHorrorFPS/Audio/Wavs/WAV_Screw.WAV_Screw" 1.0 1.0 0.0 0 0)
    (Default|SaveData (Variables|Default|GetBP_SaveLoadRHFps) (Variables|Default|GetObject%20Data))))

(event OnClicked(StaticMesh1)
  (params (TouchedComponent :type Primitive%20Component%20Object%20Reference) (ButtonPressed :type Key%20Structure :default "None"))
  ;[0 0 0 0.5] Click Object
  (if (not (Variables|Default|GetIn%20drop?))
    (CallFunction|SmoothTimiline TouchedComponent TouchedComponent -29.385751 63.482238 9.744208)
    ;[0 0 0 0.5] Save
    (Utilities|Struct|SetmembersinST_SaveLoad (Variables|Default|GetObject%20Data) true)
    (Variables|Default|SetIn%20drop? true)
    ;[0 0 0 0.5] Importante Node Focus mouse
    (Class|GameplayStatics|SetViewportMouseCaptureMode "CapturePermanently_IncludingInitialMouseDown")
    ;[0 0 0 0.5] Sound
    (Audio|PlaySound2D "/Game/ResidentHorrorFPS/Audio/Wavs/WAV_Screw.WAV_Screw" 1.0 1.0 0.0 0 0)
    (Default|SaveData (Variables|Default|GetBP_SaveLoadRHFps) (Variables|Default|GetObject%20Data))))

(event OnClicked(StaticMesh3)
  (params (TouchedComponent :type Primitive%20Component%20Object%20Reference) (ButtonPressed :type Key%20Structure :default "None"))
  ;[0 0 0 0.5] Click Object
  (if (not (Variables|Default|GetIn%20drop?))
    (CallFunction|SmoothTimiline TouchedComponent TouchedComponent 28.93785 6.325915 9.744208)
    ;[0 0 0 0.5] Save
    (Utilities|Struct|SetmembersinST_SaveLoad (Variables|Default|GetObject%20Data) true)
    (Variables|Default|SetIn%20drop? true)
    ;[0 0 0 0.5] Importante Node Focus mouse
    (Class|GameplayStatics|SetViewportMouseCaptureMode "CapturePermanently_IncludingInitialMouseDown")
    ;[0 0 0 0.5] Sound
    (Audio|PlaySound2D "/Game/ResidentHorrorFPS/Audio/Wavs/WAV_Screw.WAV_Screw" 1.0 1.0 0.0 0 0)
    (Default|SaveData (Variables|Default|GetBP_SaveLoadRHFps) (Variables|Default|GetObject%20Data))))

(event OnClicked(StaticMesh4)
  (params (TouchedComponent :type Primitive%20Component%20Object%20Reference) (ButtonPressed :type Key%20Structure :default "None"))
  ;[0 0 0 0.5] Click Object
  (if (not (Variables|Default|GetIn%20drop?))
    (CallFunction|SmoothTimiline TouchedComponent TouchedComponent -29.053743 6.325915 9.744208)
    ;[0 0 0 0.5] Save
    (Utilities|Struct|SetmembersinST_SaveLoad (Variables|Default|GetObject%20Data) true)
    (Variables|Default|SetIn%20drop? true)
    ;[0 0 0 0.5] Importante Node Focus mouse
    (Class|GameplayStatics|SetViewportMouseCaptureMode "CapturePermanently_IncludingInitialMouseDown")
    ;[0 0 0 0.5] Sound
    (Audio|PlaySound2D "/Game/ResidentHorrorFPS/Audio/Wavs/WAV_Screw.WAV_Screw" 1.0 1.0 0.0 0 0)
    (Default|SaveData (Variables|Default|GetBP_SaveLoadRHFps) (Variables|Default|GetObject%20Data))))

(event LoadedData(BP_SaveLoadRHFps)
  (params (Save%20Loaded%20Data :type ST%20Save%20Load%20Structure))
  (bind (_boolean _boolean2 _boolean3 _boolean4 _integer1) (Utilities|Struct|BreakST_SaveLoad Save%20Loaded%20Data))
  ;[0 0 0 0.5] Load
  (Utilities|FlowControl|Delay 0.2)
  (Variables|Default|SetscrewsRemove _integer1)
  (if (Math|Boolean|ANDBoolean _boolean _boolean2 _boolean3 _boolean4)
    (Physics|SetSimulatePhysics (Variables|Default|GetStaticMesh1) true)
    (Utilities|FlowControl|Sequence
      (:then_0
        (Transformation|SetRelativeRotation (Variables|Default|GetVents) (Math|Rotator|MakeRotator 0.0 9e+01 0.0) false false))
      (:then_1
        (Utilities|FlowControl|Delay 0.6)
        (CallFunction|VisibilityWidgetChange true)))
    (else
      (if _boolean
        (Physics|SetSimulatePhysics (Variables|Default|GetStaticMesh1) true))
      (if _boolean2
        (Physics|SetSimulatePhysics (Variables|Default|GetStaticMesh2) true))
      (if _boolean3
        (Physics|SetSimulatePhysics (Variables|Default|GetStaticMesh3) true))
      (if _boolean4
        (Physics|SetSimulatePhysics (Variables|Default|GetStaticMesh4) true)))))

(event Custom|Open%20Interaction%20Inputs
  (params (Open? :type Boolean))
  (bind _player (CallFunction|RHVFPSPlayerRef))
  (bind _returnvalue (Game|GetPlayerController 0))
  (bind _returnvalue_2 (Game|GetPlayerController 0))
  ;[0 0 0 0.5] Open Interaction Inputs
  (if Open?
    ;[0 0 0 0.5] Open
    (Pawn|Components|CharacterMovement|DisableMovement (Variables|/Script/Engine.Character|GetCharacterMovement (Game|GetPlayerCharacter 0)))
    (Input|SetIgnoreLookInput _returnvalue true)
    (Variables|/Script/Engine.PlayerController|SetbShowMouseCursor _returnvalue true)
    (Input|EnableInput _returnvalue)
    (Variables|/Script/Engine.PlayerController|SetbEnableClickEvents _returnvalue true)
    (Game|Player|SetViewTargetwithBlend _returnvalue self 0.8 "VTBlend_Linear" 0.0 false)
    (CallFunction|VisibilityWidgetChange true)
    (Rendering|SetActorHiddenInGame _player true)
    (Collision|SetCollisionEnabled (Variables|/Script/Engine.Character|GetMesh _player) "NoCollision")
    (bind _returnvalue_3 (UserInterface|CreateWidget "/Game/ResidentHorrorFPS/Blueprints/WBP/WBP_DropObject.WBP_DropObject_C" 0 (Variables|Default|GetInteract%20Remove%20Object)))
    (bind _output_get (Variables|Default|SetWBP%20RemoveObject _returnvalue_3))
    (UserInterface|Viewport|AddtoViewport _output_get 0)
    (Variables|/Game/ResidentHorrorFPS/Character/BP_Character/BP_RHV_FPS_Player.BP_RHV_FPS_Player_C|Setin%20Interaction? (CallFunction|RHVFPSPlayerRef) true)
    (Rendering|Material|SetOverlayMaterial (Variables|Default|GetStaticMesh1) "/Game/ResidentHorrorFPS/Demo/Materials/M_ShinyOverlay.M_ShinyOverlay" :!class /Script/Engine.MeshComponent)
    (else
      ;[0 0 0 0.5] Close
      (Game|Player|SetViewTargetwithBlend (Game|GetPlayerController 0) (Game|Player|GetPlayerPawn 0) 0.8 "VTBlend_Linear" 0.0 false)
      (Input|ResetIgnoreLookInput _returnvalue_2)
      (Variables|/Script/Engine.PlayerController|SetbShowMouseCursor _returnvalue_2 false)
      (Input|DisableInput _returnvalue_2)
      (Variables|/Script/Engine.PlayerController|SetbEnableClickEvents _returnvalue_2 false)
      (Pawn|Components|CharacterMovement|SetMovementMode (Variables|/Script/Engine.Character|GetCharacterMovement (CallFunction|RHVFPSPlayerRef)) "MOVE_Walking" 0)
      (Input|SetInputModeGameOnly (Game|GetPlayerController 0) false)
      (if (Variables|Default|GetOpen?)
        (CallFunction|VisibilityWidgetChange true)
        (else
          (CallFunction|VisibilityWidgetChange false)))
      (Rendering|SetActorHiddenInGame (CallFunction|RHVFPSPlayerRef) false)
      (Collision|SetCollisionEnabled (Variables|/Script/Engine.Character|GetMesh (CallFunction|RHVFPSPlayerRef)) "QueryAndPhysics")
      (bind _wbp_removeobject (Variables|Default|GetWBP%20RemoveObject)
        (:then
          (Widget|RemovefromParent _wbp_removeobject)
          (Input|SetInputModeGameOnly (Game|GetPlayerController 0) false)
          (Variables|/Game/ResidentHorrorFPS/Character/BP_Character/BP_RHV_FPS_Player.BP_RHV_FPS_Player_C|Setin%20Interaction? (CallFunction|RHVFPSPlayerRef) false)
          (Rendering|Material|SetOverlayMaterial (Variables|Default|GetStaticMesh1) 0 :!class /Script/Engine.MeshComponent))
        (:else)))))

(event Custom|Reset%20Bolt
  ;[0 0 0 0.5] Smooth Timiline
  (Utilities|FlowControl|DoOnce false) ; enters at Reset
)

(event Custom|Smooth%20Timiline
  (params (Relative%20Location :type Scene%20Component%20Object%20Reference) (Physic :type Primitive%20Component%20Object%20Reference) (Location%20Y :type Float%20%28double-precision%29) (Location%20Z :type Float%20%28double-precision%29) (Final%20Value :type Float%20%28double-precision%29))
  ;[0 0 0 0.5] Smooth Timiline
  (Utilities|FlowControl|DoOnce false
    (:Completed
      (Utilities|FlowControl|Sequence
        (:then_0
          (bind _boltsmooth (Timeline|Timeline_0 PlayFromStart)
            (:Update
              (Transformation|SetRelativeRotation Relative%20Location (Math|Rotator|MakeRotator (Math|Float|Lerp 0.0 9e+01 _boltsmooth) 0.0 0.0) false false))))
        (:then_1
          (bind _boltsmooth_2 (Timeline|Timeline PlayFromStart)
            (:Update
              (Transformation|SetRelativeLocation Relative%20Location (Math|Vector|MakeVector (Math|Float|Lerp 4.090455 Final%20Value _boltsmooth_2) Location%20Y Location%20Z) false false))
            (:Finished
              (Utilities|FlowControl|Sequence
                (:then_0
                  (Physics|SetSimulatePhysics Physic true)
                  (CallFunction|ResetBolt)
                  (Variables|Default|SetscrewsRemove (+ (Variables|Default|GetscrewsRemove) 1))
                  (CallFunction|OpenVents)
                  (Utilities|Struct|SetmembersinST_SaveLoad (Variables|Default|GetObject%20Data) (Variables|Default|GetscrewsRemove))
                  (Default|SaveData (Variables|Default|GetBP_SaveLoadRHFps) (Variables|Default|GetObject%20Data)))
                (:then_1
                  (Utilities|FlowControl|Delay 0.5)
                  (Variables|Default|SetIn%20drop? false))))))))))

(event Custom|Open%20Vents
  (bind _st_ventspuzzle (Variables|Default|GetST%20VentsPuzzle))
  (bind _st_ventspuzzle_2 (Variables|Default|GetST%20VentsPuzzle))
  (bind (_activatepuzzle_ _actorstouse) (Utilities|Struct|BreakST_VentsPuzzle _st_ventspuzzle))
  (bind _soundsettings (Utilities|Struct|BreakST_VentsPuzzle _st_ventspuzzle_2))
  (bind (_soundremove _attenuation _volume _pitchmultiplier) (Utilities|Struct|BreakST_SoundVentsPuzzle _soundsettings))
  ;[0 0 0 0.5] Open Vents
  (if (>= (Variables|Default|GetscrewsRemove) 4)
    (Audio|PlaySoundatLocation _soundremove (Transformation|GetActorLocation) "0, 0, 0" _volume _pitchmultiplier 0.0 _attenuation 0 0 0)
    (Variables|Default|SetOpen? true)
    (bind _openvents (Timeline|Vents%20Open Play)
      (:Update
        (Transformation|SetRelativeRotation (Variables|Default|GetVents) (Math|Rotator|MakeRotator 0.0 (Math|Float|Lerp 0.0 9e+01 _openvents) 0.0) false false))
      (:Finished
        (CallFunction|OpenInteractionInputs false)
        (if _activatepuzzle_
          ;;[0.15 0.15 0.15 0.5] Complete the Puzzle
          (for _array_element _actorstouse
            (Utilities|IsValid _array_element
              (:Is%20Valid
                (Default|Open/On _array_element)))))))))

(event EventBeginPlay
  ;[0 0 0 0.5] Begin Play
  (|CallParentFunction))

(event EventTick
  (params (DeltaSeconds :type Float%20%28single-precision%29))
  ;[0 0 0 0.5] Event Tick
  (|CallParentFunction DeltaSeconds))

(event EventInteraction
  (params (Player :type BP%20RHV%20FPS%20Player%20Object%20Reference) (AutoInteraction%28Non-Player%29 :type Boolean))
  ;[0 0 0 0.5] Interact Start
  (CallFunction|OpenInteractionInputs true))

(event Input|KeyboardEvents|E
  (params (Key :type Key%20Structure :default "None"))
  ;[0 0 0 0.5] Exit Interaction
  (:Pressed
    (CallFunction|OpenInteractionInputs false)))

(fn ConstructionScript)