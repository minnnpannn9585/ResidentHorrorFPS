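; BP_Frame is a rotatable picture frame in a puzzle system.
; Use toggles a blended camera view of the frame, switching player movement and mouse cursor, and BeginPlay links its widget to it.
; RotateFrame turns the mesh a quarter turn via a timeline, then compares the step index to a target, except on wraparound, and notifies referenced actors of completion or incompletion.
; DoOnce gates block repeat triggers during transitions.
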(event Custom|RotateFrame
  (Utilities|FlowControl|DoOnce false
    (:Completed
      (bind _alpha (Timeline|FrameRotation PlayFromStart)
        (:Update
          (Transformation|SetRelativeRotation (Variables|Default|GetStaticMesh) (Math|Rotator|MakeRotator (Math|Float|Lerp (.roll (Variables|Default|GetPaintingRotation)) (- (.roll (Variables|Default|GetPaintingRotation)) 9e+01) _alpha) 0.0 0.0) false false))
        (:Finished
          (Variables|Default|SetPaintingRotation (Math|Rotator|MakeRotator (Math|Float|Lerp (.roll (Variables|Default|GetPaintingRotation)) (- (.roll (Variables|Default|GetPaintingRotation)) 9e+01) _alpha) 0.0 0.0))
          (CallFunction|ResetDoOnceFrame)
          (bind _result (Math|Integer|IncrementInt (Variables|Default|GetRotateIndex))
            (:%20%20
              (bind _output_get (Variables|Default|SetRotateIndex _result))
              (if (>= _output_get 4)
                (Variables|Default|SetRotateIndex 0)
                (elif (== (Variables|Default|GetTargetIndex) (Variables|Default|GetRotateIndex))
                  (Audio|PlaySound2D (Utilities|Struct|BreakST_FrameSounds (Utilities|Struct|BreakST_FrameSettings (Variables|Default|GetFrameSettings))) 1.0 1.0 0.0 0 0)
                  (for _array_element (Variables|Default|GetTest)
                    (Default|PuzzleFrameCompleted _array_element))
                  (else
                    (for _array_element_2 (Variables|Default|GetTest)
                      (Default|IncompletePuzzleFrame _array_element_2))))))))))))

(event Custom|Reset%20DoOnce%20Frame
  (Utilities|FlowControl|DoOnce false) ; enters at Reset
)

(event Custom|ResetDoOnce01
  (Utilities|FlowControl|DoOnce false) ; enters at Reset
)

(event Custom|ResetDoOnce02
  (Utilities|FlowControl|DoOnce false) ; enters at Reset
)

(event EventBeginPlay
  (|CallParentFunction)
  (Default|Initialize (.AsWBP%20Frame (Utilities|Casting|CastToWBP_Frame (UserInterface|GetUserWidgetObject (Variables|Default|GetWidget)))) self (Variables|Default|GetFrameSettings)))

(event Collision|EventActorBeginOverlap
  (params (OtherActor :type Actor%20Object%20Reference))
  (|CallParentFunction OtherActor) ; This node is disabled and will not be called.\nDrag off pins to build functionality.
)

(event EventTick
  (params (DeltaSeconds :type Float%20%28single-precision%29))
  (|CallParentFunction DeltaSeconds) ; This node is disabled and will not be called.\nDrag off pins to build functionality.
)

(event EventUse
  (params (Player%20Character :type Character%20Object%20Reference))
  (bind _framesettings (Variables|Default|GetFrameSettings))
  (bind _cameratransitionspeed (Utilities|Struct|BreakST_FrameSettings _framesettings))
  (Utilities|FlowControl|FlipFlop
    (:A
      (Utilities|FlowControl|DoOnce false
        (:Completed
          (Game|Player|SetViewTargetwithBlend (Game|GetPlayerController 0) self _cameratransitionspeed "VTBlend_Linear" 0.0 false)
          (Pawn|Components|CharacterMovement|DisableMovement (Variables|/Script/Engine.Character|GetCharacterMovement (Game|GetPlayerCharacter 0)))
          (Input|SetIgnoreLookInput (Game|GetPlayerController 0) false)
          (Input|EnableInput (Game|GetPlayerController 0) 0)
          (Utilities|FlowControl|Delay (.CameraTransitionSpeed (Utilities|Struct|BreakST_FrameSettings (Variables|Default|GetFrameSettings))))
          (CallFunction|ResetDoOnce02)
          (Variables|/Script/Engine.PlayerController|SetbShowMouseCursor (Game|GetPlayerController 0) true))))
    (:B
      (Utilities|FlowControl|DoOnce false
        (:Completed
          (Game|Player|SetViewTargetwithBlend (Game|GetPlayerController 0) (Game|GetPlayerCharacter 0) _cameratransitionspeed "VTBlend_Linear" 0.0 false)
          (Variables|/Script/Engine.PlayerController|SetbShowMouseCursor (Game|GetPlayerController 0) false)
          (Pawn|Components|CharacterMovement|SetMovementMode (Variables|/Script/Engine.Character|GetCharacterMovement (Game|GetPlayerCharacter 0)) "MOVE_Walking" 0)
          (Input|ResetIgnoreLookInput (Game|GetPlayerController 0))
          (Input|DisableInput (Game|GetPlayerController 0))
          (Utilities|FlowControl|Delay 0.2)
          (CallFunction|ResetDoOnce01))))))

(fn ConstructionScript
  (|CallParentFunction))