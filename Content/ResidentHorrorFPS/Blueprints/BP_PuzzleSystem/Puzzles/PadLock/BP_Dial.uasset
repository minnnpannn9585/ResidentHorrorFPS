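; BP_Dial is a single numbered dial of the padlock puzzle, with a WBP_Arrow widget that receives a reference to it on BeginPlay.
; RotateDial plays a sound and runs a timeline that turns the mesh one of ten 36-degree steps, blocking input until finished and wrapping at 360.
; FindNumber derives Number from the rotation and has the owning padlock check it after every turn.
; SetRandomNumber can randomize the starting position, though its event-graph call is unwired.
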(event Custom|FindNumber
  ;[0.15 0.15 0.15 0.5] NN REMOVA ESSE ++ PORQUE ELE TIRA UM BUG LOCO DE LOGICA DE CONTAGEM
  (bind _result (Math|Integer|IncrementInt (Math|Float|Truncate (/ (Variables|Default|GetDialRotation) 36.0)))
    (:%20%20
      (Variables|Default|SetNumber _result)
      (Default|CheckEveryTunr (Variables|Default|GetCadiadoRef)))))

(event Custom|RotateDial
  (bind _padlocksystem (Variables|Default|GetPadlockSystem))
  (bind _soundseffects (Utilities|Struct|BreakST_PadlockSettings _padlocksystem))
  (bind (_soundrotatedial _soundattenuation _volume _pitchmultiplier) (Utilities|Struct|BreakST_Sounds _soundseffects))
  (if (Variables|Default|GetCanRotate?)
    (Variables|Default|SetCanRotate? false)
    (Audio|PlaySoundatLocation _soundrotatedial (Transformation|GetWorldLocation (Variables|Default|GetSM_DIalV3)) "0, 0, 0" _volume _pitchmultiplier 0.0 _soundattenuation 0 0 0)
    (bind _alpha (Timeline|DialRotationTL PlayFromStart)
      (:Update
        (Transformation|SetRelativeRotation (Variables|Default|GetSM_DIalV3) (Math|Rotator|MakeRotator 0.0 0.0 (Math|Float|Lerp (Variables|Default|GetDialRotation) (+ (Variables|Default|GetDialRotation) 36.0) _alpha)) false false))
      (:Finished
        (Variables|Default|SetCanRotate? true)
        (Variables|Default|SetDialRotation (Math|Float|Lerp (Variables|Default|GetDialRotation) (+ (Variables|Default|GetDialRotation) 36.0) _alpha))
        (if (>= (Variables|Default|GetDialRotation) 3.6e+02)
          (Variables|Default|SetDialRotation 0.0)
          (Transformation|SetRelativeRotation (Variables|Default|GetSM_DIalV3) "0, 0, 0" false false)
          (CallFunction|FindNumber)
          (else
            (CallFunction|FindNumber)))))))

(event EventBeginPlay
  (bind _aswbp_arrow (Utilities|Casting|CastToWBP_Arrow (UserInterface|GetUserWidgetObject (Variables|Default|GetWidget))))
  (Default|Initialize _aswbp_arrow self))

(fn ConstructionScript)

(fn SetRandomNumber
  (bind _output_get (LocalVariables|SetLocalRotation (* (Math|Random|RandomIntegerinRange 0 9) 36.0)))
  (Variables|Default|SetDialRotation _output_get)
  (Transformation|SetRelativeRotation (Variables|Default|GetSM_DIalV3) (Math|Rotator|MakeRotator 0.0 0.0 (LocalVariables|GetLocalRotation)) false false)
  (CallFunction|FindNumber))