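; Base puzzle actor for the horror FPS, defining empty hook functions for use, open/on, close/off and puzzle frame completion states.
; Its sphere component filters overlaps to the local player character and forwards them to empty BeginOverlap and EndOverlap hooks.
; A Relative Position System helper computes a point from a target actor's location, an added offset and its scaled right vector.
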(event OnComponentBeginOverlap(Sphere)
  (params (OverlappedComponent :type Primitive%20Component%20Object%20Reference) (OtherActor :type Actor%20Object%20Reference) (OtherComp :type Primitive%20Component%20Object%20Reference) (OtherBodyIndex :type Integer) (bFromSweep :type Boolean) (SweepResult :type Hit%20Result%20Structure%20%28by%20ref%29))
  (if (== OtherActor (Game|GetPlayerCharacter 0))
    (Master|BeginOverlap)))

(event OnComponentEndOverlap(Sphere)
  (params (OverlappedComponent :type Primitive%20Component%20Object%20Reference) (OtherActor :type Actor%20Object%20Reference) (OtherComp :type Primitive%20Component%20Object%20Reference) (OtherBodyIndex :type Integer))
  (if (== OtherActor (Game|GetPlayerCharacter 0))
    (Master|EndOverlap)))

(event EventBeginPlay)

(event Collision|EventActorBeginOverlap
  (params (OtherActor :type Actor%20Object%20Reference)))

(event EventTick
  (params (DeltaSeconds :type Float%20%28single-precision%29)))

(fn ConstructionScript)

(fn Use
  (params (Player%20Character :type Character%20Object%20Reference) (Hit%20Comp :type Primitive%20Component%20Object%20Reference)))

(fn BeginOverlap)

(fn EndOverlap)

(fn RelativePositionSystem
  (params (B :type Vector) (Alvo :type Actor%20Object%20Reference) (B1 :type Float%20%28single-precision%29))
  (return (+ (* (Transformation|GetActorRightVector Alvo) B1) (+ (Transformation|GetActorLocation Alvo) B))))

(fn Open/On)

(fn Close/Off)

(fn PuzzleFrameCompleted)

(fn IncompletePuzzleFrame)