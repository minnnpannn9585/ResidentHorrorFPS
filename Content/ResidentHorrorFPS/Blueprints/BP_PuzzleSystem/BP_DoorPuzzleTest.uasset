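; BP_DoorPuzzleTest is a simple test door for the puzzle system that slides up when opened.
; The Open/On event plays a timeline that lerps the static mesh's relative Z from closed to a raised position.
; When the timeline finishes, the save/load component stores an opened flag, and its LoadedData event snaps the mesh open if that flag is set.
; BeginPlay also calls VisibilityWidgetChange with true.
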(event LoadedData(BP_SaveLoadRHFps)
  (params (Save%20Loaded%20Data :type ST%20Save%20Load%20Structure))
  ;[0 0 0 0.5] Load
  (if (Utilities|Struct|BreakST_SaveLoad Save%20Loaded%20Data)
    (Transformation|SetRelativeLocation (Variables|Default|GetStaticMesh) (Math|Vector|MakeVector 0.0 0.0 186.52245) false false)))

(event EventBeginPlay
  (CallFunction|VisibilityWidgetChange true))

(event Collision|EventActorBeginOverlap
  (params (OtherActor :type Actor%20Object%20Reference))
  (|CallParentFunction OtherActor) ; This node is disabled and will not be called.\nDrag off pins to build functionality.
)

(event EventTick
  (params (DeltaSeconds :type Float%20%28single-precision%29))
  (|CallParentFunction DeltaSeconds) ; This node is disabled and will not be called.\nDrag off pins to build functionality.
)

(event EventOpen/On
  ;[0 0 0 0.5] Simple Open Door
  (bind _open (Timeline|OpenDoorPadlock PlayFromStart)
    (:Update
      (Transformation|SetRelativeLocation (Variables|Default|GetStaticMesh) (Math|Vector|MakeVector 0.0 0.0 (Math|Float|Lerp 0.0 186.52245 _open)) false false))
    (:Finished
      ;;[0 0 0 0.5] Save
      (Default|SaveData (Variables|Default|GetBP_SaveLoadRHFps) (Utilities|Struct|MakeST_SaveLoad true)))))

(fn ConstructionScript
  (|CallParentFunction))