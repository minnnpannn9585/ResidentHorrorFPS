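; BP_Tutorials is a placeable trigger box, sized in the Construction Script, that shows a tutorial when the player overlaps it.
; It creates WBP_Tutorial with the configured text and media, then branches on TypeTutorial after disabling its own collision responses.
; Video tutorials slow time to near-freeze and big-screen ones pause the game, both enabling cursor and UI input.
; Warnings play an error sound and destroy the actor after a delay.
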(event OnComponentBeginOverlap(BoxOverlapTutorial)
  (params (OverlappedComponent :type Primitive%20Component%20Object%20Reference) (OtherActor :type Actor%20Object%20Reference) (OtherComp :type Primitive%20Component%20Object%20Reference) (OtherBodyIndex :type Integer) (bFromSweep :type Boolean) (SweepResult :type Hit%20Result%20Structure%20%28by%20ref%29))
  (bind _returnvalue (Game|GetPlayerController 0))
  (bind _returnvalue_2 (Game|GetPlayerController 0))
  ;[0 0 0 0.5] Overlap
  (if (== OtherActor (CallFunction|RHVFPSPlayerRef))
    ;[0 0 0 0.5] Create Widget
    (bind _returnvalue_3 (UserInterface|CreateWidget "/Game/ResidentHorrorFPS/Blueprints/BP_Tutorials/WBP_Tutorial.WBP_Tutorial_C" 0 self (Variables|Default|GetText%20Tutorial) (Utilities|Text|ToText(Name) (Variables|Default|GetText%20Tutorial%20Warning)) (Variables|TypeTutorial|GetMedia%20Playe) (Variables|TypeTutorial|GetVideo%20Origem)))
    (bind _output_get (Variables|Default|SetWBP%20Tutorial _returnvalue_3))
    (UserInterface|Viewport|AddtoViewport _output_get 0)
    ;[0 0 0 0.5] Verification Type Tutorial
    (if (Utilities|Enum|Equal(Enum) (Variables|TypeTutorial|GetType%20Tutorial) "NewEnumerator3")
      ;[0 0 0 0.5] Video tutorial
      (Input|SetInputModeGameandUI _returnvalue_2 (Variables|Default|GetWBP%20Tutorial) "DoNotLock" true false)
      (Variables|/Script/Engine.PlayerController|SetbShowMouseCursor _returnvalue_2 true)
      (Collision|SetCollisionResponsetoAllChannels (Variables|Default|GetBoxOverlapTutorial) "ECR_Ignore")
      (Audio|PlaySound2D "/Game/ResidentHorrorFPS/Audio/Wavs/WAV_SW_leave_Inventory.WAV_SW_leave_Inventory" 2.0 1.0 0.0 0 0)
      (Utilities|Time|SetGlobalTimeDilation 0.02)
      (elif (Utilities|Enum|Equal(Enum) (Variables|TypeTutorial|GetType%20Tutorial) "NewEnumerator2")
        ;[0 0 0 0.5] Warning Tutorial
        (Audio|PlaySound2D "/Game/ResidentHorrorFPS/Audio/Wavs/WAV_SW_item_error.WAV_SW_item_error" 2.0 1.0 0.0 0 0)
        (Collision|SetCollisionResponsetoAllChannels (Variables|Default|GetBoxOverlapTutorial) "ECR_Ignore")
        (Utilities|FlowControl|Delay (Variables|Default|GetTime%20Warning%20Tutorial))
        (Actor|DestroyActor)
        (else
          ;[0 0 0 0.5] Big Screen Tutorial
          (Input|SetInputModeGameandUI _returnvalue _output_get "DoNotLock" true false)
          (Variables|/Script/Engine.PlayerController|SetbShowMouseCursor _returnvalue true)
          (Collision|SetCollisionResponsetoAllChannels (Variables|Default|GetBoxOverlapTutorial) "ECR_Ignore")
          (Audio|PlaySound2D "/Game/ResidentHorrorFPS/Audio/Wavs/WAV_SW_leave_Inventory.WAV_SW_leave_Inventory" 2.0 1.0 0.0 0 0)
          (Game|SetGamePaused true))))))

(event EventBeginPlay)

(fn ConstructionScript
  (Components|Box|SetBoxExtent (Variables|Default|GetBoxOverlapTutorial) (Variables|TypeTutorial|GetSize) true))