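; BP_MenuCamera is the main menu camera, which opens the menu widget and serves as the player's view target.
; On BeginPlay it plays an optional opening sound and a camera shake from the DAMenuCustom settings, creates WBP_Menu and hides the cursor in game-only input mode.
; Its controller input setup adds the Enhanced Input mapping context for PC_ControllerMenu.
; NextCameraLoad hides the switch to the loading-screen camera behind a fade out and back in.
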(event Custom|Next%20Camera%20Load
  ;[0 0 0 0.5] Next Camera Load
  (CameraFades|StartCameraFade :self (Game|GetPlayerCameraManager 0) :ToAlpha 1.0 :Duration 0.3 :bHoldWhenFinished true)
  (Utilities|FlowControl|Delay 0.4)
  (Game|Player|SetViewTargetwithBlend (Game|GetPlayerController 0) (Components|GetOwner (Variables|/Script/Engine.Actor|GetRootComponent (Variables|Default|GetCamera%20Load%20Screen))) 0.0 "VTBlend_Cubic" 1.0 false)
  (CameraFades|StartCameraFade :self (Game|GetPlayerCameraManager 0) :FromAlpha 1.0 :Duration 1.0))

(event EventBeginPlay
  (bind _returnvalue (Game|GetPlayerController 0))
  ;[0 0 0 0.5] Begin Play
  (if (Variables|/Game/ResidentHorrorFPS/Blueprints/BP_MainMenu/Custom/DA_MenuCustom.DA_MenuCustom_C|GetPlay%20Audio%20When%20Opening%20the%20Menu? (Variables|Default|GetDA_MenuCustom))
    (Audio|PlaySound2D (Variables|/Game/ResidentHorrorFPS/Blueprints/BP_MainMenu/Custom/DA_MenuCustom.DA_MenuCustom_C|GetSound%20Open%20Menu%20 (Variables|Default|GetDA_MenuCustom)) 1.0 1.0 0.0 0 0))
  (bind _returnvalue_2 (UserInterface|CreateWidget "/Game/ResidentHorrorFPS/Blueprints/BP_MainMenu/WBP/WBP_Menu.WBP_Menu_C"))
  (bind _output_get (Variables|Default|SetWB%20menu _returnvalue_2))
  (UserInterface|Viewport|AddtoViewport _output_get 0)
  (Camera|PlayWorldCameraShake (Variables|/Game/ResidentHorrorFPS/Blueprints/BP_MainMenu/Custom/DA_MenuCustom.DA_MenuCustom_C|GetCamera%20shake (Variables|Default|GetDA_MenuCustom)) (Transformation|GetActorLocation (Game|GetPlayerCameraManager 0)) 6e+02 6e+02)
  (Variables|/Script/Engine.PlayerController|SetbShowMouseCursor _returnvalue false)
  (Input|SetInputModeGameOnly _returnvalue false)
  (Game|Player|SetViewTargetwithBlend (Game|GetPlayerController 0) self 0.0 "VTBlend_Linear" 0.0 false)
  (|Controllerinput))

(fn ConstructionScript)