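; Game instance for Resident Horror that owns player options and save games, carrying game state across level loads.
; Options live in a lazily loaded SV_Options save; audio applies through sound mix overrides, graphics through GameUserSettings, and mouse sensitivity and inversion by rewriting input axis mappings.
; Slot saves bundle the map, location-keyed object data, music state and staged inventory, and record the Continue slot globally.
; Loading restores these and opens the saved level.
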(event EventInit
  ;[0 0 0] Reload audio settings
  (bind _sv_options (Utilities|LoadOptionsSave)
    (:OutputPin
      (Variables|Default|SetSV%20Options _sv_options)
      (|Reloadaudiosettings))))

(event EventApplyGraphicsSettings
  (params (anti%20aliasing :type Integer) (shadow%20quality :type Integer) (texture%20quality :type Integer) (foliage%20quality :type Integer) (post%20process%20quality :type Integer) (view%20distance :type Integer) (vsync :type Boolean))
  ;[0 0 0] Graphics settings
  (bind _returnvalue (Settings|GetGameUserSettings))
  (Class|GameUserSettings|SetAntiAliasingQuality _returnvalue anti%20aliasing)
  (Class|GameUserSettings|SetShadowQuality _returnvalue shadow%20quality)
  (Class|GameUserSettings|SetTextureQuality _returnvalue texture%20quality)
  (Class|GameUserSettings|SetFoliageQuality _returnvalue foliage%20quality)
  (Class|GameUserSettings|SetPostProcessingQuality _returnvalue post%20process%20quality)
  (Class|GameUserSettings|SetViewDistanceQuality _returnvalue view%20distance)
  (Class|GameUserSettings|SetVSyncEnabled _returnvalue vsync)
  (Class|GameUserSettings|ApplySettings _returnvalue true))

(event EventSaveAudioSettings
  (params (master%20vol :type Float%20%28double-precision%29) (music%20vol :type Float%20%28double-precision%29) (sfx%20vol :type Float%20%28double-precision%29) (voice%20vol :type Float%20%28double-precision%29) (audio%20language :type Integer) (subtitle%20language :type Integer) (subtitle%20enabled :type Integer))
  (bind _sv_options (Variables|Default|GetSV%20Options))
  ;[0 0 0] Save Audio Settings
  (Audio|SetSoundMixClassOverride 0 0 master%20vol 1.0 0.0 true)
  (Audio|SetSoundMixClassOverride "/Game/ResidentHorrorFPS/Blueprints/BP_BaseSoundClassMix/Mix/SCM_RHV2.SCM_RHV2" "/Engine/EngineSounds/Music.Music" music%20vol 1.0 0.0 true)
  (Audio|SetSoundMixClassOverride "/Game/ResidentHorrorFPS/Blueprints/BP_BaseSoundClassMix/Mix/SCM_RHV2.SCM_RHV2" "/Game/ResidentHorrorFPS/Blueprints/BP_BaseSoundClassMix/Mix/SC_SoundEffectsRHV2.SC_SoundEffectsRHV2" sfx%20vol 1.0 0.0 true)
  (Audio|SetSoundMixClassOverride "/Game/ResidentHorrorFPS/Blueprints/BP_BaseSoundClassMix/Mix/SCM_RHV2.SCM_RHV2" "/Game/ResidentHorrorFPS/Blueprints/BP_BaseSoundClassMix/Mix/SC_VoiceRHV2.SC_VoiceRHV2" voice%20vol 1.0 0.0 true)
  (Utilities|LoadOptionsSave
    (:OutputPin
      ;;[0.1392 0.2656 0.09953] Volumes
      (Variables|/Game/ResidentHorrorFPS/Blueprints/BP_MainMenu/SaveBase/SV_Options.SV_Options_C|Setmaster%20vol _sv_options master%20vol)
      (Variables|/Game/ResidentHorrorFPS/Blueprints/BP_MainMenu/SaveBase/SV_Options.SV_Options_C|Setmusic%20vol _sv_options music%20vol)
      (Variables|/Game/ResidentHorrorFPS/Blueprints/BP_MainMenu/SaveBase/SV_Options.SV_Options_C|Setsfx%20vol _sv_options sfx%20vol)
      (Variables|/Game/ResidentHorrorFPS/Blueprints/BP_MainMenu/SaveBase/SV_Options.SV_Options_C|Setvoice%20vol _sv_options voice%20vol)
      ;;[0.1392 0.2656 0.09953] Language and Subtitle
      (Variables|/Game/ResidentHorrorFPS/Blueprints/BP_MainMenu/SaveBase/SV_Options.SV_Options_C|Setaudio%20language _sv_options audio%20language)
      (Variables|/Game/ResidentHorrorFPS/Blueprints/BP_MainMenu/SaveBase/SV_Options.SV_Options_C|Setsubtitle%20language _sv_options subtitle%20language)
      (Variables|/Game/ResidentHorrorFPS/Blueprints/BP_MainMenu/SaveBase/SV_Options.SV_Options_C|Setsubtitle%20enabled _sv_options subtitle%20enabled)
      (CallFunction|SaveOptions))))

(event EventSaveGamePlayOptions
  (params (difficuluty%20level :type Integer) (aiming%20mode :type Boolean) (auto%20reload :type Boolean) (invert%20mouse%20Y%20 :type Boolean) (mouse%20sensitivity%20X :type Float%20%28double-precision%29) (mouse%20sensitivity%20Y :type Float%20%28double-precision%29))
  ;[0 0 0 0.5] Save play opotions
  (Utilities|LoadOptionsSave
    (:OutputPin
      (Variables|/Game/ResidentHorrorFPS/Blueprints/BP_MainMenu/SaveBase/SV_Options.SV_Options_C|Setdifficulty (Variables|Default|GetSV%20Options) difficuluty%20level)
      (Variables|/Game/ResidentHorrorFPS/Blueprints/BP_MainMenu/SaveBase/SV_Options.SV_Options_C|Setaiming%20mode (Variables|Default|GetSV%20Options) aiming%20mode)
      (Variables|/Game/ResidentHorrorFPS/Blueprints/BP_MainMenu/SaveBase/SV_Options.SV_Options_C|Setauto%20reload (Variables|Default|GetSV%20Options) auto%20reload)
      (CallFunction|MouseYUpdate (Variables|Default|GetSV%20Options) mouse%20sensitivity%20Y invert%20mouse%20Y%20)
      (CallFunction|MouseXUpdate mouse%20sensitivity%20X (Variables|Default|GetSV%20Options))
      (CallFunction|SaveOptions))))

(fn SaveOptions
  (SaveGame|SaveGametoSlot (Variables|Default|GetSV%20Options) (Variables|Default|Getoption%20save%20slot)))

(fn MouseYUpdate
  (params (sv%20options :type SV%20Options%20Object%20Reference) (mouse%20y%20sensitivity :type Float%20%28double-precision%29) (invert%20mouse%20axis :type Boolean))
  (bind _output_get (Variables|/Game/ResidentHorrorFPS/Blueprints/BP_MainMenu/SaveBase/SV_Options.SV_Options_C|Setinvert%20mouse%20axis sv%20options invert%20mouse%20axis))
  (bind _output_get_2 (Variables|/Game/ResidentHorrorFPS/Blueprints/BP_MainMenu/SaveBase/SV_Options.SV_Options_C|Setmouse%20y%20sensitivity sv%20options mouse%20y%20sensitivity))
  (bind _output_get_3 (LocalVariables|SetLookUp%20mappings (Class|InputSettings|GetAxisMappingbyName (Class|InputSettings|GetInputSettings) "LookUp")))
  (for _array_element _output_get_3
    (Class|InputSettings|RemoveAxisMapping (Class|InputSettings|GetInputSettings) _array_element true)
    (bind _structout (Utilities|Struct|SetmembersinInputAxisKeyMapping _array_element (* (Math|Float|Clamp(Float) (* _output_get_2 2.0) 0.1 2.0) (Math|Float|SelectFloat 1.0 -1.0 _output_get))))
    (Class|InputSettings|AddAxisMapping (Class|InputSettings|GetInputSettings) _structout true)))

(fn MouseXUpdate
  (params (mouse%20x%20sensitivity :type Float%20%28double-precision%29) (sv%20options :type SV%20Options%20Object%20Reference))
  (bind _returnvalue (Class|InputSettings|GetInputSettings))
  (bind _output_get (Variables|/Game/ResidentHorrorFPS/Blueprints/BP_MainMenu/SaveBase/SV_Options.SV_Options_C|Setmouse%20x%20sensitivity sv%20options mouse%20x%20sensitivity))
  (bind _output_get_2 (LocalVariables|SetTurn%20settings (Class|InputSettings|GetAxisMappingbyName _returnvalue "Turn")))
  (for _array_element _output_get_2
    (Class|InputSettings|RemoveAxisMapping _returnvalue _array_element true)
    (bind _structout (Utilities|Struct|SetmembersinInputAxisKeyMapping _array_element (Math|Float|Clamp(Float) (* _output_get 2.0) 0.1 2.0)))
    (Class|InputSettings|AddAxisMapping _returnvalue _structout true)))

(fn SaveGameResidentHorror
  (params (Slot :type Integer) (Slot%20Info :type ST%20Load%20Slots%20Structure))
  (bind _returnvalue (SaveGame|CreateSaveGameObject "/Game/ResidentHorrorFPS/Blueprints/BP_SaveSystem/BP_SaveGameResidentHorror.BP_SaveGameResidentHorror_C"))
  (Variables|Default|SetActive%20Save%20Game%20object _returnvalue)
  (bind _returnvalue_2 (Game|GetCurrentLevelName true))
  (Variables|/Game/ResidentHorrorFPS/Blueprints/BP_SaveSystem/BP_SaveGameResidentHorror.BP_SaveGameResidentHorror_C|SetCurrent%20Map (Variables|Default|GetActive%20Save%20Game%20object) (Utilities|String|StringToName _returnvalue_2))
  (Variables|/Game/ResidentHorrorFPS/Blueprints/BP_SaveSystem/BP_SaveGameResidentHorror.BP_SaveGameResidentHorror_C|SetObjectSaveData (Variables|Default|GetActive%20Save%20Game%20object) (Variables|Map|GetObjectSaveData))
  (LocalVariables|SetLocal%20save%20slots (Variables|/Game/ResidentHorrorFPS/Blueprints/BP_SaveSystem/BP_SaveGameResidentHorror.BP_SaveGameResidentHorror_C|GetSaveSlotsInfo (Variables|Default|GetActive%20Save%20Game%20object)))
  (Utilities|Map|Add (LocalVariables|GetLocal%20save%20slots) Slot Slot%20Info)
  (Variables|/Game/ResidentHorrorFPS/Blueprints/BP_SaveSystem/BP_SaveGameResidentHorror.BP_SaveGameResidentHorror_C|SetSaveSlotsInfo (Variables|Default|GetActive%20Save%20Game%20object) (LocalVariables|GetLocal%20save%20slots))
  (Variables|/Game/ResidentHorrorFPS/Blueprints/BP_SaveSystem/BP_SaveGameResidentHorror.BP_SaveGameResidentHorror_C|SetAmbient%20Music (Variables|Default|GetActive%20Save%20Game%20object) (Variables|Default|GetAmbient%20Music))
  (Variables|/Game/ResidentHorrorFPS/Blueprints/BP_SaveSystem/BP_SaveGameResidentHorror.BP_SaveGameResidentHorror_C|SetBattle%20music (Variables|Default|GetActive%20Save%20Game%20object) (Variables|Default|GetBattle%20music))
  (Variables|/Game/ResidentHorrorFPS/Blueprints/BP_SaveSystem/BP_SaveGameResidentHorror.BP_SaveGameResidentHorror_C|SetStart%20battle%20Fade%20in%20%28Battle%20Music%29 (Variables|Default|GetActive%20Save%20Game%20object) (Variables|Float|GetStart%20battle%20Fade%20in%20%28Battle%20Music%29))
  (Variables|/Game/ResidentHorrorFPS/Blueprints/BP_SaveSystem/BP_SaveGameResidentHorror.BP_SaveGameResidentHorror_C|SetStart%20battle%20-%20fade%20out%20background%20music (Variables|Default|GetActive%20Save%20Game%20object) (Variables|Float|GetStart%20battle%20-%20fade%20out%20background%20music))
  (Variables|/Game/ResidentHorrorFPS/Blueprints/BP_SaveSystem/BP_SaveGameResidentHorror.BP_SaveGameResidentHorror_C|SetEnd%20Battle%20Fade%20Out%20%28End%20Battle%29 (Variables|Default|GetActive%20Save%20Game%20object) (Variables|Float|GetEnd%20Battle%20Fade%20Out%20%28End%20Battle%29))
  (Variables|/Game/ResidentHorrorFPS/Blueprints/BP_SaveSystem/BP_SaveGameResidentHorror.BP_SaveGameResidentHorror_C|SetEnd%20of%20battle%20Fade%20in%20%28Background%20music%29 (Variables|Default|GetActive%20Save%20Game%20object) (Variables|Float|GetEnd%20of%20battle%20Fade%20in%20%28Background%20music%29))
  (Default|SetInventorySaveSnapshot (Variables|Default|GetActive%20Save%20Game%20object) (Variables|Default|GetInventorySaveEntries) (Variables|Default|GetInventoryItemInformation) (Variables|Default|GetEquipmentItemIndices) (Variables|Default|GetCurrentEquipmentItemIndex) (Variables|Default|GetHasInventorySaveData))
  (bind _returnvalue_3 (SaveGame|SaveGametoSlot (Variables|Default|GetActive%20Save%20Game%20object) (Utilities|String|ToString(Integer) Slot)))
  (if _returnvalue_3
    (CallFunction|SaveSlottoGlobalConfig Slot)))

(fn LoadGameResidentHorror
  (params (Slot :type Integer))
  (Variables|Boolean|Setin%20Loading? true)
  (bind _returnvalue (SaveGame|LoadGamefromSlot (Utilities|String|ToString(Integer) Slot)))
  (bind _asbp_save_game_resident_horror (Utilities|Casting|CastToBP_SaveGameResidentHorror _returnvalue))
  (Variables|Default|SetActive%20Save%20Game%20object _asbp_save_game_resident_horror)
  (bind (_inventorysaveentries _inventoryiteminformation _equipmentitemindices _currentequipmentitemindex _hasinventorysavedata) (Default|GetInventorySaveSnapshot (Variables|Default|GetActive%20Save%20Game%20object)))
  (Variables|Default|SetInventorySaveEntries _inventorysaveentries)
  (Variables|Default|SetInventoryItemInformation _inventoryiteminformation)
  (Variables|Default|SetEquipmentItemIndices _equipmentitemindices)
  (Variables|Default|SetCurrentEquipmentItemIndex _currentequipmentitemindex)
  (Variables|Default|SetHasInventorySaveData _hasinventorysavedata)
  (Variables|Map|SetObjectSaveData (Variables|/Game/ResidentHorrorFPS/Blueprints/BP_SaveSystem/BP_SaveGameResidentHorror.BP_SaveGameResidentHorror_C|GetObjectSaveData (Variables|Default|GetActive%20Save%20Game%20object)))
  (Variables|Default|SetAmbient%20Music (Variables|/Game/ResidentHorrorFPS/Blueprints/BP_SaveSystem/BP_SaveGameResidentHorror.BP_SaveGameResidentHorror_C|GetAmbient%20Music (Variables|Default|GetActive%20Save%20Game%20object)))
  (Variables|Default|SetBattle%20music (Variables|/Game/ResidentHorrorFPS/Blueprints/BP_SaveSystem/BP_SaveGameResidentHorror.BP_SaveGameResidentHorror_C|GetBattle%20music (Variables|Default|GetActive%20Save%20Game%20object)))
  (Variables|Float|SetStart%20battle%20Fade%20in%20%28Battle%20Music%29 (Variables|/Game/ResidentHorrorFPS/Blueprints/BP_SaveSystem/BP_SaveGameResidentHorror.BP_SaveGameResidentHorror_C|GetStart%20battle%20Fade%20in%20%28Battle%20Music%29 (Variables|Default|GetActive%20Save%20Game%20object)))
  (Variables|Float|SetStart%20battle%20-%20fade%20out%20background%20music (Variables|/Game/ResidentHorrorFPS/Blueprints/BP_SaveSystem/BP_SaveGameResidentHorror.BP_SaveGameResidentHorror_C|GetStart%20battle%20-%20fade%20out%20background%20music (Variables|Default|GetActive%20Save%20Game%20object)))
  (Variables|Float|SetEnd%20Battle%20Fade%20Out%20%28End%20Battle%29 (Variables|/Game/ResidentHorrorFPS/Blueprints/BP_SaveSystem/BP_SaveGameResidentHorror.BP_SaveGameResidentHorror_C|GetEnd%20Battle%20Fade%20Out%20%28End%20Battle%29 (Variables|Default|GetActive%20Save%20Game%20object)))
  (Variables|Float|SetEnd%20of%20battle%20Fade%20in%20%28Background%20music%29 (Variables|/Game/ResidentHorrorFPS/Blueprints/BP_SaveSystem/BP_SaveGameResidentHorror.BP_SaveGameResidentHorror_C|GetEnd%20of%20battle%20Fade%20in%20%28Background%20music%29 (Variables|Default|GetActive%20Save%20Game%20object)))
  (Game|OpenLevel(byName) (Variables|/Game/ResidentHorrorFPS/Blueprints/BP_SaveSystem/BP_SaveGameResidentHorror.BP_SaveGameResidentHorror_C|GetCurrent%20Map _asbp_save_game_resident_horror)))

(fn SaveObjectData
  (params (Object%20Data :type ST%20Save%20Load%20Structure) (Object%20Loc :type Vector))
  (Utilities|Map|Add (Variables|Map|GetObjectSaveData) Object%20Loc Object%20Data))

(fn SaveSlottoGlobalConfig
  (params (Continue%20Slot :type Integer))
  (bind _returnvalue (SaveGame|DoesSaveGameExist "ResidentHorrorGlobal"))
  (if _returnvalue
    (bind _returnvalue_2 (SaveGame|LoadGamefromSlot "ResidentHorrorGlobal"))
    (bind _asbp_save_game_resident_horror_global (Utilities|Casting|CastToBP_SaveGameResidentHorrorGlobal _returnvalue_2))
    (Variables|/Game/ResidentHorrorFPS/Blueprints/BP_SaveSystem/BP_SaveGameResidentHorrorGlobal.BP_SaveGameResidentHorrorGlobal_C|SetContinue%20Slot _asbp_save_game_resident_horror_global Continue%20Slot)
    (SaveGame|SaveGametoSlot _asbp_save_game_resident_horror_global "ResidentHorrorGlobal")
    (else
      (bind _returnvalue_3 (SaveGame|CreateSaveGameObject "/Game/ResidentHorrorFPS/Blueprints/BP_SaveSystem/BP_SaveGameResidentHorrorGlobal.BP_SaveGameResidentHorrorGlobal_C"))
      (Variables|/Game/ResidentHorrorFPS/Blueprints/BP_SaveSystem/BP_SaveGameResidentHorrorGlobal.BP_SaveGameResidentHorrorGlobal_C|SetContinue%20Slot _returnvalue_3 Continue%20Slot)
      (SaveGame|SaveGametoSlot _returnvalue_3 "ResidentHorrorGlobal"))))

(fn GetOptionSetEvent
  (bind _sv_options (Utilities|LoadOptionsSave)
    (:OutputPin
      (return _sv_options))))

(fn StageInventorySaveSnapshot
  (params (InventorySaveEntries :type Array%20of%20ST%20Inventory%20Save%20Entry%20Structures) (EquipmentItemIndices :type Array%20of%20Integers) (CurrentEquipmentItemIndex :type Integer) (HasInventorySaveData :type Boolean))
  (Variables|Default|SetInventorySaveEntries InventorySaveEntries)
  (Variables|Default|SetEquipmentItemIndices EquipmentItemIndices)
  (Variables|Default|SetCurrentEquipmentItemIndex CurrentEquipmentItemIndex)
  (Variables|Default|SetHasInventorySaveData HasInventorySaveData))

(fn GetOptionsRHV2
  (bind _sv_options (Utilities|LoadOptionsSave)
    (:OutputPin
      (return _sv_options))))

(fn IsRestarting?
  (return (Variables|Boolean|GetIs%20Restarting)))

(fn RetrieveGameInstance
  (return self))

(fn RetrieveGamemode
  (return 0))