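; Sliding door that opens once the player collects a required number of items.
; Interacting from the front pauses the game and shows a message on the door camera; a facing dot-product check toggles interact-widget collision.
; CollectItems counts pickups, then plays a camera cutscene with timeline-driven slide, audio and shake while input is disabled.
; BP_SaveLoadRHFps persists the open state and position, though it saves the required count as collected progress.
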(event LoadedData(BP_SaveLoadRHFps)
  (params (Save%20Loaded%20Data :type ST%20Save%20Load%20Structure))
  (bind (_vvector _boolean4 _integer1) (Utilities|Struct|BreakST_SaveLoad Save%20Loaded%20Data))
  ;[0 0 0 0.5] Load Door
  (Variables|Default|SetCollected%20Items _integer1)
  (if _boolean4
    (Transformation|SetRelativeLocation (Variables|Default|GetSM_Door) _vvector false false)
    (Variables|Default|SetDoor%20Is%20Open? true)
    (CallFunction|VisibilityWidgetChange true)))

(event Custom|A%20message%20appears
  (bind _returnvalue (Game|GetPlayerController 0))
  ;[0 0 0] A message appears
  (Audio|PlaySound2D (Variables|Default|GetSound%20Interact) 1.0 1.0 0.0 0 0)
  (CallFunction|HaveACamera)
  (if (not (Variables|Default|GetMessage%20Enabled?))
    (CallFunction|CreateWidget)
    (Variables|Default|SetMessage%20Enabled? true)
    (Default|UpdateText (Variables|Default|GetWB%20Fast%20Inspect) (Variables|Default|GetWrite%20Message))
    (Game|SetGamePaused true)
    (Variables|/Script/Engine.PlayerController|SetbShowMouseCursor _returnvalue true)
    (Input|SetInputModeUIOnly _returnvalue (Variables|Default|GetWB%20Fast%20Inspect) "DoNotLock" false)
    (Widget|SetVisibility (Variables|Default|GetWB%20Fast%20Inspect) "Visible")))

(event Custom|Collect%20Items
  ;[0 0 0] PICK UP ITEM AND OPEN DOOR
  ;;[0 0 0] collect items to open the door
  (Math|Integer|IncrementInt (Variables|Default|GetCollected%20Items)
    (:%20%20
      (Default|SaveData (Variables|Default|GetBP_SaveLoadRHFps) (Utilities|Struct|MakeST_SaveLoad (Variables|Default|Get%20Items%20Collect) false))
      (if (not (Variables|Default|GetDoor%20Is%20Open?))
        (if (>= (Variables|Default|GetCollected%20Items) (Variables|Default|Get%20Items%20Collect))
          (Variables|Default|SetDoor%20Is%20Open? true)
          (CallFunction|HaveACamera)
          (Audio|Components|Audio|Play (Variables|Default|GetAudio) 0.0)
          (CameraShakes|StartCameraShake (Variables|Default|GetCameraShakeSource) "/Game/ResidentHorrorFPS/Blueprints/BP_CameraShake/CS_SpeedBalance.CS_SpeedBalance_C" 0.1 "CameraLocal" "0, 0, 0")
          (Input|DisableInput (CallFunction|RHVFPSPlayerRef) (Game|GetPlayerController 0))
          (Rendering|SetVisibility (Variables|Default|GetInteractWidget) false false)
          (bind _open (Timeline|Timeline PlayFromStart)
            (:Update
              (Transformation|SetRelativeLocation (Variables|Default|GetSM_Door) (Math|Vector|MakeVector 0.0 (Math|Float|Lerp 0.0 95.38909 _open) 0.0) false false))
            (:Finished
              (Audio|Components|Audio|Stop (Variables|Default|GetAudio))
              (CameraShake|StopAllCameraShakes (Variables|Default|GetCameraShakeSource) true)
              (Utilities|FlowControl|Delay 1.0)
              (CallFunction|RemoveCamera)
              (CameraShakes|StartCameraShake (Variables|Default|GetCameraShakeSource) 0 0.1 "CameraLocal" "0, 0, 0")
              (Variables|Default|SetDoor%20Is%20Open? true)
              (Collision|SetCollisionEnabled (Variables|Default|GetInteractableAlert) "NoCollision")
              (Rendering|SetVisibility (Variables|Default|GetInteractWidget) false false)
              (Input|EnableInput (CallFunction|RHVFPSPlayerRef) (Game|GetPlayerController 0))
              (Default|SaveData (Variables|Default|GetBP_SaveLoadRHFps) (Utilities|Struct|MakeST_SaveLoad (Variables|/Script/Engine.SceneComponent|GetRelativeLocation (Variables|Default|GetSM_Door)) true)))))))))

(event Custom|Create%20Widget
  ;[0 0 0] Create Widget
  (bind _returnvalue (UserInterface|CreateWidget "/Game/ResidentHorrorFPS/Blueprints/BP_FastInspectV2/WBP_FastInspectV2.WBP_FastInspectV2_C" 0 0 self))
  (bind _output_get (Variables|Default|SetWB%20Fast%20Inspect _returnvalue))
  (UserInterface|Viewport|AddtoViewport _output_get 0))

(event Custom|Have%20A%20Camera
  ;[0 0 0] Have A Camera
  (Game|Player|SetViewTargetwithBlend (Game|GetPlayerController 0) (Components|GetOwner (Variables|Default|GetCamera)) 0.0 "VTBlend_Cubic" 1.0 false)
  (Widget|SetVisibility (Variables|/Game/ResidentHorrorFPS/Character/BP_Character/BP_RHV_FPS_Player.BP_RHV_FPS_Player_C|GetWBP%20Main%20Hud (CallFunction|RHVFPSPlayerRef)) "Hidden")
  (Rendering|SetActorHiddenInGame (Game|Player|GetPlayerPawn 0) true))

(event Custom|Remove%20Camera
  ;[0 0 0] REMOVE CAMERA
  (Utilities|FlowControl|Sequence
    (:then_0
      (Game|Player|SetViewTargetwithBlend (Game|GetPlayerController 0) (Game|Player|GetPlayerPawn 0) 0.0 "VTBlend_Cubic" 0.0 false)
      (Widget|SetVisibility (Variables|/Game/ResidentHorrorFPS/Character/BP_Character/BP_RHV_FPS_Player.BP_RHV_FPS_Player_C|GetWBP%20Main%20Hud (CallFunction|RHVFPSPlayerRef)) "Visible")
      (Rendering|SetActorHiddenInGame (Game|Player|GetPlayerPawn 0) false))
    (:then_1
      (CallFunction|VisibilityWidgetChange false))))

(event EventTick
  (params (DeltaSeconds :type Float%20%28single-precision%29))
  ;[0 0 0 0.5] Event TICK
  (if (CallFunction|VerificationSideDoor)
    (Collision|SetCollisionEnabled (Variables|Default|GetInteractWidget) "NoCollision")
    (elif (not (Variables|Default|GetDoor%20Is%20Open?))
      (Collision|SetCollisionEnabled (Variables|Default|GetInteractWidget) "QueryAndPhysics"))))

(event EventInteraction
  (params (Player :type BP%20RHV%20FPS%20Player%20Object%20Reference) (AutoInteraction%28Non-Player%29 :type Boolean))
  ;[0 0 0] Create Widget
  (if (> (Math|Vector|DotProduct (Math|Vector|GetForwardVector (Variables|Default|GetArrow)) (Transformation|GetActorForwardVector (CallFunction|RHVFPSPlayerRef))) 0.6)
    (if (not (Variables|Default|GetDoor%20Is%20Open?))
      (CallFunction|AMessageAppears)
      (CallFunction|VisibilityWidgetChange true))))

(fn ConstructionScript
  (|CallParentFunction))

(fn VerificationSideDoor
  (return (> (Math|Vector|DotProduct (Math|Vector|GetForwardVector (Variables|Default|GetArrow1)) (Transformation|GetActorForwardVector (CallFunction|RHVFPSPlayerRef))) 0.6)))