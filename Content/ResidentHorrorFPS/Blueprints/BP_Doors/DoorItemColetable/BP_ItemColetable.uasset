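; Collectible item that counts toward a referenced door's item puzzle when the player character walks into its trigger.
; On overlap with a valid door, it notifies that door, plays a sound, shows the collectable puzzle widget, saves its collected flag and destroys itself.
; The save/load component's loaded event destroys already collected items.
; The construction script sets the preview mesh and optional shiny overlay material.
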(event OnComponentBeginOverlap(CollisionCollect)
  (params (OverlappedComponent :type Primitive%20Component%20Object%20Reference) (OtherActor :type Actor%20Object%20Reference) (OtherComp :type Primitive%20Component%20Object%20Reference) (OtherBodyIndex :type Integer) (bFromSweep :type Boolean) (SweepResult :type Hit%20Result%20Structure%20%28by%20ref%29))
  ;[0 0 0] TRIGGER TO COLLECT
  (if (== OtherActor (Game|GetPlayerCharacter 0))
    (bind _door_ref (Variables|Default|GetDoor%20Ref)
      (:then
        (Default|CollectItems _door_ref)
        (Audio|PlaySound2D (Variables|Default|GetSound%20Interact) 1.0 1.0 0.0 0 0)
        (bind _returnvalue (UserInterface|CreateWidget "/Game/ResidentHorrorFPS/Blueprints/WBP/items/WBP_ColectablePuzzle.WBP_ColectablePuzzle_C" 0 _door_ref))
        (UserInterface|Viewport|AddtoViewport _returnvalue 0)
        (Default|SaveData (Variables|Default|GetBP_SaveLoadRHFps) (Utilities|Struct|MakeST_SaveLoad true 0 0))
        (Actor|DestroyActor))
      (:else))))

(event LoadedData(BP_SaveLoadRHFps)
  (params (Save%20Loaded%20Data :type ST%20Save%20Load%20Structure))
  ;[0 0 0 0.5] Load
  (if (.Boolean2 (Utilities|Struct|BreakST_SaveLoad Save%20Loaded%20Data))
    (Actor|DestroyActor)))

(fn ConstructionScript
  ;[0.15 0.15 0.15 0.5] Overlay Item
  (if (Variables|Default|GetOverlay%20item?)
    (Rendering|Material|SetOverlayMaterial (Variables|Default|GetItem%20Mesh) "/Game/ResidentHorrorFPS/Demo/Materials/M_ShinyOverlay.M_ShinyOverlay" :!class /Script/Engine.MeshComponent))
  (Components|StaticMesh|SetStaticMesh (Variables|Default|GetItem%20Mesh) (Variables|Default|GetItem%20Mesh%20Preview)))