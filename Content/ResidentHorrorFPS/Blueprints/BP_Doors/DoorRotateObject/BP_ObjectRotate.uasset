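; BP_ObjectRotate is an interactable puzzle piece that opens a linked door after a set number of turns.
; Each interaction plays a sound and Timeline that turns the mesh 90 degrees in pitch, then increments a turn counter.
; When the counter reaches HowManySpins, it opens the door and locks itself.
; Rotation and count persist through the save/load component, which restores the solved state on load.
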(event LoadedData(BP_SaveLoadRHFps)
  (params (Save%20Loaded%20Data :type ST%20Save%20Load%20Structure))
  (bind (_boolean4 _rotator _integer1) (Utilities|Struct|BreakST_SaveLoad Save%20Loaded%20Data))
  ;[0.15 0.15 0.15 0.5] Load
  (Transformation|SetRelativeRotation (Variables|Default|GetStaticMesh) _rotator false false)
  (Variables|Default|SetStore%20Rotation%20Table _rotator)
  (Variables|Default|SetObject%20position _integer1)
  (if (== _integer1 (Variables|Default|GetHow%20many%20spins?))
    (Variables|Default|SetFinish? true)
    (CallFunction|VisibilityWidgetChange true)
    (Collision|SetCollisionResponsetoAllChannels (Variables|Default|GetStaticMesh) "ECR_Ignore")))

(event Custom|Rotate%20Object
  ;[0 0 0] Rotate Object
  (Default|SaveData (Variables|Default|GetBP_SaveLoadRHFps) (Utilities|Struct|MakeST_SaveLoad (Variables|Default|GetStore%20Rotation%20Table)))
  (if (not (Variables|Default|GetMovement%20of%20the%20object))
    (Variables|Default|SetMovement%20of%20the%20object true)
    (Audio|PlaySound2D (Variables|Default|GetNoise%20when%20turning%20the%20part) 1.0 1.0 0.0 0 0)
    (bind _rotação_suave (Timeline|Timeline PlayFromStart)
      (:Update
        (Transformation|SetRelativeRotation (Variables|Default|GetStaticMesh) (Math|Rotator|MakeRotator 0.0 (Math|Float|Lerp (.pitch (Variables|Default|GetStore%20Rotation%20Table)) (- (.pitch (Variables|Default|GetStore%20Rotation%20Table)) 9e+01) _rotação_suave) 0.0) false false))
      (:Finished
        (bind _output_get (Variables|Default|SetStore%20Rotation%20Table (Math|Rotator|MakeRotator 0.0 (Math|Float|Lerp (.pitch (Variables|Default|GetStore%20Rotation%20Table)) (- (.pitch (Variables|Default|GetStore%20Rotation%20Table)) 9e+01) _rotação_suave) 0.0)))
        (Variables|Default|SetMovement%20of%20the%20object false)
        (bind _result (Math|Integer|IncrementInt (Variables|Default|GetObject%20position))
          (:%20%20
            ;;[0.06979 0.06937 0.06732] This section of the code checks whether the object is in the correct position; if so, it opens the door
            (Variables|Default|SetObject%20position _result)
            (Default|SaveData (Variables|Default|GetBP_SaveLoadRHFps) (Utilities|Struct|MakeST_SaveLoad _output_get (Variables|Default|GetObject%20position)))
            (if (== (Variables|Default|GetHow%20many%20spins?) (Variables|Default|GetObject%20position))
              (Variables|/Game/ResidentHorrorFPS/Blueprints/BP_Doors/DoorRotateObject/BP_DoorRotateObject.BP_DoorRotateObject_C|SetClose? (Variables|Default|GetWhich%20door%20should%20I%20open?) false)
              (Default|OpenDoorObjectRotate (Variables|Default|GetWhich%20door%20should%20I%20open?) "NewEnumerator0")
              (Variables|Default|SetFinish? true)
              (Audio|PlaySound2D (Variables|Default|GetSound%20when%20the%20puzzle%20is%20completed) 1.0 1.0 0.0 0 0)
              (Rendering|SetVisibility (Variables|Default|GetInteractWidget) false false))))))))

(event EventBeginPlay
  ;[0 0 0] Save Relative Rotation
  (Utilities|FlowControl|Delay 0.2)
  (Variables|Default|SetStore%20Rotation%20Table (Variables|/Script/Engine.SceneComponent|GetRelativeRotation (Variables|Default|GetStaticMesh)))
  (|CallParentFunction)
  (if (Variables|Default|GetFinish?)
    (Utilities|FlowControl|Delay 0.2)
    (Rendering|SetVisibility (Variables|Default|GetInteractWidget) false false)))

(event EventInteraction
  (params (Player :type BP%20RHV%20FPS%20Player%20Object%20Reference) (AutoInteraction%28Non-Player%29 :type Boolean))
  ;[0 0 0] Interact with the puzzle
  (if (not (Variables|Default|GetFinish?))
    (CallFunction|RotateObject)))

(event Collision|EventActorBeginOverlap
  (params (OtherActor :type Actor%20Object%20Reference)))

(fn ConstructionScript
  (|CallParentFunction))