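; Master interactive door that the player opens, closes, tries while locked, or unlocks with a matching inventory key.
; Side colliders and door state select paired player montages and door animations, and a proximity widget shows the prompt.
; A timeline aligns player and view before playback, while weapons are hidden and montage notifies handle the key mesh.
; Non-player interaction skips player alignment, and save loading restores mesh rotation.
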(event OnComponentBeginOverlap(InteractableAlert)
  (params (OverlappedComponent :type Primitive%20Component%20Object%20Reference) (OtherActor :type Actor%20Object%20Reference) (OtherComp :type Primitive%20Component%20Object%20Reference) (OtherBodyIndex :type Integer) (bFromSweep :type Boolean) (SweepResult :type Hit%20Result%20Structure%20%28by%20ref%29))
  (bind _frontinteractionwidget (Variables|Default|GetFrontInteractionWidget))
  ;[0.15 0.15 0.15 0.5] Begin Overlap
  (if (== OtherActor (CallFunction|RHVFPSPlayerRef))
    (bind _returnvalue (UserInterface|CreateWidget "/Game/ResidentHorrorFPS/Blueprints/BP_InteractMaster/InteractionSystem/WBP_SingleInteraction.WBP_SingleInteraction_C" 0 "Door Interact"))
    (bind _output_get (Variables|Default|SetWBP%20Interact _returnvalue))
    (if (Utilities|Enum|Equal(Enum) (Variables|Default|GetInteractPosition) "NewEnumerator1")
      (Rendering|SetVisibility _frontinteractionwidget true true)
      (UserInterface|SetWidget _frontinteractionwidget _output_get)
      (Rendering|SetVisibility (Variables|Default|GetBackInteractionWidget) false false)
      (else
        (Rendering|SetVisibility (Variables|Default|GetBackInteractionWidget) true true)
        (Rendering|SetVisibility (Variables|Default|GetFrontInteractionWidget) false false)
        (UserInterface|SetWidget (Variables|Default|GetBackInteractionWidget) _output_get)))
    (Default|FadinAlert (Variables|Default|GetWBP%20Interact))))

(event OnComponentEndOverlap(InteractableAlert)
  (params (OverlappedComponent :type Primitive%20Component%20Object%20Reference) (OtherActor :type Actor%20Object%20Reference) (OtherComp :type Primitive%20Component%20Object%20Reference) (OtherBodyIndex :type Integer))
  ;[0.15 0.15 0.15 0.5] End Overlap
  (bind _wbp_interact (Variables|Default|GetWBP%20Interact)
    (:then
      (Widget|RemovefromParent _wbp_interact)
      (Rendering|SetVisibility (Variables|Default|GetBackInteractionWidget) false false))
    (:else)))

(event OnComponentBeginOverlap(BackInteractionCollider)
  (params (OverlappedComponent :type Primitive%20Component%20Object%20Reference) (OtherActor :type Actor%20Object%20Reference) (OtherComp :type Primitive%20Component%20Object%20Reference) (OtherBodyIndex :type Integer) (bFromSweep :type Boolean) (SweepResult :type Hit%20Result%20Structure%20%28by%20ref%29))
  ;[0.15 0.15 0.15 0.5] Check Player Position
  (if (== OtherActor (Game|GetPlayerCharacter 0))
    (bind _output_get (Variables|Default|SetInteractPosition "NewEnumerator2"))
    (Variables|Default|SetLocalInteractPosition _output_get)))

(event OnComponentEndOverlap(BackInteractionCollider)
  (params (OverlappedComponent :type Primitive%20Component%20Object%20Reference) (OtherActor :type Actor%20Object%20Reference) (OtherComp :type Primitive%20Component%20Object%20Reference) (OtherBodyIndex :type Integer))
  ;[0.15 0.15 0.15 0.5] Check Player Position
  (if (== OtherActor (Game|GetPlayerCharacter 0))
    (Variables|Default|SetInteractPosition "NewEnumerator0")))

(event OnComponentBeginOverlap(FrontInteractionCollider)
  (params (OverlappedComponent :type Primitive%20Component%20Object%20Reference) (OtherActor :type Actor%20Object%20Reference) (OtherComp :type Primitive%20Component%20Object%20Reference) (OtherBodyIndex :type Integer) (bFromSweep :type Boolean) (SweepResult :type Hit%20Result%20Structure%20%28by%20ref%29))
  ;[0.15 0.15 0.15 0.5] Check Player Position
  (if (== OtherActor (Game|GetPlayerCharacter 0))
    (bind _output_get (Variables|Default|SetInteractPosition "NewEnumerator1"))
    (Variables|Default|SetLocalInteractPosition _output_get)))

(event OnComponentEndOverlap(FrontInteractionCollider)
  (params (OverlappedComponent :type Primitive%20Component%20Object%20Reference) (OtherActor :type Actor%20Object%20Reference) (OtherComp :type Primitive%20Component%20Object%20Reference) (OtherBodyIndex :type Integer))
  ;[0.15 0.15 0.15 0.5] Check Player Position
  (if (== OtherActor (Game|GetPlayerCharacter 0))
    (Variables|Default|SetInteractPosition "NewEnumerator0")))

(event LoadedData(BP_SaveLoadRHFps)
  (params (Save%20Loaded%20Data :type ST%20Save%20Load%20Structure))
  ;[0.15 0.15 0.15 0.5] Load
  (Transformation|SetRelativeRotation (Variables|Default|GetMesh) (.Rotator (Utilities|Struct|BreakST_SaveLoad Save%20Loaded%20Data)) false false))

(event Custom|Set%20Player%20Position
  (bind _returnvalue (Game|GetPlayerController 0))
  (bind _player (Variables|Default|GetPlayer))
  (bind _player_2 (Variables|Default|GetPlayer))
  (bind _abp_rhfps (Variables|/Game/ResidentHorrorFPS/Character/BP_Character/BP_RHV_FPS_Player.BP_RHV_FPS_Player_C|GetABP%20RHFPS _player_2))
  ;[0.15 0.15 0.15 0.5] Set Player Position
  (if (Variables|Default|GetAuto%20Interaction%28Non-%20Player%29)
    (Variables|Default|SetDoorState "NewEnumerator0")
    (Variables|Default|SetLocalInteractPosition "NewEnumerator1")
    (Utilities|PlayMontageandAnim 0 (.AnimReturnValue (CallFunction|GetDoorAnimation)))
    (else
      (Input|DisableInput (Variables|Default|GetPlayer) _returnvalue)
      (Input|SetIgnoreLookInput _returnvalue true)
      (Collision|SetActorEnableCollision _player false)
      (Pawn|Components|CharacterMovement|SetMovementMode (Variables|/Script/Engine.Character|GetCharacterMovement _player) "MOVE_None" 0)
      (bind _positionalpha (Timeline|Timeline PlayFromStart)
        (:Update
          (CallFunction|SetControlRotation (Transformation|GetWorldRotation (Utilities|Select :Index (Variables|Default|GetLocalInteractPosition) :NewEnumerator0 0 :NewEnumerator1 (Variables|Default|GetForwardFocusePoint) :NewEnumerator2 (Variables|Default|GetBackwardFocusePoint))) _positionalpha)
          (CallFunction|SetPlayerLocation (Transformation|GetWorldLocation (Utilities|Select :Index (Variables|Default|GetLocalInteractPosition) :NewEnumerator0 0 :NewEnumerator1 (Variables|Default|GetCorrectPositionForward) :NewEnumerator2 (Variables|Default|GetCorrectPositionBackward))) _positionalpha)
          (Transformation|SetActorRotation (Variables|Default|GetPlayer) (Math|Rotator|Lerp(Rotator) (Transformation|GetActorRotation (Variables|Default|GetPlayer)) (Transformation|GetWorldRotation (Utilities|Select :Index (Variables|Default|GetLocalInteractPosition) :NewEnumerator0 0 :NewEnumerator1 (Variables|Default|GetCorrectPositionForward) :NewEnumerator2 (Variables|Default|GetCorrectPositionBackward))) _positionalpha true) true)
          (Variables|/Game/ResidentHorrorFPS/Character/BP_Character/ABP_RHPlayer.ABP_RHPlayer_C|SetRootYawOffset _abp_rhfps (Math|Float|Lerp (Variables|/Game/ResidentHorrorFPS/Character/BP_Character/ABP_RHPlayer.ABP_RHPlayer_C|GetRootYawOffset _abp_rhfps) 0.0 _positionalpha))
          (Variables|/Game/ResidentHorrorFPS/Character/BP_Character/ABP_RHPlayer.ABP_RHPlayer_C|SetIK_Foot_Alpha _abp_rhfps (Math|Float|Lerp 1.0 0.0 _positionalpha)))
        (:Finished
          (if (Variables|Default|GetAuto%20Interaction%28Non-%20Player%29)
            (Variables|Default|SetDoorState (Utilities|Select :Index "NewEnumerator0" :NewEnumerator0 "NewEnumerator1" :NewEnumerator1 "NewEnumerator0" :NewEnumerator2 "NewEnumerator2" :NewEnumerator3 "NewEnumerator0"))
            (else
              (CallFunction|PlayAnimations)
              (bind _player_3 (Variables|Default|GetPlayer)
                (:then
                  (Transformation|AttachComponentToComponent _player_3 (Utilities|Select :Index (Variables|Default|GetLocalInteractPosition) :NewEnumerator0 0 :NewEnumerator1 (Variables|Default|GetCorrectPositionForward) :NewEnumerator2 (Variables|Default|GetCorrectPositionBackward)) "None" "KeepWorld" "KeepWorld" "KeepWorld" true)
                  (Variables|/Script/Engine.CameraComponent|SetbUsePawnControlRotation (Variables|/Game/ResidentHorrorFPS/Character/BP_Character/BP_RHV_FPS_Player.BP_RHV_FPS_Player_C|GetCamera (Variables|Default|GetPlayer)) false))
                (:else)))))))))

(event Custom|PlayAnimations
  (bind (_montagereturnvalue _animreturnvalue) (CallFunction|GetDoorAnimation))
  (bind _player (CallFunction|RHVFPSPlayerRef))
  (bind _bpc_equipment (Variables|/Game/ResidentHorrorFPS/Character/BP_Character/BP_RHV_FPS_Player.BP_RHV_FPS_Player_C|GetBPC_Equipment _player))
  ;[0.15 0.15 0.15 0.5] PlayAnimations
  (if (Variables|/Game/ResidentHorrorFPS/Blueprints/BP_Inventory/Inventory/Equipment/BPC_Equipment.BPC_Equipment_C|GetEquip%20Item? _bpc_equipment)
    (Default|ActivateEquipment/UseItem _bpc_equipment (Variables|/Game/ResidentHorrorFPS/Blueprints/BP_Inventory/Inventory/Equipment/BPC_Equipment.BPC_Equipment_C|GetCurrentIndex _bpc_equipment))
    (Utilities|FlowControl|Delay 1.0)
    (Variables|Default|SetDid%20you%20have%20the%20item%20equipped? true))
  (CallFunction|OcultWeapon false)
  (bind _notifyname (Utilities|PlayMontageandAnim _montagereturnvalue _animreturnvalue)
    (:On%20Completed
      (CallFunction|ResetPlayer)
      (Variables|Default|SetDoorState (Utilities|Select :Index (Variables|Default|GetDoorState) :NewEnumerator0 "NewEnumerator1" :NewEnumerator1 "NewEnumerator0" :NewEnumerator2 "NewEnumerator2" :NewEnumerator3 "NewEnumerator0"))
      (Utilities|FlowControl|Delay 0.5)
      (CallFunction|VerificationItemEquipped))
    (:On%20Notify%20Begin
      (switch name _notifyname
        (:Spawn
          (Components|StaticMesh|SetStaticMesh (Variables|Default|GetKey) "/Game/ResidentHorrorFPS/Demo/Mesh/SM_DoorKey.SM_DoorKey")
          (Transformation|AttachComponentToComponent (Variables|Default|GetScene) (Variables|/Script/Engine.Character|GetMesh (Variables|Default|GetPlayer)) "weapon_r" "SnapToTarget" "SnapToTarget" "KeepRelative" true))
        (:Destroy
          (Components|StaticMesh|SetStaticMesh (Variables|Default|GetKey) 0)
          (Transformation|DetachFromComponent (Variables|Default|GetScene) "KeepWorld" "KeepWorld" "KeepWorld" true)
          (CallFunction|OcultWeapon true))))))

(event Custom|Verification%20Item%20equipped
  (bind _player (CallFunction|RHVFPSPlayerRef))
  (bind _bpc_equipment (Variables|/Game/ResidentHorrorFPS/Character/BP_Character/BP_RHV_FPS_Player.BP_RHV_FPS_Player_C|GetBPC_Equipment _player))
  ;[0.15 0.15 0.15 0.5] Verification Item equipped
  (if (not (Variables|/Game/ResidentHorrorFPS/Blueprints/BP_Inventory/Inventory/Equipment/BPC_Equipment.BPC_Equipment_C|GetEquip%20Item? _bpc_equipment))
    (if (Variables|Default|GetDid%20you%20have%20the%20item%20equipped?)
      (Default|ActivateEquipment/UseItem _bpc_equipment (Variables|/Game/ResidentHorrorFPS/Blueprints/BP_Inventory/Inventory/Equipment/BPC_Equipment.BPC_Equipment_C|GetCurrentIndex _bpc_equipment))
      (Variables|Default|SetDid%20you%20have%20the%20item%20equipped? false))))

(event Custom|Ocult%20Weapon
  (params (Visibility :type Boolean))
  ;[0.15 0.15 0.15 0.5] Ocult Weapon
  (if Visibility
    (bind _outactors (Actor|GetAllActorsOfClass "/Game/ResidentHorrorFPS/Blueprints/BP_WeaponSystem/BP_WeaponBase.BP_WeaponBase_C"))
    (for _array_element _outactors
      (Utilities|IsValid _array_element
        (:Is%20Valid
          (Rendering|SetActorHiddenInGame _array_element false))))
    (Utilities|IsValid _array_element
      (:Is%20Valid
        (Rendering|SetActorHiddenInGame _array_element false)))
    (else
      (bind _outactors_2 (Actor|GetAllActorsOfClass "/Game/ResidentHorrorFPS/Blueprints/BP_WeaponSystem/BP_WeaponBase.BP_WeaponBase_C"))
      (for _array_element_2 _outactors_2
        (Utilities|IsValid _array_element_2
          (:Is%20Valid
            (Rendering|SetActorHiddenInGame _array_element_2 true))))
      (Utilities|IsValid _array_element_2
        (:Is%20Valid
          (Rendering|SetActorHiddenInGame _array_element_2 true))))))

(event Custom|ResetPlayer
  (bind _returnvalue (Game|GetPlayerController 0))
  (bind _player (Variables|Default|GetPlayer))
  ;[0.15 0.15 0.15 0.5] ResetPlayer
  (Input|EnableInput (Variables|Default|GetPlayer) _returnvalue)
  (Input|SetIgnoreLookInput _returnvalue false)
  (Collision|SetActorEnableCollision _player true)
  (Pawn|Components|CharacterMovement|SetMovementMode (Variables|/Script/Engine.Character|GetCharacterMovement _player) "MOVE_Walking" 0)
  (Transformation|DetachFromActor _player "KeepWorld" "KeepWorld" "KeepWorld")
  (Variables|/Script/Engine.CameraComponent|SetbUsePawnControlRotation (Variables|/Game/ResidentHorrorFPS/Character/BP_Character/BP_RHV_FPS_Player.BP_RHV_FPS_Player_C|GetCamera (Variables|Default|GetPlayer)) true))

(event EventDefineActor
  (params (Hit? :type Boolean))
  ;[0.15 0.15 0.15 0.5] Visual Widget Visibility
  (if Hit?
    (Default|FadOutAlert (Variables|Default|GetWBP%20Interact))
    (Default|FadinInteraction (Variables|Default|GetWBP%20Interact))
    (else
      (Default|FadinAlert (Variables|Default|GetWBP%20Interact))
      (Default|FadOutInteraction (Variables|Default|GetWBP%20Interact)))))

(event EventInteraction
  (params (Player :type BP%20RHV%20FPS%20Player%20Object%20Reference) (AutoInteraction%28Non-Player%29 :type Boolean))
  ;[0.15 0.15 0.15 0.5] Interact
  (Variables|Default|SetAuto%20Interaction%28Non-%20Player%29 AutoInteraction%28Non-Player%29)
  (if AutoInteraction%28Non-Player%29
    (CallFunction|SetPlayerPosition :!label _label)
    (elif (Utilities|Enum|NotEqual(Enum) (Variables|Default|GetInteractPosition) "NewEnumerator0")
      (Variables|Default|SetPlayer Player)
      (bind _findresult (CallFunction|FindKey))
      (if _findresult
        (Variables|Default|SetDoorState "NewEnumerator3")
        (goto _label)
        (else
          (goto _label))))))

(fn ConstructionScript)

(fn SetPlayerLocation
  (params (NewLocation :type Vector) (Alpha :type Float%20%28single-precision%29))
  (bind _player (Variables|Default|GetPlayer))
  (bind _returnvalue (Transformation|GetActorLocation _player))
  (bind _returnvalue_2 (Math|Vector|Lerp(Vector) _returnvalue NewLocation Alpha))
  (Transformation|SetActorLocation (Variables|Default|GetPlayer) (Math|Vector|MakeVector (.x _returnvalue_2) (.y _returnvalue_2) (.Z (Math|Vector|BreakVector _returnvalue))) false false))

(fn SetControlRotation
  (params (NewRotation :type Rotator) (Alpha :type Float%20%28single-precision%29))
  (bind _returnvalue (Game|GetPlayerController 0))
  (bind _returnvalue_2 (Pawn|GetControlRotation _returnvalue :!class /Script/Engine.Controller))
  (bind _returnvalue_3 (Math|Rotator|Lerp(Rotator) _returnvalue_2 NewRotation Alpha true))
  (Pawn|SetControlRotation _returnvalue (Math|Rotator|MakeRotator (.roll _returnvalue_3) (.pitch _returnvalue_3) (.yaw _returnvalue_3))))

(fn GetDoorAnimation
  (return (Utilities|Select :Index (Variables|Default|GetLocalInteractPosition) :NewEnumerator0 0 :NewEnumerator1 (Utilities|Select :Index (Variables|Default|GetDoorState) :NewEnumerator0 "/Game/ResidentHorrorFPS/Character/Animations/Door/Basic/AM_Door_Forward_Open_Montage.AM_Door_Forward_Open_Montage" :NewEnumerator1 "/Game/ResidentHorrorFPS/Character/Animations/Door/Basic/AM_Door_Forward_Close_Montage.AM_Door_Forward_Close_Montage" :NewEnumerator2 "/Game/ResidentHorrorFPS/Character/Animations/Door/Basic/AM_Door_Forward_Locked_Montage.AM_Door_Forward_Locked_Montage" :NewEnumerator3 "/Game/ResidentHorrorFPS/Character/Animations/Door/Basic/AM_Door_Backward_Key_Montage.AM_Door_Backward_Key_Montage") :NewEnumerator2 (Utilities|Select :Index (Variables|Default|GetDoorState) :NewEnumerator0 "/Game/ResidentHorrorFPS/Character/Animations/Door/Basic/AM_Door_Backward_Open_Montage.AM_Door_Backward_Open_Montage" :NewEnumerator1 "/Game/ResidentHorrorFPS/Character/Animations/Door/Basic/AM_Door_Backward_Close_Montage.AM_Door_Backward_Close_Montage" :NewEnumerator2 "/Game/ResidentHorrorFPS/Character/Animations/Door/Basic/AM_Door_Backward_Locked_Montage.AM_Door_Backward_Locked_Montage" :NewEnumerator3 "/Game/ResidentHorrorFPS/Character/Animations/Door/Basic/AM_Door_Forward_Key_Montage.AM_Door_Forward_Key_Montage")) (Utilities|Select :Index (Variables|Default|GetLocalInteractPosition) :NewEnumerator0 0 :NewEnumerator1 (Utilities|Select :Index (Variables|Default|GetDoorState) :NewEnumerator0 "/Game/ResidentHorrorFPS/Character/Animations/AnimationDoor/AS_Door_Open_F.AS_Door_Open_F" :NewEnumerator1 "/Game/ResidentHorrorFPS/Character/Animations/AnimationDoor/AS_Door_Close_F.AS_Door_Close_F" :NewEnumerator2 "/Game/ResidentHorrorFPS/Character/Animations/AnimationDoor/AS_Door_Locked_F.AS_Door_Locked_F" :NewEnumerator3 0) :NewEnumerator2 (Utilities|Select :Index (Variables|Default|GetDoorState) :NewEnumerator0 "/Game/ResidentHorrorFPS/Character/Animations/AnimationDoor/AS_Door_Open_B.AS_Door_Open_B" :NewEnumerator1 "/Game/ResidentHorrorFPS/Character/Animations/AnimationDoor/AS_Door_Close_B.AS_Door_Close_B" :NewEnumerator2 "/Game/ResidentHorrorFPS/Character/Animations/AnimationDoor/AS_Door_Locked_B.AS_Door_Locked_B" :NewEnumerator3 0))))

(fn FindKey
  (bind _keytouse (Variables|Default|GetKeyToUse))
  (if (Utilities|Enum|Equal(Enum) (Variables|Default|GetDoorState) "NewEnumerator2")
    (bind _array_element (Utilities|Array|ForEachLoopwithBreak (Variables|/Game/ResidentHorrorFPS/Blueprints/BP_Inventory/Inventory/BPC_Inventory.BPC_Inventory_C|GetInventoryItems (Variables|/Game/ResidentHorrorFPS/Character/BP_Character/BP_RHV_FPS_Player.BP_RHV_FPS_Player_C|GetBPC_Inventory (Variables|Default|GetPlayer))) :!label _label)
      (:LoopBody
        (Utilities|IsValid _array_element
          (:Is%20Valid
            (if (== (.datatable (.Information (Utilities|Struct|BreakST_UsableInfo (.UsableInformation (Utilities|Struct|BreakST_ItemInformation (Variables|/Game/ResidentHorrorFPS/Blueprints/BP_Inventory/Inventory/ItemData/BP_ItemObject.BP_ItemObject_C|GetInformation _array_element)))))) (.datatable _keytouse))
              (if (== (.rowname (.Information (Utilities|Struct|BreakST_UsableInfo (.UsableInformation (Utilities|Struct|BreakST_ItemInformation (Variables|/Game/ResidentHorrorFPS/Blueprints/BP_Inventory/Inventory/ItemData/BP_ItemObject.BP_ItemObject_C|GetInformation _array_element)))))) (.rowname _keytouse))
                (LocalVariables|SetKeyFind? true)
                (goto _label Break)
                (else
                  _)))
            (LocalVariables|SetKeyFind? false))))
      (:Completed
        (return (LocalVariables|GetKeyFind?))))
    (else
      (return false))))