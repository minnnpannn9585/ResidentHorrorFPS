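; BP_InspectFastV1 is a quick-inspect interactable that shows a text message in a UI widget when the player interacts.
; Interaction plays a sound, then, unless TrueMessage is set, creates a WBP_FastInspectV2 with the message, pauses the game and switches to UI-only input.
; When CameraOn is set, it blends the view to the owner of its Camera, hiding pawn and HUD.
; RemoveCamera reverses the camera change.
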(event Custom|Menssagem%20Displayed
  (bind _returnvalue (Game|GetPlayerController 0))
  ;[0 0 0] Menssage Displayed
  (Audio|PlaySound2D (Variables|Default|GetSound%20Interact) 1.0 1.0 0.0 0 0)
  (if (Variables|Default|GetCamera%20on?)
    (CallFunction|PossesCamera))
  (if (not (Variables|Default|GetTrue%20Message?))
    (CallFunction|CreateWidgetFastInspect)
    (Variables|Default|SetTrue%20Message? true)
    (Default|UpdateText (Variables|Default|GetWb%20FastInspect) (Variables|Default|GetWrite%20Message))
    (Game|SetGamePaused true)
    (Variables|/Script/Engine.PlayerController|SetbShowMouseCursor _returnvalue true)
    (Input|SetInputModeUIOnly _returnvalue (Variables|Default|GetWb%20FastInspect) "DoNotLock" false)
    (Widget|SetVisibility (Variables|Default|GetWb%20FastInspect) "Visible")))

(event Custom|Create%20Widget%20Fast%20inspect
  ;[0 0 0] Create Widget
  (bind _returnvalue (UserInterface|CreateWidget "/Game/ResidentHorrorFPS/Blueprints/BP_FastInspectV2/WBP_FastInspectV2.WBP_FastInspectV2_C" 0 self 0))
  (bind _output_get (Variables|Default|SetWb%20FastInspect _returnvalue))
  (UserInterface|Viewport|AddtoViewport _output_get 0))

(event Custom|Posses%20Camera
  ;[0 0 0] Posses Camera
  (if (Variables|Default|GetCamera%20on?)
    (Game|Player|SetViewTargetwithBlend (Game|GetPlayerController 0) (Components|GetOwner (Variables|Default|GetCamera)) 0.0 "VTBlend_Cubic" 1.0 false)
    (Widget|SetVisibility (Variables|/Game/ResidentHorrorFPS/Character/BP_Character/BP_RHV_FPS_Player.BP_RHV_FPS_Player_C|GetWBP%20Main%20Hud (CallFunction|RHVFPSPlayerRef)) "Hidden")
    (Rendering|SetActorHiddenInGame (Game|Player|GetPlayerPawn 0) true)
    (CallFunction|VisibilityWidgetChange true)))

(event Custom|Remove%20Camera
  ;[0 0 0] Remove Camera
  (if (Variables|Default|GetCamera%20on?)
    (Game|Player|SetViewTargetwithBlend (Game|GetPlayerController 0) (Game|Player|GetPlayerPawn 0) 0.0 "VTBlend_Cubic" 0.0 false)
    (Widget|SetVisibility (Variables|/Game/ResidentHorrorFPS/Character/BP_Character/BP_RHV_FPS_Player.BP_RHV_FPS_Player_C|GetWBP%20Main%20Hud (CallFunction|RHVFPSPlayerRef)) "Visible")
    (Rendering|SetActorHiddenInGame (Game|Player|GetPlayerPawn 0) false)
    (CallFunction|VisibilityWidgetChange false)))

(event EventBeginPlay
  (|CallParentFunction))

(event EventTick
  (params (DeltaSeconds :type Float%20%28single-precision%29))
  (|CallParentFunction DeltaSeconds))

(event EventInteraction
  (params (Player :type BP%20RHV%20FPS%20Player%20Object%20Reference) (AutoInteraction%28Non-Player%29 :type Boolean))
  ;[0 0 0] Create Widget
  (CallFunction|MenssagemDisplayed))

(fn ConstructionScript
  (|CallParentFunction))