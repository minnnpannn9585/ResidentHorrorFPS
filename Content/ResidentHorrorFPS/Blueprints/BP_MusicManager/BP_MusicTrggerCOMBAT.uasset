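; One-shot trigger volume that configures the combat music on the RHVFPS player when the player overlaps its box.
; It copies its battle track, finishing sound and fade settings for battle start and end into player variables, without playing audio itself.
; It then destroys itself and saves a used flag through the save/load component, so it also removes itself when that flag is loaded.
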(event OnComponentBeginOverlap(Box)
  (params (OverlappedComponent :type Primitive%20Component%20Object%20Reference) (OtherActor :type Actor%20Object%20Reference) (OtherComp :type Primitive%20Component%20Object%20Reference) (OtherBodyIndex :type Integer) (bFromSweep :type Boolean) (SweepResult :type Hit%20Result%20Structure%20%28by%20ref%29))
  ;[0 0 0 0.5] Overlap Trigge
  (if (== OtherActor (CallFunction|RHVFPSPlayerRef))
    (Utilities|FlowControl|Sequence
      (:then_0
        ;[0 0 0] Variable Set Music
        (Variables|/Game/ResidentHorrorFPS/Character/BP_Character/BP_RHV_FPS_Player.BP_RHV_FPS_Player_C|SetBattle%20music (CallFunction|RHVFPSPlayerRef) (Variables|Default|GetMusic%20to%20play)))
      (:then_1
        (Variables|/Game/ResidentHorrorFPS/Character/BP_Character/BP_RHV_FPS_Player.BP_RHV_FPS_Player_C|SetStart%20battle%20Fade%20in%20%28Battle%20Music%29 (CallFunction|RHVFPSPlayerRef) (Variables|Default|GetStart%20Combat%20Fade%20In%20%28Combat%20Song%29)))
      (:then_2
        (Variables|/Game/ResidentHorrorFPS/Character/BP_Character/BP_RHV_FPS_Player.BP_RHV_FPS_Player_C|SetEnd%20Battle%20Fade%20Out%20%28End%20Battle%29 (CallFunction|RHVFPSPlayerRef) (Variables|Default|GetStart%20Combat%20-%20Fade%20Out%20Background%20Music)))
      (:then_3
        (Variables|/Game/ResidentHorrorFPS/Character/BP_Character/BP_RHV_FPS_Player.BP_RHV_FPS_Player_C|SetEnd%20of%20battle%20Fade%20in%20%28Background%20music%29 (CallFunction|RHVFPSPlayerRef) (Variables|Default|GetEnd%20of%20Battle%20Fade%20In%20%28Background%20Music%29)))
      (:then_5
        (Actor|DestroyActor)
        (Default|SaveData (Variables|Default|GetBP_SaveLoadRHFps) (Utilities|Struct|MakeST_SaveLoad true 0 0)))
      (:then_6
        (Variables|/Game/ResidentHorrorFPS/Character/BP_Character/BP_RHV_FPS_Player.BP_RHV_FPS_Player_C|SetFinishing%20Sound (CallFunction|RHVFPSPlayerRef) (Variables|Default|GetSound%20Finish))))))

(event LoadedData(BP_SaveLoadRHFps)
  (params (Save%20Loaded%20Data :type ST%20Save%20Load%20Structure))
  ;[0 0 0 0.5] Load
  (if (.Boolean2 (Utilities|Struct|BreakST_SaveLoad Save%20Loaded%20Data))
    (Actor|DestroyActor)))

(fn ConstructionScript)