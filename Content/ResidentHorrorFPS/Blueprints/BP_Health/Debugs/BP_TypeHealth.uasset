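; Debug interactable actor that switches the player's health bar style between classic and normal.
; Each interaction uses a FlipFlop to set the health bar type enum on the player's HealthComponent, starting with classic.
; Every tick, its TextRender shows the name of the type currently set on that component.
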(event EventBeginPlay)

(event Collision|EventActorBeginOverlap
  (params (OtherActor :type Actor%20Object%20Reference)))

(event EventTick
  (params (DeltaSeconds :type Float%20%28single-precision%29))
  ;[0.15 0.15 0.15 0.5] Event Tick
  (Rendering|Components|TextRender|SetText (Variables|Default|GetTextRender) (Utilities|Select :Index (Variables|/Game/ResidentHorrorFPS/Blueprints/BP_Health/BPC_RHHealhtSystem.BPC_RHHealhtSystem_C|GetE%20Type%20Health%20Bar (Variables|/Game/ResidentHorrorFPS/Character/BP_Character/BP_RHV_FPS_Player.BP_RHV_FPS_Player_C|GetHealthComponent (CallFunction|RHVFPSPlayerRef))) :NewEnumerator0 (Variables|Default|GetNormal%20Bar) :NewEnumerator1 (Variables|Default|GetClassic%20Health%20Bar))))

(event EventInteraction
  (params (Player :type BP%20RHV%20FPS%20Player%20Object%20Reference) (AutoInteraction%28Non-Player%29 :type Boolean))
  (bind _player (CallFunction|RHVFPSPlayerRef))
  (bind _healthcomponent (Variables|/Game/ResidentHorrorFPS/Character/BP_Character/BP_RHV_FPS_Player.BP_RHV_FPS_Player_C|GetHealthComponent _player))
  ;[0.15 0.15 0.15 0.5] Interact
  (Utilities|FlowControl|FlipFlop
    (:A
      (Variables|/Game/ResidentHorrorFPS/Blueprints/BP_Health/BPC_RHHealhtSystem.BPC_RHHealhtSystem_C|SetE%20Type%20Health%20Bar _healthcomponent "NewEnumerator1"))
    (:B
      (Variables|/Game/ResidentHorrorFPS/Blueprints/BP_Health/BPC_RHHealhtSystem.BPC_RHHealhtSystem_C|SetE%20Type%20Health%20Bar _healthcomponent "NewEnumerator0"))))

(fn ConstructionScript)