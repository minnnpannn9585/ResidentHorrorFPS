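; Player health component for the horror FPS that applies clamped damage and healing, toggling an injured sound at low health.
; Damage adds camera shake and a hit sound; at zero health it plays the death animation, disables input, shows the death widget and switches music through BP_Music_Manager.
; Separate events time post-death stingers, plus optional player mourning and slow motion after AI deaths.
; Tick clears the player's enemy list while dead, working around stuck combat music.
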(event Custom|Post-mortem%20AI%20Event
  (params ({%20AI%20}%20%201st%20Post-Mortem%20Impact%20Sound%20Custom :type Sound%20Base%20Object%20Reference) ({%20AI%20}%20%20When%20the%20first%20sound%20plays,%20death%20occurs%20Custom :type Float%20%28double-precision%29) ({%20AI%20}%20%202nd%20sound:%20Post-mortem%20impact%20Custom :type Sound%20Base%20Object%20Reference) ({%20AI%20}%20When%20the%202nd%20Impact%20Sound%20Plays,%20Death%20Custom :type Float%20%28double-precision%29) (Does%20the%20Player%20Play%20a%20Sound%20When%20the%20AI%20Dies?%20Custom :type Boolean) (Player's%20Voice%20When%20the%20AI%20Dies%20Custom :type Sound%20Base%20Object%20Reference) (When%20does%20the%20game%20notify%20the%20player%20that%20the%20AI%20has%20died?%20Custom :type Float%20%28double-precision%29) (Anim%20Mourns%20the%20Death%20of%20AI%20Custom :type Animation%20Asset%20Object%20Reference) (Time%20of%20Mourning%20for%20the%20Death%20of%20AI%20Custom :type Float%20%28single-precision%29) (Does%20the%20Player%20Have%20an%20Animation%20After%20the%20AI%20Dies?%20Custom :type Boolean) (Leave%20It%20in%20Slow%20Motion%20After%20the%20Death%20of%20AI?%20Custom :type Boolean) (Play%20in%20slow%20motion%20after%20Custom%20: :type Float%20%28single-precision%29) (Slow%20Motion%20value%20Custom :type Float%20%28single-precision%29))
  ;[0 0 0] Play music after the AI's death
  (Utilities|FlowControl|Sequence
    (:then_0
      (Utilities|FlowControl|Delay {%20AI%20}%20%20When%20the%20first%20sound%20plays,%20death%20occurs%20Custom)
      (Audio|PlaySound2D {%20AI%20}%20%201st%20Post-Mortem%20Impact%20Sound%20Custom 1.0 1.0 0.0 0 0))
    (:then_1
      (Utilities|FlowControl|Delay {%20AI%20}%20When%20the%202nd%20Impact%20Sound%20Plays,%20Death%20Custom)
      (Audio|PlaySound2D {%20AI%20}%20%202nd%20sound:%20Post-mortem%20impact%20Custom 1.0 1.0 0.0 0 0)
      (if Does%20the%20Player%20Play%20a%20Sound%20When%20the%20AI%20Dies?%20Custom
        (Utilities|FlowControl|Delay When%20does%20the%20game%20notify%20the%20player%20that%20the%20AI%20has%20died?%20Custom)
        (Audio|PlaySound2D Player's%20Voice%20When%20the%20AI%20Dies%20Custom 1.0 1.0 0.0 0 0))
      (if Does%20the%20Player%20Have%20an%20Animation%20After%20the%20AI%20Dies?%20Custom
        (Utilities|FlowControl|Delay Time%20of%20Mourning%20for%20the%20Death%20of%20AI%20Custom)
        (Components|Animation|PlayAnimation (Variables|/Script/Engine.Character|GetMesh (CallFunction|RHVFPSPlayerRef)) Anim%20Mourns%20the%20Death%20of%20AI%20Custom false))
      (if Leave%20It%20in%20Slow%20Motion%20After%20the%20Death%20of%20AI?%20Custom
        (Utilities|FlowControl|Delay Play%20in%20slow%20motion%20after%20Custom%20:)
        (Utilities|Time|SetGlobalTimeDilation Slow%20Motion%20value%20Custom)))))

(event Custom|Play%20music%20after%20death
  (params (1.%20Sound%20Impact%20After%20Death :type Sound%20Base%20Object%20Reference) (When%20the%20First%20Sound%20Plays:%20Instant%20Death :type Float%20%28double-precision%29) (2nd%20track:%20“Impact%20After%20Death” :type Sound%20Base%20Object%20Reference) (When%20the%202nd%20Impact%20Sound%20Plays,%20Death :type Float%20%28double-precision%29))
  ;[0 0 0] Play music after death
  (Utilities|FlowControl|Sequence
    (:then_0
      (Utilities|FlowControl|Delay When%20the%20First%20Sound%20Plays:%20Instant%20Death)
      (Audio|PlaySound2D 1.%20Sound%20Impact%20After%20Death 1.0 1.0 0.0 0 0))
    (:then_1
      (Utilities|FlowControl|Delay When%20the%202nd%20Impact%20Sound%20Plays,%20Death)
      (Audio|PlaySound2D 2nd%20track:%20“Impact%20After%20Death” 1.0 1.0 0.0 0 0))))

(event EventTick
  (params (DeltaSeconds :type Float%20%28single-precision%29))
  ;[0 0 0] Event Tick
  (|ForceFinishMusicCombat) ; I created these nodes here because for some reason, when the companion dies, the combat music doesn't stop, so with this, the event tick forces it to pause.
)

(fn TakeDamage
  (params (Damage :type Float%20%28double-precision%29) (Hit%20Result :type Hit%20Result%20Structure))
  (bind _returnvalue (Game|GetPlayerController 0))
  ;[0 0 0 0.5] Verification Dead Character Main
  (if (not (Variables|Default|GetPlayer%20Dead?))
    ;[0 0 0 0.5] Verification Health
    (bind _output_get (Variables|HPPLAYER|SetCurrent%20Hp (Math|Float|Clamp(Float) (- (Variables|HPPLAYER|GetCurrent%20Hp) Damage) 0.0 (Variables|HPPLAYER|GetMaxHp))))
    (if (<= _output_get 32.0)
      ;[0 0 0 0.5] Injured Pose
      (if (not (Variables|Default|GetPlay%20Sound%20Injured?))
        (Audio|Components|Audio|SetSound (Variables|/Game/ResidentHorrorFPS/Character/BP_Character/BP_RHV_FPS_Player.BP_RHV_FPS_Player_C|GetAll%20Sound%20Player (CallFunction|RHVFPSPlayerRef)) (Variables|/Game/ResidentHorrorFPS/Blueprints/BP_DataAsset/DA_CustomCharacter/DA_SettingsCharacter.DA_SettingsCharacter_C|GetInjured%20Sound (Variables|Default|GetDA_SettingsCharacter)))
        (Audio|Components|Audio|Play (Variables|/Game/ResidentHorrorFPS/Character/BP_Character/BP_RHV_FPS_Player.BP_RHV_FPS_Player_C|GetAll%20Sound%20Player (CallFunction|RHVFPSPlayerRef)) 0.0)
        (Variables|Default|SetPlay%20Sound%20Injured? true)))
    ;[0 0 0 0.5] Play Camera Shake Hit
    (Camera|PlayWorldCameraShake (Variables|/Game/ResidentHorrorFPS/Blueprints/BP_DataAsset/DA_CustomCharacter/DA_SettingsCharacter.DA_SettingsCharacter_C|GetShake%20Damage (Variables|Default|GetDA_SettingsCharacter)) (Transformation|GetActorLocation (CallFunction|RHVFPSPlayerRef)) 1.0 4.5e+02)
    ;[0 0 0 0.5] Sound Damage
    (Audio|Components|Audio|SetSound (Variables|/Game/ResidentHorrorFPS/Character/BP_Character/BP_RHV_FPS_Player.BP_RHV_FPS_Player_C|GetAudio%20Character (CallFunction|RHVFPSPlayerRef)) (Variables|Sounds|GetSound%20Damage))
    (Audio|Components|Audio|Play (Variables|/Game/ResidentHorrorFPS/Character/BP_Character/BP_RHV_FPS_Player.BP_RHV_FPS_Player_C|GetAudio%20Character (CallFunction|RHVFPSPlayerRef)) 0.0)
    ;[0 0 0 0.5] Dead?
    (if (<= _output_get 0.0)
      (Default|CallHealthDepleted) ; Notify when the battery is low
      ;[0 0 0 0.5] Play Animation Dead
      (Components|Animation|PlayAnimation (Variables|/Script/Engine.Character|GetMesh (CallFunction|RHVFPSPlayerRef)) "/Game/ResidentHorrorFPS/Character/Animations/AS_Zombie_Death.AS_Zombie_Death" false)
      ;[0 0 0 0.5] True Dead
      (Variables|Default|SetPlayer%20Dead? true)
      ;[0 0 0 0.5] Widget Animation Dead
      (bind _returnvalue_2 (UserInterface|CreateWidget "/Game/ResidentHorrorFPS/Blueprints/WBP/Player/WBP_Dead.WBP_Dead_C"))
      (UserInterface|Viewport|AddtoViewport _returnvalue_2 0)
      (Input|DisableInput (CallFunction|RHVFPSPlayerRef) _returnvalue)
      (Variables|/Script/Engine.PlayerController|SetbShowMouseCursor _returnvalue true)
      (Input|SetInputModeGameandUI _returnvalue _returnvalue_2 "DoNotLock" true false)
      ;[0 0 0 0.5] Stop Music Dead
      (Audio|Components|Audio|Stop (Variables|/Game/ResidentHorrorFPS/Character/BP_Character/BP_RHV_FPS_Player.BP_RHV_FPS_Player_C|GetAll%20Sound%20Player (CallFunction|RHVFPSPlayerRef)))
      (bind _returnvalue_3 (Actor|GetActorOfClass "/Game/ResidentHorrorFPS/Blueprints/BP_MusicManager/BP_Music_Manager.BP_Music_Manager_C"))
      (Utilities|IsValid _returnvalue_3
        (:Is%20Valid
          (Default|StartMusicAmbient _returnvalue_3 (Variables|MusicofDeath|GetSound%20Dead) 0.4 (Variables|MusicofDeath|GetFade%20in%20%28Music%20Dead%29) 0.0 false)
          (Utilities|Array|Clear (Variables|/Game/ResidentHorrorFPS/Character/BP_Character/BP_RHV_FPS_Player.BP_RHV_FPS_Player_C|GetEnemies%20fighting%20me (CallFunction|RHVFPSPlayerRef)))
          (Default|FinsherMusicCombat _returnvalue_3 "/Engine/EngineSounds/1kSineTonePing.1kSineTonePing" 0.0 0.0)
          ;[0 0 0 0.5] Play Music Dead
          (CallFunction|PlayMusicAfterDeath (Variables|FirstSound:ImpactAfterDeath|Get1%20Post-Mortem%20Impact%20Sound) (Variables|FirstSound:ImpactAfterDeath|GetWhen%20the%20first%20sound%20is%20heard,%20death%20strikes) (Variables|2ndSound:Post-MortemImpact|Get2nd%20track:%20“Impact%20After%20Death”) (Variables|2ndSound:Post-MortemImpact|GetWhen%20the%202nd%20Impact%20Sound%20Plays,%20Death)))))))

(fn TakeHealing
  (params (Healing%20Amount :type Float%20%28double-precision%29))
  (bind _player (CallFunction|RHVFPSPlayerRef))
  (bind _audio_character (Variables|/Game/ResidentHorrorFPS/Character/BP_Character/BP_RHV_FPS_Player.BP_RHV_FPS_Player_C|GetAudio%20Character _player))
  (CallFunction|DebugHealth "(R=0.152434,G=1.000000,B=0.176967,A=1.000000)" (Variables|Debug?|GetDebug%20Health?) Healing%20Amount "LIFE RECOVERED IN:")
  (bind _output_get (Variables|HPPLAYER|SetCurrent%20Hp (Math|Float|Clamp(Float) (+ (Variables|HPPLAYER|GetCurrent%20Hp) Healing%20Amount) 0.0 (Variables|HPPLAYER|GetMaxHp))))
  (Variables|HPPLAYER|SetMax%20Hp%20of%20game _output_get)
  (Audio|Components|Audio|SetSound _audio_character (Variables|Sounds|GetSound%20Healling))
  (Audio|Components|Audio|Play _audio_character 0.0)
  (if (>= (Variables|HPPLAYER|GetCurrent%20Hp) 33.0)
    (if (Variables|Default|GetPlay%20Sound%20Injured?)
      (Audio|Components|Audio|Stop (Variables|/Game/ResidentHorrorFPS/Character/BP_Character/BP_RHV_FPS_Player.BP_RHV_FPS_Player_C|GetAll%20Sound%20Player (CallFunction|RHVFPSPlayerRef)))
      (Variables|Default|SetPlay%20Sound%20Injured? false))))

(fn DebugHealth
  (params (TextColor :type Linear%20Color%20Structure) (InputPin :type Boolean) (InDouble :type Float%20%28double-precision%29) (A :type String))
  (if InputPin
    (Development|PrintString (Utilities|String|Append A (Utilities|String|ToString(Float) InDouble)) true true TextColor InDouble)))