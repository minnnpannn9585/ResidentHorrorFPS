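; Crow Blueprint child, named as a spline variant, that decides when to trigger the StartFlight call it uses to take off.
; Flight can start on BeginPlay after a configurable delay, or when actors tagged as main character, vehicle or AI enemy overlap its spheres.
; Sphere additionally requires the CrowPlane flag and a player-controlled pawn, while Sphere1 reacts to any tagged actor.
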(event OnComponentBeginOverlap(Sphere)
  (params (OverlappedComponent :type Primitive%20Component%20Object%20Reference) (OtherActor :type Actor%20Object%20Reference) (OtherComp :type Primitive%20Component%20Object%20Reference) (OtherBodyIndex :type Integer) (bFromSweep :type Boolean) (SweepResult :type Hit%20Result%20Structure%20%28by%20ref%29))
  ;[0 0 0 0.5 37] Fly
  (if (Variables|Default|GetCrow%20Plane?)
    (bind _aspawn (Utilities|Casting|CastToPawn OtherActor))
    (if (CallFunction|ActoTag? OtherActor OtherActor OtherActor)
      (if (Pawn|IsPlayerControlled _aspawn)
        (CallFunction|StartFlight)))))

(event OnComponentBeginOverlap(Sphere1)
  (params (OverlappedComponent :type Primitive%20Component%20Object%20Reference) (OtherActor :type Actor%20Object%20Reference) (OtherComp :type Primitive%20Component%20Object%20Reference) (OtherBodyIndex :type Integer) (bFromSweep :type Boolean) (SweepResult :type Hit%20Result%20Structure%20%28by%20ref%29))
  ;[0 0 0 0.5 37] Fly
  (if (CallFunction|ActoTag? OtherActor OtherActor OtherActor)
    (CallFunction|StartFlight)))

(event EventBeginPlay
  (if (Variables|Default|GetStart%20Flight?)
    (Utilities|FlowControl|Delay (Variables|Default|GetDelay%20Start%20Flight))
    (CallFunction|StartFlight)))

(fn ConstructionScript
  (|CallParentFunction))

(fn ActoTag?
  (params (AiEnemy :type Actor%20Object%20Reference) (CharacterMain :type Actor%20Object%20Reference) (Vehicle :type Actor%20Object%20Reference))
  (return (Math|Boolean|ORBoolean (Actor|ActorHasTag CharacterMain "CharacterMain") (Actor|ActorHasTag Vehicle "Vehicle") (Actor|ActorHasTag AiEnemy "AITag01"))))