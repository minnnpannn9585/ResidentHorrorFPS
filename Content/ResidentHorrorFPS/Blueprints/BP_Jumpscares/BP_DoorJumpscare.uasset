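; Door jumpscare Blueprint that slams a partly open door shut when its OverlapJumpscare event fires.
; A timeline lerps the DoorClose component's yaw to its closed angle, while a short delay leads into the Sound event.
; Sound plays at a location taken from the Door's world scale rather than its world position.
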(event Custom|Sound
  ;[0.15 0.15 0.15 0.5] Sound
  (Audio|PlaySoundatLocation 0 (Transformation|GetWorldScale (Variables|Default|GetDoor)) "0, 0, 0" 4.0 1.0 0.0 0 0 0 0))

(event EventOverlapJumpscare
  ;[0.15 0.15 0.15 0.5] close door
  (Utilities|FlowControl|Sequence
    (:then_0
      (bind _closedoor (Timeline|Close%20door%20Timeline Play)
        (:Update
          (Transformation|SetRelativeRotation (Variables|Default|GetDoorClose) (Math|Rotator|MakeRotator 0.0 0.0 (Math|Float|Lerp -4e+01 0.0 _closedoor)) false false))))
    (:then_1
      (Utilities|FlowControl|Delay 0.3)
      (CallFunction|Sound))))

(fn ConstructionScript)