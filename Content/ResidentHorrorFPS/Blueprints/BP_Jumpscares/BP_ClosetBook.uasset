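; BP_ClosetBook is a jumpscare prop that flings a set of book meshes on demand.
; Its FlipBook event loops over a hand-built array of book static mesh components, plus one found by class lookup.
; Each gets an impulse along its own forward vector at a random strength between ForceMin and ForceMax, applied as a velocity change so mass is ignored.
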(event EventFlipBook
  ;[0.15 0.15 0.15 0.5] Impulse
  (for _array_element (Utilities|Array|MakeArray (Actor|GetComponentbyClass "/Script/Engine.StaticMeshComponent") (Variables|Default|GetSM_Book1) (Variables|Default|GetSM_Book2) (Variables|Default|GetSM_Book3) (Variables|Default|GetSM_Book4) (Variables|Default|GetSM_Book5) (Variables|Default|GetSM_Book) (Variables|Default|GetSM_Book9) (Variables|Default|GetSM_Book8) (Variables|Default|GetSM_Book3) (Variables|Default|GetSM_Book4) (Variables|Default|GetSM_Book) (Variables|Default|GetSM_Book18) (Variables|Default|GetSM_Book12) (Variables|Default|GetSM_Book17) (Variables|Default|GetSM_Book19))
    (Physics|AddImpulse _array_element (* (Math|Vector|GetForwardVector _array_element) (Math|Random|RandomFloatinRange (Variables|Default|GetForce%20Min) (Variables|Default|GetForce%20Max))) "None" true)))

(fn ConstructionScript)