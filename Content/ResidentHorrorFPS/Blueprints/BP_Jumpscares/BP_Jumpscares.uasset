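; Placeable jumpscare trigger that fires when the player overlaps it, running a monster, door or book scare chosen by enum.
; Monster mode plays a looping run animation while sliding the mesh to a target point, then destroys the actor.
; Door and book modes message a referenced actor, then destroy themselves.
; All modes play a 2D sting plus a delayed positional voice; the construction script shows monster components only in that mode.
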(event OnComponentBeginOverlap(OverlapScare)
  (params (OverlappedComponent :type Primitive%20Component%20Object%20Reference) (OtherActor :type Actor%20Object%20Reference) (OtherComp :type Primitive%20Component%20Object%20Reference) (OtherBodyIndex :type Integer) (bFromSweep :type Boolean) (SweepResult :type Hit%20Result%20Structure%20%28by%20ref%29))
  ;[0.15 0.15 0.15 0.5] Overlap
  (if (== OtherActor (CallFunction|RHVFPSPlayerRef))
    (CallFunction|EventJumpscare)))

(event Custom|Event%20Jumpscare
  ;[0.15 0.15 0.15 0.5] Event Jumpscare
  (switch Utilities|FlowControl|Switch|SwitchonE_Jumpscare (Variables|Default|GetE_Jumpscare)
    (:NewEnumerator0
      (CallFunction|JumpscareMonster))
    (:NewEnumerator1
      (CallFunction|JumpscareDoor))
    (:NewEnumerator3
      (CallFunction|FlipbookJumpscare))))

(event Custom|Jumpscare%20Monster
  (Utilities|FlowControl|Sequence
    (:then_0
      ;[0.15 0.15 0.15 0.5] Mover Enemy
      (Components|MoveComponentTo (Variables|Default|GetSkeletalMesh) (Variables|/Script/Engine.SceneComponent|GetRelativeLocation (Variables|Default|GetPoint%20Move)) "0, 0, 0" false false (Variables|Default|GetSpeed) false)
      (Actor|DestroyActor))
    (:then_1
      (Utilities|FlowControl|Sequence
        (:then_0
          ;[0.15 0.15 0.15 0.5] Play animation
          (Components|Animation|PlayAnimation (Variables|Default|GetSkeletalMesh) "/Game/ResidentHorrorFPS/Character/Animations/Locomotion/AS_N_Run_F.AS_N_Run_F" true)
          ;[0.15 0.15 0.15 0.5] Disable Collision
          (Collision|SetCollisionEnabled (Variables|Default|GetOverlapScare) "NoCollision")
          (Collision|SetCollisionResponsetoAllChannels (Variables|Default|GetOverlapScare) "ECR_Ignore"))
        (:then_1
          ;[0.15 0.15 0.15 0.5] Sounds
          (CallFunction|SoundPlay))))))

(event Custom|Jumpscare%20Door
  ;[0.15 0.15 0.15 0.5] Jumpscare Door
  (Utilities|IsValid (Variables|Default|GetDoor)
    (:Is%20Valid
      (Class|BPIJumpscare|OverlapJumpscare(Message) (Variables|Default|GetDoor))
      (CallFunction|SoundPlay)
      (Actor|DestroyActor))))

(event Custom|Sound%20Play
  ;[0.15 0.15 0.15 0.5] Sounds
  (Utilities|FlowControl|Sequence
    (:then_0
      (Utilities|FlowControl|Delay (Variables|Default|GetWhen%20will%20the%20audio%20play?))
      (Audio|SpawnSoundatLocation (Variables|Default|GetSound%20Jumpscare%20Voice) (Transformation|GetActorLocation) "0, 0, 0" 2.0 1.0 0.0 0 0))
    (:then_1
      (Audio|PlaySound2D (Variables|Default|GetSound%20Jumpscare) 2.0 1.0 0.0 0 0))))

(event Custom|FlipbookJumpscare
  ;[0.15 0.15 0.15 0.5] FlipbookJumpscare
  (Utilities|IsValid (Variables|Default|GetBP%20BookJumpscare)
    (:Is%20Valid
      (Class|BPIJumpscare|FlipBook(Message) (Variables|Default|GetBP%20BookJumpscare))
      (CallFunction|SoundPlay)
      (Actor|DestroyActor))))

(fn ConstructionScript
  (CallFunction|SwitchVisibility))

(fn SwitchVisibility
  (switch Utilities|FlowControl|Switch|SwitchonE_Jumpscare (Variables|Default|GetE_Jumpscare)
    (:NewEnumerator0
      (Rendering|SetVisibility (Variables|Default|GetSkeletalMesh) true false))
    (:NewEnumerator1
      (Rendering|SetVisibility (Variables|Default|GetSkeletalMesh) false false :!label _label))
    (:NewEnumerator3
      (goto _label))))