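; Interactable switch that toggles between on and off and sends an activation message to a linked target actor.
; Interaction locks input and lerps the player and view to preset points, then plays a montage, using the held item's variant if available.
; The montage notify plays a click, signals the target and runs a timeline forward or backward to rotate the switch.
; The save component stores switch state and rotation and reapplies them on load.
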(event LoadedData(BP_SaveLoadRHFps)
  (params (Save%20Loaded%20Data :type ST%20Save%20Load%20Structure))
  (bind (_boolean2 _boolean4 _rotator) (Utilities|Struct|BreakST_SaveLoad Save%20Loaded%20Data))
  ;[0 0 0 0.5] Load
  (if _boolean2
    (if _boolean4
      (CallFunction|ReversAnimation)
      (else
        (Transformation|SetRelativeRotation (Variables|Default|GetSwitch) _rotator false false)
        ;[0 0 0 0.5] activae light
        (Class|BPIActivation|Activation(Message) (Variables|Default|GetTargetActivationActor))))))

(event Custom|Interact%20Play%20Animation
  (bind _returnvalue (Game|GetPlayerController 0))
  (bind _player (Variables|Default|GetPlayer))
  (bind _bpc_equipment (Variables|/Game/ResidentHorrorFPS/Character/BP_Character/BP_RHV_FPS_Player.BP_RHV_FPS_Player_C|GetBPC_Equipment _player))
  (bind _child_actor (Default|GetCurrentHandItem _bpc_equipment))
  (bind _interactanimation (Class|BPIConstantUse|GetInteractAnimation(Message) _child_actor))
  (bind _notifyname (Animation|Montage|PlayMontage (Variables|/Script/Engine.Character|GetMesh (Variables|Default|GetPlayer)) (select (Utilities|IsValid _child_actor) (Utilities|Struct|BreakST_InteractionAnimation _interactanimation) (Variables|Default|GetMontage%20to%20Play)))
    (:then
      (Default|UpdateGlobalState (Variables|Default|GetPlayer) "NewEnumerator1")
      (Timeline|FocuseCamera Play
        (:Update
          (Pawn|SetControlRotation _returnvalue (Math|Interpolation|RInterpTo (Pawn|GetControlRotation _returnvalue :!class /Script/Engine.Controller) (Transformation|GetWorldRotation (Variables|Default|GetFocusePoint)) (Utilities|Time|GetWorldDeltaSeconds) 15.0)))))
    (:OnCompleted
      (Input|EnableInput (Game|GetPlayerCharacter 0) (Game|GetPlayerController 0))
      (Default|UpdateGlobalState (Variables|Default|GetPlayer) "NewEnumerator0")
      (Input|ResetIgnoreLookInput (Game|GetPlayerController 0))
      (CallFunction|ResetInteraction)
      (Timeline|FocuseCamera Stop))
    (:OnNotifyBegin
      (switch name _notifyname
        (:Tuch
          (Audio|PlaySoundatLocation "/Game/ResidentHorrorFPS/Audio/Wavs/WAV_ui-click-43196.WAV_ui-click-43196" (Transformation|GetWorldLocation (Variables|Default|GetRoot)) "0, 0, 0" 1.0 1.0 0.0 "/Game/ResidentHorrorFPS/Audio/Attenuation/Att_ImpactsAttenuation.Att_ImpactsAttenuation" 0 0 0)
          ;[0.15 0.15 0.15 0.5] activae light
          (Class|BPIActivation|Activation(Message) (Variables|Default|GetTargetActivationActor))
          (if (Variables|Default|GetOff)
            (CallFunction|ReversAnimation)
            (else
              (CallFunction|ForwardAnimation))))))))

(event Custom|ForwardAnimation
  ;[0 0 0] Static Mesh Animation Time Line
  (bind (_direction _rotationalpha) (Timeline|Timeline Play)
    (:Update
      (Transformation|SetRelativeRotation (Variables|Default|GetSwitch) (Math|Rotator|Lerp(Rotator) "0.000000,0.000000,-20.000000" "0, 0, 0" _rotationalpha true) false false))
    (:Finished
      (bind _output_get (Variables|Default|SetOff (Utilities|Select :Index _direction :Forward true :Backward false)))
      (Collision|SetActorEnableCollision true)
      (Default|SaveData (Variables|Default|GetBP_SaveLoadRHFps) (Utilities|Struct|MakeST_SaveLoad true _output_get (Variables|/Script/Engine.SceneComponent|GetRelativeRotation (Variables|Default|GetSwitch)))))))

(event Custom|ResetInteraction
  ;[0 0 0] Interaction
  (Utilities|FlowControl|DoOnce false) ; enters at Reset
)

(event Custom|StopInteraction
  ;[0 0 0] Stop Interaction
  (CallFunction|ResetInteraction)
  (bind _player (Variables|Default|GetPlayer)
    (:then
      (if (Animation|Montage|MontageIsPlaying (Variables|/Game/ResidentHorrorFPS/Character/BP_Character/BP_RHV_FPS_Player.BP_RHV_FPS_Player_C|GetABP%20RHFPS _player) (Variables|Default|GetMontage%20to%20Play))
        (Animation|Montage|MontageStop (Variables|/Game/ResidentHorrorFPS/Character/BP_Character/BP_RHV_FPS_Player.BP_RHV_FPS_Player_C|GetABP%20RHFPS _player) 0.25 (Variables|Default|GetMontage%20to%20Play))
        (CallFunction|VisibilityWidgetChange true)))
    (:else)))

(event Custom|ReversAnimation
  ;[0 0 0] Static Mesh Animation Time Line
  (bind (_direction _rotationalpha) (Timeline|Timeline ReverseFromEnd)
    (:Update
      (Transformation|SetRelativeRotation (Variables|Default|GetSwitch) (Math|Rotator|Lerp(Rotator) "0.000000,0.000000,-20.000000" "0, 0, 0" _rotationalpha true) false false))
    (:Finished
      (bind _output_get (Variables|Default|SetOff (Utilities|Select :Index _direction :Forward true :Backward false)))
      (Collision|SetActorEnableCollision true)
      (Default|SaveData (Variables|Default|GetBP_SaveLoadRHFps) (Utilities|Struct|MakeST_SaveLoad true _output_get (Variables|/Script/Engine.SceneComponent|GetRelativeRotation (Variables|Default|GetSwitch)))))))

(event Custom|SetPositionAndControlRotationPlayer
  (bind _returnvalue (Game|GetPlayerController 0))
  (bind _playerposition (Variables|Default|GetPlayerPosition))
  (bind _returnvalue_2 (Transformation|GetWorldLocation _playerposition))
  ;[0 0 0] PlayerPosition
  (Input|DisableInput (Variables|Default|GetPlayer) _returnvalue)
  (Input|SetIgnoreLookInput _returnvalue true)
  (bind _positionalpha (Timeline|Timeline_0 PlayFromStart)
    (:Update
      (CallFunction|SetControlRotation (Transformation|GetWorldRotation (Variables|Default|GetFocusePoint)) _positionalpha)
      (CallFunction|SetPlayerLocation (Math|Vector|MakeVector (.x _returnvalue_2) (.y _returnvalue_2) (.z (Transformation|GetActorLocation (Variables|Default|GetPlayer)))) _positionalpha))
    (:Finished
      (CallFunction|InteractPlayAnimation))))

(event EventBeginPlay
  ;[0 0 0] Begin Play
  (|CallParentFunction)
  (Class|BPIInteractWidget|AddInteractInfo(Message) (UserInterface|GetWidget (Variables|Default|GetInteractWidget_0)) "/ControlRigModules/Modules/Icons/ModRigHand256.ModRigHand256"))

(event EventInteraction
  (params (Player :type BP%20RHV%20FPS%20Player%20Object%20Reference) (AutoInteraction%28Non-Player%29 :type Boolean))
  ;[0 0 0] Interaction
  (Variables|Default|SetPlayer Player)
  (CallFunction|VisibilityWidgetChange false)
  (Utilities|FlowControl|DoOnce false
    (:Completed
      (CallFunction|SetPositionandControlRotationPlayer)
      (Collision|SetActorEnableCollision false))))

(fn ConstructionScript)

(fn SetControlRotation
  (params (NewRotation :type Rotator) (Alpha :type Float%20%28single-precision%29))
  (bind _returnvalue (Game|GetPlayerController 0))
  (Pawn|SetControlRotation _returnvalue (Math|Rotator|Lerp(Rotator) (Pawn|GetControlRotation _returnvalue :!class /Script/Engine.Controller) NewRotation Alpha true)))

(fn SetPlayerLocation
  (params (NewLocation :type Vector) (Alpha :type Float%20%28single-precision%29))
  (Transformation|SetActorLocation (Variables|Default|GetPlayer) (Math|Vector|Lerp(Vector) (Transformation|GetActorLocation (Variables|Default|GetPlayer)) NewLocation Alpha) false false))