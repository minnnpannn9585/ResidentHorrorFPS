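; BP_NameLocalText is a one-shot trigger box, resizable in the editor, that shows a location name on screen when the player enters it.
; On player overlap it waits a set delay, creates a WBP_LocalName widget, plays a sound and passes the text to the widget.
; It then saves a triggered flag through SaveLoadComponent and destroys itself, and destroys itself again on load if that flag is set.
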(event OnComponentBeginOverlap(Box)
  (params (OverlappedComponent :type Primitive%20Component%20Object%20Reference) (OtherActor :type Actor%20Object%20Reference) (OtherComp :type Primitive%20Component%20Object%20Reference) (OtherBodyIndex :type Integer) (bFromSweep :type Boolean) (SweepResult :type Hit%20Result%20Structure%20%28by%20ref%29))
  ;[0 0 0] THIS CODE DISPLAYS THE NAME ON THE SCREEN
  (if (== OtherActor (Game|GetPlayerCharacter 0))
    (Utilities|FlowControl|Delay (Variables|Default|GetDuration))
    (bind _returnvalue (UserInterface|CreateWidget "/Game/ResidentHorrorFPS/Blueprints/BP_NameScreenLocal/WBP_LocalName.WBP_LocalName_C"))
    (bind _output_get (Variables|Default|SetWB%20LOCAL _returnvalue))
    (UserInterface|Viewport|AddtoViewport _output_get 0)
    (Audio|PlaySound2D (Variables|Default|GetSound%20when%20the%20trigger%20is%20pressed) 1.0 1.0 0.0 0 0)
    (Default|EventWrite (Variables|Default|GetWB%20LOCAL) (Variables|Default|GetText?))
    (Default|SaveData (Variables|Default|GetSaveLoadComponent) (Utilities|Struct|MakeST_SaveLoad true 0 0))
    (Actor|DestroyActor)))

(event LoadedData(SaveLoadComponent)
  (params (Save%20Loaded%20Data :type ST%20Save%20Load%20Structure))
  ;[0.15 0.15 0.15 0.5] Load
  (if (.Boolean4 (Utilities|Struct|BreakST_SaveLoad Save%20Loaded%20Data))
    (Actor|DestroyActor)))

(fn ConstructionScript
  (Components|Box|SetBoxExtent (Variables|Default|GetBox) (Variables|Default|GetSize) true))