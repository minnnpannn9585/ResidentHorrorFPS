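; Drag-and-drop operation that carries an item while it is dragged in the grid-based inventory.
; It holds the item object, source inventory, tile and rotation state, exposed through simple getters.
; Rotation requests are forwarded to the drag widget.
; A cancelled drag re-adds the item at its stored tile, converted to an index, and fires the inventory-changed notification if the inventory is still valid.
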(event EventDragCancelled
  (params (PointerEvent :type Pointer%20Event%20Structure%20%28by%20ref%29))
  ;[0 0 0 0.5] Cancelled Drag
  (bind _inventory (Variables|Default|GetInventory)
    (:then
      (Default|AddItem _inventory (Default|TiletoIndex _inventory (Variables|Default|GetCurrentTile)) (Variables|Default|GetItemObject))
      (Default|CallOnInventoryChanged (Variables|Default|GetInventory)))
    (:else)))

(fn RotateSlot
  (Default|Rotate (Variables|Default|GetDragWidget))
  (return))

(fn GetCurrentTile
  (return (Variables|Default|GetCurrentTile) (Variables|Default|GetRotate?) (Variables|Default|GetInventory)))

(fn GetItemObject
  (return (Variables|Default|GetItemObject)))

(fn GetOperation
  (return self))