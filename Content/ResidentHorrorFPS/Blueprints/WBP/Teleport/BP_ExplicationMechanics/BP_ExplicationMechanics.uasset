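; BP_ExplicationMechanics is a proximity trigger that shows a mechanics explanation widget to the player.
; A second after BeginPlay, its Sphere switches to overlap all channels.
; When the RHVFPS player enters, it creates and caches WBP_ExplicationMechanics once, plays its fade animation and displays it in the ExplicationBP widget component.
; Leaving the sphere hides that component; the exit event does not check which actor left.
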(event OnComponentBeginOverlap(Sphere)
  (params (OverlappedComponent :type Primitive%20Component%20Object%20Reference) (OtherActor :type Actor%20Object%20Reference) (OtherComp :type Primitive%20Component%20Object%20Reference) (OtherBodyIndex :type Integer) (bFromSweep :type Boolean) (SweepResult :type Hit%20Result%20Structure%20%28by%20ref%29))
  ;[0 0 0 0.5] Begin Overlap
  (if (== OtherActor (CallFunction|RHVFPSPlayerRef))
    (Variables|Default|GetBP%20Explication
      (:then
        _)
      (:else
        (bind _returnvalue (UserInterface|CreateWidget "/Game/ResidentHorrorFPS/Blueprints/WBP/Teleport/BP_ExplicationMechanics/WBP_ExplicationMechanics.WBP_ExplicationMechanics_C" 0 self))
        (bind _output_get (Variables|Default|SetBP%20Explication _returnvalue))))
    (Default|FadAnim (Variables|Default|GetBP%20Explication) "Forward")
    (Rendering|SetVisibility (Variables|Default|GetExplicationBP) true true)
    (UserInterface|SetWidget (Variables|Default|GetExplicationBP) _output_get)))

(event OnComponentEndOverlap(Sphere)
  (params (OverlappedComponent :type Primitive%20Component%20Object%20Reference) (OtherActor :type Actor%20Object%20Reference) (OtherComp :type Primitive%20Component%20Object%20Reference) (OtherBodyIndex :type Integer))
  ;[0 0 0 0.5] End Overlap
  (Variables|Default|GetBP%20Explication
    (:then
      (Rendering|SetVisibility (Variables|Default|GetExplicationBP) false false))
    (:else)))

(event EventBeginPlay
  (bind _sphere (Variables|Default|GetSphere))
  ;[0 0 0 0.5] Begim Play Validate Collision
  (Utilities|FlowControl|Delay 1.0)
  (Collision|SetCollisionResponsetoAllChannels _sphere "ECR_Overlap")
  (Collision|SetCollisionEnabled _sphere "QueryAndPhysics"))

(fn ConstructionScript)