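; Trigger-box teleporter that sends the player to a named destination on overlap, with its WriteDestination name shown on a TextRender by the construction script.
; The Teleport macro or event briefly slows global time, then searches all BP_TeleportWidget actors for a matching TeleportName.
; On a match it moves and reorients the player and restores time, with sound and post-process effects.
; A parallel sequence branch restores game-only input and hides the cursor.
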(event OnComponentBeginOverlap(Box)
  (params (OverlappedComponent :type Primitive%20Component%20Object%20Reference) (OtherActor :type Actor%20Object%20Reference) (OtherComp :type Primitive%20Component%20Object%20Reference) (OtherBodyIndex :type Integer) (bFromSweep :type Boolean) (SweepResult :type Hit%20Result%20Structure%20%28by%20ref%29))
  ;[0 0 0 0.5] Teleport
  (if (== OtherActor (CallFunction|RHVFPSPlayerRef))
    (Utilities|Teleport (Variables|Default|GetWrite%20destination))))

(fn ConstructionScript
  (Rendering|Components|TextRender|SetText (Variables|Default|GetTextRender) (Utilities|Text|ToText(Name) (Variables|Default|GetWrite%20destination))))