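; Footstep anim notify that plays surface-specific sounds and Niagara effects for the resident horror FPS.
; A short line trace at the left or right foot socket, or mesh origin, reads the physical surface to pick assets from data assets, with an optional extra sound.
; Blood surfaces set a player flag that leaves fading footprint decals, and water clears it.
; Foley tag and audio bank helpers exist, but ReceivedNotify does not call them.
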(fn ReceivedNotify
  (params (MeshComp :type Skeletal%20Mesh%20Component%20Object%20Reference) (Animation :type Anim%20Sequence%20Base%20Object%20Reference) (EventReference :type Anim%20Notify%20Event%20Reference%20Structure%20%28by%20ref%29))
  (bind _player (CallFunction|RHVFPSPlayerRef))
  (bind _player_2 (CallFunction|RHVFPSPlayerRef))
  (bind _da_footstep (Variables|Default|GetDA_Footstep))
  (bind _volumemultiplier (Variables|Default|GetVolumeMultiplier))
  (bind _volumemultiplier_2 (Variables|Default|GetVolumeMultiplier))
  (bind _volumemultiplier_3 (Variables|Default|GetVolumeMultiplier))
  (bind _side (Variables|Default|GetSide))
  (bind _da_niagarafx (Variables|Default|GetDA_NiagaraFx))
  (bind _returnvalue (Transformation|GetWorldLocation MeshComp))
  (bind _returnvalue_2 (Transformation|GetSocketLocation MeshComp "Footstep_R"))
  (bind _returnvalue_3 (Transformation|GetSocketLocation MeshComp "Footstep_L"))
  (bind _returnvalue_4 (Utilities|Select :Index _side :NewEnumerator4 _returnvalue :NewEnumerator0 _returnvalue_3 :NewEnumerator2 _returnvalue_2))
  ;[0 0 0 0.5] Trace Spawn Sound and Visual Effects
  (Utilities|IsValid MeshComp
    (:Is%20Valid
      (Utilities|IsValid Animation
        (:Is%20Valid
          (bind (_outhit _returnvalue_5) (Collision|LineTraceByChannel (+ _returnvalue_4 "0.000000,0.000000,15.000000") (+ _returnvalue_4 "0.000000,0.000000,-15.000000") "TraceTypeQuery1" true 0 "None" true "(R=1.000000,G=0.000000,B=0.000000,A=1.000000)" "(R=0.000000,G=1.000000,B=0.000000,A=1.000000)" 1.0))
          (if _returnvalue_5
            (Niagara|SpawnSystematLocation (Utilities|Select :Index (Collision|GetSurfaceType _outhit) :SurfaceType_Default (Variables|/Game/ResidentHorrorFPS/Blueprints/BP_DataAsset/DA_Footstep/VisualEffects/DA_FootstepEffects.DA_FootstepEffects_C|GetDefault%20Footstep _da_niagarafx) :SurfaceType1 (Variables|/Game/ResidentHorrorFPS/Blueprints/BP_DataAsset/DA_Footstep/VisualEffects/DA_FootstepEffects.DA_FootstepEffects_C|GetGrass%20Footstep _da_niagarafx) :SurfaceType2 (Variables|/Game/ResidentHorrorFPS/Blueprints/BP_DataAsset/DA_Footstep/VisualEffects/DA_FootstepEffects.DA_FootstepEffects_C|GetStone%20Footstep _da_niagarafx) :SurfaceType3 (Variables|/Game/ResidentHorrorFPS/Blueprints/BP_DataAsset/DA_Footstep/VisualEffects/DA_FootstepEffects.DA_FootstepEffects_C|GetWater%20Footstep _da_niagarafx) :SurfaceType4 (Variables|/Game/ResidentHorrorFPS/Blueprints/BP_DataAsset/DA_Footstep/VisualEffects/DA_FootstepEffects.DA_FootstepEffects_C|GetWood%20Footstep _da_niagarafx) :SurfaceType5 (Variables|/Game/ResidentHorrorFPS/Blueprints/BP_DataAsset/DA_Footstep/VisualEffects/DA_FootstepEffects.DA_FootstepEffects_C|GetMetal%20Footstep _da_niagarafx) :SurfaceType6 (Variables|/Game/ResidentHorrorFPS/Blueprints/BP_DataAsset/DA_Footstep/VisualEffects/DA_FootstepEffects.DA_FootstepEffects_C|GetBlood%20Footstep _da_niagarafx) :SurfaceType7 (Variables|/Game/ResidentHorrorFPS/Blueprints/BP_DataAsset/DA_Footstep/VisualEffects/DA_FootstepEffects.DA_FootstepEffects_C|GetGlass%20Footstep _da_niagarafx)) (.Location (Collision|BreakHitResult _outhit)))
            (switch Utilities|FlowControl|Switch|SwitchonEPhysicalSurface (Collision|GetSurfaceType _outhit)
              (:SurfaceType_Default
                ;[0 0 0 0.5] Sound Footsteps
                (bind _returnvalue_6 (Audio|SpawnSoundAttached (Variables|/Game/ResidentHorrorFPS/Blueprints/BP_DataAsset/DA_Footstep/Sound/DA_Sound_Footstep.DA_Sound_Footstep_C|GetDefault%20Som _da_footstep) MeshComp (Variables|Default|GetAttach%20Point%20Name) (.Location (Collision|BreakHitResult _outhit)) "0, 0, 0" "KeepWorldPosition" false (Variables|Default|GetVolumeMultiplier) 1.0 0.0 "/Game/ResidentHorrorFPS/Audio/Attenuation/Att_Footstep.Att_Footstep" 0))
                (Utilities|IsValid _returnvalue_6
                  (:Is%20Valid
                    _)))
              (:SurfaceType1
                (bind _returnvalue_7 (Audio|SpawnSoundAttached (Variables|/Game/ResidentHorrorFPS/Blueprints/BP_DataAsset/DA_Footstep/Sound/DA_Sound_Footstep.DA_Sound_Footstep_C|GetGrass _da_footstep) MeshComp (Variables|Default|GetAttach%20Point%20Name) (.Location (Collision|BreakHitResult _outhit)) "0, 0, 0" "KeepWorldPosition" false _volumemultiplier_3 1.0 0.0 "/Game/ResidentHorrorFPS/Audio/Attenuation/Att_Footstep.Att_Footstep" 0))
                (Utilities|IsValid _returnvalue_7
                  (:Is%20Valid
                    _)))
              (:SurfaceType2
                (bind _returnvalue_8 (Audio|SpawnSoundAttached (Variables|/Game/ResidentHorrorFPS/Blueprints/BP_DataAsset/DA_Footstep/Sound/DA_Sound_Footstep.DA_Sound_Footstep_C|GetGravel _da_footstep) MeshComp (Variables|Default|GetAttach%20Point%20Name) (.Location (Collision|BreakHitResult _outhit)) "0, 0, 0" "KeepWorldPosition" false _volumemultiplier_3 1.0 0.0 "/Game/ResidentHorrorFPS/Audio/Attenuation/Att_Footstep.Att_Footstep" 0))
                (Utilities|IsValid _returnvalue_8
                  (:Is%20Valid
                    _)))
              (:SurfaceType3
                (bind _returnvalue_9 (Audio|SpawnSoundAttached (Variables|/Game/ResidentHorrorFPS/Blueprints/BP_DataAsset/DA_Footstep/Sound/DA_Sound_Footstep.DA_Sound_Footstep_C|GetWater _da_footstep) MeshComp (Variables|Default|GetAttach%20Point%20Name) (.Location (Collision|BreakHitResult _outhit)) "0, 0, 0" "KeepWorldPosition" false _volumemultiplier_3 1.0 0.0 "/Game/ResidentHorrorFPS/Audio/Attenuation/Att_Footstep.Att_Footstep" 0))
                (Utilities|IsValid _returnvalue_9
                  (:Is%20Valid
                    (if (Variables|/Game/ResidentHorrorFPS/Character/BP_Character/BP_RHV_FPS_Player.BP_RHV_FPS_Player_C|GetDid%20I%20step%20in%20blood? _player)
                      (Variables|/Game/ResidentHorrorFPS/Character/BP_Character/BP_RHV_FPS_Player.BP_RHV_FPS_Player_C|SetDid%20I%20step%20in%20blood? _player false)))))
              (:SurfaceType4
                (bind _returnvalue_10 (Audio|SpawnSoundAttached (Variables|/Game/ResidentHorrorFPS/Blueprints/BP_DataAsset/DA_Footstep/Sound/DA_Sound_Footstep.DA_Sound_Footstep_C|GetWood _da_footstep) MeshComp (Variables|Default|GetAttach%20Point%20Name) (.Location (Collision|BreakHitResult _outhit)) "0, 0, 0" "KeepWorldPosition" false _volumemultiplier_2 1.0 0.0 "/Game/ResidentHorrorFPS/Audio/Attenuation/Att_Footstep.Att_Footstep" 0))
                (Utilities|IsValid _returnvalue_10
                  (:Is%20Valid
                    _)))
              (:SurfaceType5
                (bind _returnvalue_11 (Audio|SpawnSoundAttached (Variables|/Game/ResidentHorrorFPS/Blueprints/BP_DataAsset/DA_Footstep/Sound/DA_Sound_Footstep.DA_Sound_Footstep_C|GetMetal _da_footstep) MeshComp (Variables|Default|GetAttach%20Point%20Name) (.Location (Collision|BreakHitResult _outhit)) "0, 0, 0" "KeepWorldPosition" false _volumemultiplier_2 1.0 0.0 "/Game/ResidentHorrorFPS/Audio/Attenuation/Att_Footstep.Att_Footstep" 0))
                (Utilities|IsValid _returnvalue_11
                  (:Is%20Valid
                    _)))
              (:SurfaceType6
                (bind _returnvalue_12 (Audio|SpawnSoundAttached (Variables|/Game/ResidentHorrorFPS/Blueprints/BP_DataAsset/DA_Footstep/Sound/DA_Sound_Footstep.DA_Sound_Footstep_C|GetBlood _da_footstep) MeshComp (Variables|Default|GetAttach%20Point%20Name) (.Location (Collision|BreakHitResult _outhit)) "0, 0, 0" "KeepWorldPosition" false _volumemultiplier 1.0 0.0 "/Game/ResidentHorrorFPS/Audio/Attenuation/Att_Footstep.Att_Footstep" 0))
                (Utilities|IsValid _returnvalue_12
                  (:Is%20Valid
                    (Variables|/Game/ResidentHorrorFPS/Character/BP_Character/BP_RHV_FPS_Player.BP_RHV_FPS_Player_C|SetDid%20I%20step%20in%20blood? _player_2 true))))
              (:SurfaceType7
                (bind _returnvalue_13 (Audio|SpawnSoundAttached (Variables|/Game/ResidentHorrorFPS/Blueprints/BP_DataAsset/DA_Footstep/Sound/DA_Sound_Footstep.DA_Sound_Footstep_C|GetGlass _da_footstep) MeshComp (Variables|Default|GetAttach%20Point%20Name) (.Location (Collision|BreakHitResult _outhit)) "0, 0, 0" "KeepWorldPosition" false _volumemultiplier 1.0 0.0 "/Game/ResidentHorrorFPS/Audio/Attenuation/Att_Footstep.Att_Footstep" 0))
                (Utilities|IsValid _returnvalue_13
                  (:Is%20Valid
                    _)))))
          (if (Variables|Default|GetAdditional%20Sound?)
            (CallFunction|SoundAdditional MeshComp (.Location (Collision|BreakHitResult _outhit))))
          ;[0 0 0 0.5] Footstep Blood
          (if (Variables|/Game/ResidentHorrorFPS/Character/BP_Character/BP_RHV_FPS_Player.BP_RHV_FPS_Player_C|GetDid%20I%20step%20in%20blood? _player_2)
            (Default|ISteppedinBlood (CallFunction|RHVFPSPlayerRef))
            (bind _returnvalue_14 (Rendering|Decal|SpawnDecalatLocation "/Game/ResidentHorrorFPS/Demo/Materials/M_MD_Footprints.M_MD_Footprints" "3.500000,18.000000,18.000000" (.Location (Collision|BreakHitResult _outhit)) (Utilities|Select :Index (Variables|Default|GetSide) :NewEnumerator4 (Transformation|GetWorldRotation MeshComp) :NewEnumerator0 (Transformation|GetSocketRotation MeshComp "Footstep_L") :NewEnumerator2 (Transformation|GetSocketRotation MeshComp "Footstep_R")) 0.0))
            (Rendering|Components|Decal|SetFadeOut _returnvalue_14 2.0 8.0 true)
            (return true)))))))

(fn GetNotifyName
  (return (Utilities|String|ToString(Text) (Utilities|Text|FormatText "FoleyEvent: {Type}" (.RightS (Utilities|String|Split (GameplayTags|GetDebugStringfromGameplayTag (Variables|Default|GetEvent)) "." "IgnoreCase" "FromEnd"))))))

(fn GetAudioBank
  (params (MeshComponent :type Skeletal%20Mesh%20Component%20Object%20Reference))
  (bind _returnvalue (Components|GetOwner MeshComponent))
  (Utilities|Casting|CastToAnimationEditorPreviewActor _returnvalue
    (:then
      (if (Audio|Components|Audio|IsPlaying MeshComponent)
        (return (Variables|Default|GetDefaultBank) true)))
    (:CastFailed
      (if (not (GameplayTags|HasTag (GameplayTags|MakeLiteralGameplayTagContainer "(GameplayTags=((TagName=\"Foley.Event.Jump\"),(TagName=\"Foley.Event.Land\")))") (Variables|Default|GetEvent)))
        (if (Utilities|DoesObjectImplementInterface _returnvalue "/Game/ResidentHorrorFPS/Blueprints/BP_MetaSound/Foley/I_FoleyAudioBankInterface.I_FoleyAudioBankInterface_C")
          (bind _foleyaudiobank (Class|IFoleyAudioBankInterface|GetFoleyAudioBank(Message) _returnvalue))
          (if (GameplayTags|HasTag (GameplayTags|MakeLiteralGameplayTagContainer "(GameplayTags=((TagName=\"Foley.Event.Run\"),(TagName=\"Foley.Event.Scuff\"),(TagName=\"Foley.Event.Walk\"),(TagName=\"Foley.Event.RunBackwds\"),(TagName=\"Foley.Event.RunStrafe\"),(TagName=\"Foley.Event.WalkBackwds\"),(TagName=\"Foley.Event.ScuffPivot\")))") (Variables|Default|GetEvent))
            (bind _returnvalue_2 (Class|IFoleyAudioBankInterface|CanPlayFootstepSounds(Message) _returnvalue))
            (return _foleyaudiobank _returnvalue_2)
            (else
              (return _foleyaudiobank true))))))))

(fn SoundAdditional
  (params (AttachToComponent :type Scene%20Component%20Object%20Reference) (Location :type Vector))
  (Audio|SpawnSoundAttached (Variables|Default|GetAdditional%20Sound) AttachToComponent (Variables|Default|GetAttach%20Point%20Name) Location "0, 0, 0" "KeepWorldPosition" false (Variables|Default|GetVolume%20Additonal%20Sound) 1.0 0.0 (Variables|Default|Get%20Additonal%20Sound%20Attenuation%20Settings) 0))