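; Explosive barrel hazard for the horror FPS that the player can disarm by interacting, swapping its material.
; While armed, a hit or player overlap triggers its explosive component, then destroys it and optionally a linked actor.
; Overlap damages the player, or AI enemies even when disarmed and without exploding.
; Disarming and hit-triggered destruction are saved and restored on load; overlap detonation is not saved.
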(event LoadedData(BP_SaveLoadRHFps)
  (params (Save%20Loaded%20Data :type ST%20Save%20Load%20Structure))
  (bind (_boolean3 _boolean4) (Utilities|Struct|BreakST_SaveLoad Save%20Loaded%20Data))
  (if _boolean3
    (Actor|DestroyActor)
    (elif _boolean4
      (Variables|Default|SetOff? true)
      (Rendering|Material|SetMaterial (Variables|Default|GetSM_Explosive_Barrel3) 0 "/Game/ResidentHorrorFPS/Demo/Materials/M_OffExplosive.M_OffExplosive")
      (CallFunction|VisibilityWidgetChange true))))

(event OnComponentBeginOverlap(BoxDamage)
  (params (OverlappedComponent :type Primitive%20Component%20Object%20Reference) (OtherActor :type Actor%20Object%20Reference) (OtherComp :type Primitive%20Component%20Object%20Reference) (OtherBodyIndex :type Integer) (bFromSweep :type Boolean) (SweepResult :type Hit%20Result%20Structure%20%28by%20ref%29))
  ;[0 0 0 0.5] Damage Ai enemy
  (bind _asbp_aimaster (Utilities|Casting|CastToBP_AIMaster OtherActor)
    (:then
      (if (== OtherActor _asbp_aimaster)
        (bind _returnvalue (Game|Damage|ApplyDamage _asbp_aimaster 6e+02 0 0))
        (CallFunction|BPIDamage :DamageCauser _asbp_aimaster :Base%20Damage _returnvalue)))
    (:CastFailed
      ;[0 0 0 0.5] Damage Player
      (if (not (Variables|Default|GetOff?))
        (if (== OtherActor (CallFunction|RHVFPSPlayerRef))
          (Default|Explode (Variables|Default|GetExplosiveComponet))
          (Default|TakeDamage (Variables|/Game/ResidentHorrorFPS/Character/BP_Character/BP_RHV_FPS_Player.BP_RHV_FPS_Player_C|GetHealthComponent (CallFunction|RHVFPSPlayerRef)) (Variables|Default|Get%20Damage%20In%20Player))
          ;[0 0 0 0.5] Destroy Actors
          (Utilities|FlowControl|Sequence
            (:then_0
              (Utilities|FlowControl|Delay 0.1)
              (Actor|DestroyActor))
            (:then_1
              (if (Variables|Default|GetDestroy%20Other%20Actors?)
                (bind _actor_destroyer (Variables|Default|GetActor%20Destroyer)
                  (:then
                    (Actor|DestroyActor _actor_destroyer))
                  (:else))))))))))

(event Custom|Off
  ;[0 0 0] Turn off the logic to avoid explosions.
  (Variables|Default|SetOff? true)
  (Rendering|Material|SetMaterial (Variables|Default|GetSM_Explosive_Barrel3) 0 "/Game/ResidentHorrorFPS/Demo/Materials/M_OffExplosive.M_OffExplosive")
  (Audio|PlaySound2D "/Engine/VREditor/Sounds/UI/Click_on_Button.Click_on_Button" 1.0 1.0 0.0 0 0)
  (CallFunction|VisibilityWidgetChange true)
  (Default|SaveData (Variables|Default|GetBP_SaveLoadRHFps) (Utilities|Struct|MakeST_SaveLoad true)))

(event EventInteraction
  (params (Player :type BP%20RHV%20FPS%20Player%20Object%20Reference) (AutoInteraction%28Non-Player%29 :type Boolean))
  ;[0 0 0] Turn off the logic to avoid explosions.
  (if (not (Variables|Default|GetOff?))
    (CallFunction|Off)))

(event EventEventDamageRHFPS
  (params (Damage :type Float%20%28double-precision%29) (Hitresult :type Hit%20Result%20Structure) (Preparator :type Actor%20Object%20Reference))
  ;[0 0 0] Explode
  (if (== (.HitActor (Collision|BreakHitResult Hitresult)) self)
    (if (not (Variables|Default|GetOff?))
      (Default|Explode (Variables|Default|GetExplosiveComponet))
      (Utilities|FlowControl|Sequence
        (:then_0
          (Utilities|FlowControl|Delay 0.1)
          (Default|SaveData (Variables|Default|GetBP_SaveLoadRHFps) (Utilities|Struct|MakeST_SaveLoad true))
          (Actor|DestroyActor))
        (:then_1
          (if (Variables|Default|GetDestroy%20Other%20Actors?)
            (bind _actor_destroyer (Variables|Default|GetActor%20Destroyer)
              (:then
                (Actor|DestroyActor _actor_destroyer)
                (CallFunction|VisibilityWidgetChange true))
              (:else))))))))

(fn ConstructionScript)

(fn ActorinStealth
  (return false))

(fn BPICanForgetAboutEnemy
  (params (Enemy :type Actor%20Object%20Reference))
  (return false))

(fn BPICheckStunTags
  (params (Tags :type Gameplay%20Tag%20Container%20Structure))
  (return false))

(fn BPIEditStunTags
  (params (Tags :type Array%20of%20Gameplay%20Tag%20Structures) (Remove :type Boolean))
  (return false))

(fn BPIGetAIStats
  (return 0))

(fn BPIGetCreatureName
  (return "NewEnumerator0"))

(fn BPIGetDamageTrigger
  (params (TriggerName :type Name :default "None"))
  (return false ""))

(fn BPIGetMesh
  (return 0))

(fn CanAlertOtherEntities
  (return false))

(fn GetCombatStyle
  (return "NewEnumerator0"))

(fn GetLocation
  (return "0, 0, 0"))

(fn GetTeamID
  (return 0))

(fn IsAlive
  (return false))

(fn IsEnemy
  (params (TeamID :type Integer))
  (return false))

(fn IsPawnDead
  (return false))

(fn IsPlayer
  (return false))