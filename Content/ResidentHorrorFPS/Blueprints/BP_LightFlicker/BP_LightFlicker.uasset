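; Breakable lamp actor with an optional flickering spotlight and buzz audio.
; On BeginPlay a lit lamp can start a random-delay loop that flip-flops intensity between min and max with a sound, until shot.
; Damage depletes its resistance, then a lit lamp bursts with particles and sound, hides the light, stops audio, swaps material and disables sphere collision.
; SaveLoadComponent saves the shot state; loading restores only that flag.
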(event LoadedData(SaveLoadComponent)
  (params (Save%20Loaded%20Data :type ST%20Save%20Load%20Structure))
  ;[0 0 0 0.5] Save And Load
  (if (.Boolean (Utilities|Struct|BreakST_SaveLoad Save%20Loaded%20Data))
    (Variables|Default|SetShot%20Lamp? true)))

(event EventBeginPlay
  ;[0 0 0] Light Flicker
  (Rendering|Components|Light|SetLightColor (Variables|Default|GetSpotLight) (Variables|Default|GetColor%20Light) true)
  (if (Variables|Default|GetLight%20On?)
    (CallFunction|Lighton)
    (if (Variables|Default|GetLight%20Flicker?)
      (Rendering|Components|Light|SetCastShadows (Variables|Default|GetSpotLight) (Variables|Default|GetShadow%20On?))
      (Utilities|FlowControl|RetriggerableDelay (Math|Random|RandomFloatinRange (Variables|Default|GetMin%20time) (Variables|Default|GetMax%20time)) :!label _label)
      (Utilities|FlowControl|FlipFlop
        (:A
          (Components|Activation|Activate (Variables|Default|GetSound%20Luz%20Piscando) false)
          (Rendering|Components|Light|SetIntensity (Variables|Default|GetSpotLight) (Variables|Default|GetMin%20Intensity)))
        (:B
          (Components|Activation|Activate (Variables|Default|GetSound%20Luz%20Piscando) false)
          (Rendering|Components|Light|SetIntensity (Variables|Default|GetSpotLight) (Variables|Default|GetMax%20Intensity))))
      (if (not (Variables|Default|GetShot%20Lamp?))
        (goto _label)))
    (else
      (CallFunction|LightOff))))

(event EventEventDamageRHFPS
  (params (Damage :type Float%20%28double-precision%29) (Hitresult :type Hit%20Result%20Structure) (Preparator :type Actor%20Object%20Reference))
  (bind _spotlight (Variables|Default|GetSpotLight))
  (bind _returnvalue (Transformation|GetWorldLocation _spotlight))
  ;[0 0 0] burst lamp Hit Weapon
  (Variables|Default|SetResistence%20lamp (- (Variables|Default|GetResistence%20lamp) Damage))
  (if (<= (Variables|Default|GetResistence%20lamp) 0.0)
    (if (Variables|Default|GetLight%20On?)
      (if (not (Variables|Default|GetShot%20Lamp?))
        (CallFunction|LightOff)
        (Effects|SpawnEmitteratLocation (Variables|Default|GetEffect%20Bust%20Lamp) _returnvalue)
        (Audio|PlaySoundatLocation (Variables|Default|GetSound%20Bust%20%20Lamp) _returnvalue "0, 0, 0" 1.0 1.0 0.0 (Variables|Default|GetAttenuation) 0 0 0)
        (Rendering|SetVisibility (Variables|Default|GetSpotLight) false false)
        (Components|Activation|Deactivate (Variables|Default|GetSound%20Luz%20Piscando))
        (Rendering|Material|SetMaterial (Variables|Default|GetStaticMesh) 0 0)
        (Variables|Default|SetShot%20Lamp? true)
        (Collision|SetCollisionResponsetoAllChannels (Variables|Default|GetSphere) "ECR_Ignore")
        (Default|SaveData (Variables|Default|GetSaveLoadComponent) (Utilities|Struct|MakeST_SaveLoad true))))))

(fn ConstructionScript)

(fn Lighton
  (Rendering|SetVisibility (Variables|Default|GetSpotLight) (Variables|Default|GetLight%20On?) false)
  (Components|Activation|Activate (Variables|Default|GetLightbuzz_Cue1) false))

(fn LightOff
  (bind _spotlight (Variables|Default|GetSpotLight))
  (Rendering|SetVisibility _spotlight (Variables|Default|GetLight%20On?) false)
  (Development|SetHiddeninGame _spotlight false false))