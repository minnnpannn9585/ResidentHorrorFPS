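; BP_Loot is an interactable loot actor that exposes its own inventory component to the interacting player.
; On Interaction it toggles the inventory through the player's BPCEquipment component.
; If that inventory is now open, it assigns its BPCInventory as the loot inventory, refreshes the loot UI, then registers itself as the loot actor.
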(event EventBeginPlay
  (|CallParentFunction))

(event Collision|EventActorBeginOverlap
  (params (OtherActor :type Actor%20Object%20Reference)))

(event EventTick
  (params (DeltaSeconds :type Float%20%28single-precision%29)))

(event EventInteraction
  (params (Player :type BP%20RHV%20FPS%20Player%20Object%20Reference) (AutoInteraction%28Non-Player%29 :type Boolean))
  ;[0.15 0.15 0.15 0.5] Interact
  (bind _output_get (Variables|Default|SetBPC%20Equipment (Variables|/Game/ResidentHorrorFPS/Character/BP_Character/BP_RHV_FPS_Player.BP_RHV_FPS_Player_C|GetBPC_Equipment Player)))
  (Default|ToggleInventory _output_get)
  (if (Variables|/Game/ResidentHorrorFPS/Blueprints/BP_Inventory/Inventory/Equipment/BPC_Equipment.BPC_Equipment_C|GetInventoryOpen? _output_get)
    (Variables|/Game/ResidentHorrorFPS/Blueprints/BP_Inventory/Inventory/Equipment/BPC_Equipment.BPC_Equipment_C|SetLootInventory (Variables|Default|GetBPC%20Equipment) (Variables|Default|GetBPC_Inventory))
    (Default|UpdateLootUI (Variables|Default|GetBPC%20Equipment))
    (Variables|/Game/ResidentHorrorFPS/Blueprints/BP_Inventory/Inventory/Equipment/BPC_Equipment.BPC_Equipment_C|SetLootActor (Variables|Default|GetBPC%20Equipment) self)))

(fn ConstructionScript)