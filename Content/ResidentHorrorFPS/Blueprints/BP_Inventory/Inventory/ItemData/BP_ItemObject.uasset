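; BP_ItemObject is the data object for a single item in the inventory system.
; It exposes getters for the Information struct's amount, visualization, tags and usable data, plus its primary item data, and can update the current amount.
; A rotation flag toggles the item's orientation, and GetTile swaps the tile's X and Y footprint when rotated.
; It also stores an item sub-object reference, set by event.
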(event EventSetSubObject
  (params (ItemSubObject :type BP%20Item%20Object%20Object%20Reference))
  (Variables|SubItemObject|SetItem%20Sub%20Object ItemSubObject))

(fn GetAmount
  (return (.Amount (Utilities|Struct|BreakST_ItemInformation (Variables|Info|GetInformation)))))

(fn GetVisualization
  (return (.Visualization (Utilities|Struct|BreakST_ItemInformation (Variables|Info|GetInformation)))))

(fn GetTags
  (return (.Tags (Utilities|Struct|BreakST_ItemInformation (Variables|Info|GetInformation)))))

(fn SetAmount
  (params (CurrentAmount :type Integer))
  (Utilities|Struct|SetmembersinST_Amount (.Amount (Utilities|Struct|BreakST_ItemInformation (Variables|Info|GetInformation))) CurrentAmount)
  (return))

(fn RotateItem
  (Variables|Check|SetIconRotate (not (Variables|Check|GetIconRotate)))
  (return))

(fn GetUsableInformation
  (return (.UsableInformation (Utilities|Struct|BreakST_ItemInformation (Variables|Info|GetInformation)))))

(fn GetTile
  (bind _information (Variables|Info|GetInformation))
  (bind _visualization (Utilities|Struct|BreakST_ItemInformation _information))
  (bind _tile (Utilities|Struct|BreakST_ItemVisualization _visualization))
  (bind (_x _y) (Utilities|Struct|BreakST_Tile _tile))
  (return (select (Variables|Check|GetIconRotate) (Utilities|Struct|MakeST_Tile _y _x) _tile)))

(fn CanRotate?
  (return (Utilities|Struct|BreakST_ItemVisualization (.Visualization (Utilities|Struct|BreakST_ItemInformation (Variables|Info|GetInformation))))))

(fn GetPrimaryItemData
  (return (Variables|Info|GetPrimaryItemData)))

(fn GetItemObject
  (return self))

(fn GetSubObject
  (return (Variables|SubItemObject|GetItem%20Sub%20Object)))