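; Breakable wooden crate that drops a random item when broken by player damage or a BoxBroken event.
; A one-time break spawns wood Niagara FX, plays sound, swaps to the broken mesh and spawns an item from ItemDropped at LocItemspawn.
; The save component stores the broken state and dropped item.
; Loading restores the mesh and respawns that item, but leaves the BoxBroken flag unset.
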(event LoadedData(BP_SaveLoadRHFps)
  (params (Save%20Loaded%20Data :type ST%20Save%20Load%20Structure))
  (bind (_boolean2 _integer1 _itemsdropped) (Utilities|Struct|BreakST_SaveLoad Save%20Loaded%20Data))
  (bind _locitemspawn (Variables|Default|GetLocItemspawn))
  ;[0.15 0.15 0.15 0.5] Load
  (if _boolean2
    (Components|StaticMesh|SetStaticMesh (Variables|Default|GetStaticMesh) "/Game/ResidentHorrorFPS/Demo/Mesh/SM_BOX_BROKEN.SM_BOX_BROKEN")
    (Game|SpawnActorfromClass "/Game/ResidentHorrorFPS/Blueprints/BP_ItemBase/BP_ItemBaseRHFPS.BP_ItemBaseRHFPS_C" (Math|Transform|MakeTransform (Transformation|GetWorldLocation _locitemspawn) (Transformation|GetWorldRotation _locitemspawn) "1.000000,1.000000,1.000000") "Undefined" "MultiplyWithRoot" 0 false 0 _itemsdropped 0)))

(event Custom|Box%20Broken
  (bind _drs_car_close_01_cue (Variables|Default|GetDrs_Car_Close_01_Cue))
  (bind _locitemspawn (Variables|Default|GetLocItemspawn))
  ;[0 0 0] Broken Box Logic
  (if (not (Variables|Default|GetBox%20Broken?))
    (Niagara|SpawnSystematLocation "/Game/ResidentHorrorFPS/Demo/ParticleEffects/NS_Wood2.NS_Wood2" (Transformation|GetWorldLocation (Variables|Default|GetStaticMesh)) "0, 0, 0" "3.000000,3.000000,3.000000")
    (Variables|Default|SetBox%20Broken? true)
    (Audio|PlaySound2D "/Game/ResidentHorrorFPS/Audio/Cue/CUE_Car_Close_01_Cue.CUE_Car_Close_01_Cue" 4.0 1.0 0.0 0 0)
    (bind _itemobject (Class|BPIItemObject|GetItemObject(Message) (Variables|/Game/ResidentHorrorFPS/Character/BP_Character/BP_RHV_FPS_Player.BP_RHV_FPS_Player_C|GetBPC_Equipment (CallFunction|RHVFPSPlayerRef))))
    (bind _returnvalue (Game|SpawnActorfromClass "/Game/ResidentHorrorFPS/Blueprints/BP_ItemBase/BP_ItemBaseRHFPS.BP_ItemBaseRHFPS_C" (Math|Transform|MakeTransform (Transformation|GetWorldLocation _locitemspawn) (Transformation|GetWorldRotation _locitemspawn) "1.000000,1.000000,1.000000") "Undefined" "MultiplyWithRoot" 0 false _itemobject (.OutItem (Utilities|Array|Random (Variables|Default|GetItem%20Dropped))) (CallFunction|RHVFPSPlayerRef)))
    (bind _output_get (Variables|Default|SetItem%20Spawn _returnvalue))
    (Default|SaveData (Variables|Default|GetBP_SaveLoadRHFps) (Utilities|Struct|MakeST_SaveLoad true 0 (Variables|/Game/ResidentHorrorFPS/Blueprints/BP_InteractMaster/BP_RHMasterInteract.BP_RHMasterInteract_C|GetPrymaryDataAsset _output_get)))
    (Components|StaticMesh|SetStaticMesh (Variables|Default|GetStaticMesh) "/Game/ResidentHorrorFPS/Demo/Mesh/SM_BOX_BROKEN.SM_BOX_BROKEN")
    (Variables|Default|SetBox%20Broken? true)
    (Utilities|IsValid _drs_car_close_01_cue
      (:Is%20Valid
        (Audio|Components|Audio|Play _drs_car_close_01_cue 0.0)))))

(event EventEventDamageRHFPS
  (params (Damage :type Float%20%28double-precision%29) (Hitresult :type Hit%20Result%20Structure) (Preparator :type Actor%20Object%20Reference))
  (bind _drs_car_close_01_cue (Variables|Default|GetDrs_Car_Close_01_Cue))
  (bind _locitemspawn (Variables|Default|GetLocItemspawn))
  ;[0 0 0] Broken Box Logic
  (if (== (.HitActor (Collision|BreakHitResult Hitresult)) self)
    (if (not (Variables|Default|GetBox%20Broken?))
      (Niagara|SpawnSystematLocation "/Game/ResidentHorrorFPS/Demo/ParticleEffects/NS_Wood2.NS_Wood2" (Transformation|GetWorldLocation (Variables|Default|GetStaticMesh)) "0, 0, 0" "3.000000,3.000000,3.000000")
      (Variables|Default|SetBox%20Broken? true)
      (Audio|PlaySound2D "/Game/ResidentHorrorFPS/Audio/Cue/CUE_Car_Close_01_Cue.CUE_Car_Close_01_Cue" 4.0 1.0 0.0 0 0)
      (bind _itemobject (Class|BPIItemObject|GetItemObject(Message) (Variables|/Game/ResidentHorrorFPS/Character/BP_Character/BP_RHV_FPS_Player.BP_RHV_FPS_Player_C|GetBPC_Equipment (CallFunction|RHVFPSPlayerRef))))
      (bind _returnvalue (Game|SpawnActorfromClass "/Game/ResidentHorrorFPS/Blueprints/BP_ItemBase/BP_ItemBaseRHFPS.BP_ItemBaseRHFPS_C" (Math|Transform|MakeTransform (Transformation|GetWorldLocation _locitemspawn) (Transformation|GetWorldRotation _locitemspawn) "1.000000,1.000000,1.000000") "Undefined" "MultiplyWithRoot" 0 false _itemobject (.OutItem (Utilities|Array|Random (Variables|Default|GetItem%20Dropped))) (CallFunction|RHVFPSPlayerRef)))
      (bind _output_get (Variables|Default|SetItem%20Spawn _returnvalue))
      (Default|SaveData (Variables|Default|GetBP_SaveLoadRHFps) (Utilities|Struct|MakeST_SaveLoad true 0 (Variables|/Game/ResidentHorrorFPS/Blueprints/BP_InteractMaster/BP_RHMasterInteract.BP_RHMasterInteract_C|GetPrymaryDataAsset _output_get)))
      (Components|StaticMesh|SetStaticMesh (Variables|Default|GetStaticMesh) "/Game/ResidentHorrorFPS/Demo/Mesh/SM_BOX_BROKEN.SM_BOX_BROKEN")
      (Variables|Default|SetBox%20Broken? true)
      (Utilities|IsValid _drs_car_close_01_cue
        (:Is%20Valid
          (Audio|Components|Audio|Play _drs_car_close_01_cue 0.0))))))

(fn ConstructionScript)