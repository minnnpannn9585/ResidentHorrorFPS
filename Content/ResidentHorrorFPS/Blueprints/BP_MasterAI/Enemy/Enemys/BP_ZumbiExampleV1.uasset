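; Example zombie enemy built on a parent AI, serving as a template for melee, long-distance and combo attacks.
; AfterAttackFilter takes a queue position, runs the attack matching the ID and starts cooldowns.
; Dispatched attacks motion-warp to the enemy and lock yaw so fast players can dodge, then play montages ending in OnAttackEnd.
; SetupHitBoxes registers body parts with damage and stun multipliers; the roll attack is defined but not dispatched.
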(event Custom|Long-Distance%20Attack%20Example
  (bind (_validenemy _enemy) (CallFunction|GetEnemyActor))
  (bind _returnvalue (Transformation|GetActorLocation))
  (bind _returnvalue_2 (Transformation|GetActorLocation _enemy))
  (bind _returnvalue_3 (Math|Rotator|FindLookatRotation _returnvalue _returnvalue_2))
  ;[0 0 0] Esses são exemplos de ataques - Use essas bases como inspirações para desenvolver novos ataques.
  ;;[0 0 0] Example of an attack #4
  ;;;[1 1 1] Add the player to the warp system
  ;;;;[1 1 1] The warp system is a way to link this AI to the player. The warp time is specified in the anim montage
  (CallFunction|AddEnemytoWarpComp 1e+03 true)
  (if _validenemy
    ;;;[1 1 1] Stop this AI from rotating so that it misses its attack if the player is faster
    (Variables|Default|SetbUseControllerRotationYaw true)
    (Variables|Default|SetLockRotation (Math|Rotator|MakeRotator 0.0 0.0 (.yaw _returnvalue_3)))
    (Transformation|SetActorRotation (Math|Rotator|MakeRotator 0.0 0.0 (.yaw _returnvalue_3)) true)
    ;;;[1 1 1] Play attack animation
    (Animation|Montage|PlayMontage (Variables|Character|GetMesh) "/Game/ResidentHorrorFPS/Character/Animations/EnemyIA/AM_Attack_D1_Montage.AM_Attack_D1_Montage"
      (:OnCompleted
        _)
      (:OnInterrupted
        _))
    ;;;[1 1 1] Remover warp
    (Class|MotionWarpingComponent|RemoveWarpTarget (Variables|Default|GetMotionWarping) "enemy")
    ;;;[1 1 1] Unlock rotation
    (Variables|Default|SetLockRotation "0.000000,-999.000000,0.000000")
    ;;;[1 1 1] END THE ATTACK
    (CallFunction|OnAttackEnd 1.0)
    (else
      (Variables|Default|SetAttacking false))))

(event Custom|ExampleAttack1_Close
  (bind (_validenemy _enemy) (CallFunction|GetEnemyActor))
  (bind _returnvalue (Transformation|GetActorLocation))
  (bind _returnvalue_2 (Transformation|GetActorLocation _enemy))
  (bind _returnvalue_3 (Math|Rotator|FindLookatRotation _returnvalue _returnvalue_2))
  ;[0 0 0] Esses são exemplos de ataques - Use essas bases como inspirações para desenvolver novos ataques.
  ;;[0 0 0] Example of an attack #1
  ;;;[1 1 1] Add the player to the warp system
  ;;;;[1 1 1] The warp system is a way to link this AI to the player. The warp time is specified in the anim montage
  (CallFunction|AddEnemytoWarpComp 5e+02 false)
  (if _validenemy
    ;;;[1 1 1] Stop this AI's turn so that it misses its attack if the player is faster
    (Variables|Default|SetbUseControllerRotationYaw true)
    (Variables|Default|SetLockRotation (Math|Rotator|MakeRotator 0.0 0.0 (.yaw _returnvalue_3)))
    (Transformation|SetActorRotation (Math|Rotator|MakeRotator 0.0 0.0 (.yaw _returnvalue_3)) true)
    ;;;[1 1 1] Play attack animation
    (Animation|Montage|PlayMontage (Variables|Character|GetMesh) "/Game/ResidentHorrorFPS/Character/Animations/EnemyIA/AM_Attack_A1_Montage.AM_Attack_A1_Montage"
      (:OnCompleted
        _)
      (:OnInterrupted
        _))
    ;;;[1 1 1] Remover warp
    (Class|MotionWarpingComponent|RemoveWarpTarget (Variables|Default|GetMotionWarping) "enemy")
    ;;;[1 1 1] Unlock rotation
    (Variables|Default|SetLockRotation "0.000000,-999.000000,0.000000")
    ;;;[1 1 1] END THE ATTACK
    (CallFunction|OnAttackEnd 1.0)
    (else
      (Variables|Default|SetAttacking false))))

(event Custom|ExampleAttack6_Combo
  (bind (_validenemy _enemy) (CallFunction|GetEnemyActor))
  (bind _returnvalue (Transformation|GetActorLocation))
  (bind (_validenemy_2 _enemy_2) (CallFunction|GetEnemyActor))
  (bind _returnvalue_2 (Transformation|GetActorLocation))
  (bind _returnvalue_3 (Transformation|GetActorLocation _enemy))
  (bind _returnvalue_4 (Transformation|GetActorLocation _enemy_2))
  (bind _returnvalue_5 (Math|Rotator|FindLookatRotation _returnvalue _returnvalue_3))
  (bind _returnvalue_6 (Math|Rotator|FindLookatRotation _returnvalue_2 _returnvalue_4))
  ;[0 0 0] Esses são exemplos de ataques - Use essas bases como inspirações para desenvolver novos ataques.
  ;;[0 0 0] Attack Example #6 - COMBO - Combining Attacks 1 and 2
  ;;;[1 1 1] Add the player to the warp system
  ;;;;[1 1 1] The warp system is a way to link this AI to the player. The warp time is specified in the anim montage
  (CallFunction|AddEnemytoWarpComp 5e+02 false)
  (if _validenemy
    ;;;[1 1 1] Stop this AI from rotating so that it misses its attack if the player is faster
    (Variables|Default|SetbUseControllerRotationYaw true)
    (Variables|Default|SetLockRotation (Math|Rotator|MakeRotator 0.0 0.0 (.yaw _returnvalue_5)))
    (Transformation|SetActorRotation (Math|Rotator|MakeRotator 0.0 0.0 (.yaw _returnvalue_5)) true)
    ;;;[1 1 1] Play attack animation
    (Animation|Montage|PlayMontage (Variables|Character|GetMesh) "/Game/ResidentHorrorFPS/Character/Animations/EnemyIA/AM_Attack_A1_Montage.AM_Attack_A1_Montage"
      (:OnBlendOut
        ;;;[1 1 1] Remover warp
        (Class|MotionWarpingComponent|RemoveWarpTarget (Variables|Default|GetMotionWarping) "enemy")
        ;;;[1 0.5602 0.0349] Delay until the next attack
        (Utilities|FlowControl|Delay 0.0)
        ;;;[1 1 1] Add the player to the warp system
        ;;;;[1 1 1] The warp system is a way to link this AI to the player. The warp time is specified in the anim montage
        (CallFunction|AddEnemytoWarpComp 5e+02 false)
        (if _validenemy_2
          ;;;[1 1 1] Stop this AI from rotating so that it misses its attack if the player is faster
          (Variables|Default|SetbUseControllerRotationYaw true)
          (Variables|Default|SetLockRotation (Math|Rotator|MakeRotator 0.0 0.0 (.yaw _returnvalue_6)))
          (Transformation|SetActorRotation (Math|Rotator|MakeRotator 0.0 0.0 (.yaw _returnvalue_6)) true)
          ;;;[1 1 1] Play attack animation
          (Animation|Montage|PlayMontage (Variables|Character|GetMesh) "/Game/ResidentHorrorFPS/Character/Animations/EnemyIA/AM_Attack_D1_Montage.AM_Attack_D1_Montage"
            (:OnCompleted
              _)
            (:OnInterrupted
              _))
          ;;;[1 1 1] Remover warp
          (Class|MotionWarpingComponent|RemoveWarpTarget (Variables|Default|GetMotionWarping) "enemy")
          ;;;[1 1 1] Unlock rotation
          (Variables|Default|SetLockRotation "0.000000,-999.000000,0.000000")
          ;;;[1 1 1] END THE ATTACK
          (CallFunction|OnAttackEnd 1.0)
          (else
            (CallFunction|OnAttackEnd 1.0)))))
    (else
      (Variables|Default|SetAttacking false))))

(event Custom|Attack_Mid_Roll_Forward
  ;[0 0 0] Esses são exemplos de ataques - Use essas bases como inspirações para desenvolver novos ataques.
  ;;[1 0.01516 0] Example Attack #3 - Rolling Forward When Far Away
  (Animation|Montage|PlayMontage (Variables|Character|GetMesh) 0
    (:OnCompleted
      _)
    (:OnInterrupted
      _))
  ;;;[1 1 1] END THE ATTACK
  (CallFunction|OnAttackEnd 1.0))

(event Custom|ExampleAttack2_Close
  (bind (_validenemy _enemy) (CallFunction|GetEnemyActor))
  (bind _returnvalue (Transformation|GetActorLocation))
  (bind _returnvalue_2 (Transformation|GetActorLocation _enemy))
  (bind _returnvalue_3 (Math|Rotator|FindLookatRotation _returnvalue _returnvalue_2))
  ;[0 0 0] Esses são exemplos de ataques - Use essas bases como inspirações para desenvolver novos ataques.
  ;;[0 0 0] Example of an attack #1
  ;;;[1 1 1] The warp system is a way to link this AI to the player. The warp time is specified in the anim montage
  (CallFunction|AddEnemytoWarpComp 5e+02 false)
  ;;;[1 1 1] Add the player to the warp system
  (if _validenemy
    (Variables|Default|SetbUseControllerRotationYaw true)
    (Variables|Default|SetLockRotation (Math|Rotator|MakeRotator 0.0 0.0 (.yaw _returnvalue_3)))
    ;;;[1 1 1] Stop this AI from rotating so that it misses its attack if the player is faster
    (Transformation|SetActorRotation (Math|Rotator|MakeRotator 0.0 0.0 (.yaw _returnvalue_3)) true)
    ;;;;[1 1 1] Play attack animation
    (Animation|Montage|PlayMontage (Variables|Character|GetMesh) "/Game/ResidentHorrorFPS/Character/Animations/EnemyIA/AM_Attack_D1_Montage.AM_Attack_D1_Montage"
      (:OnCompleted
        _)
      (:OnInterrupted
        _))
    ;;;[1 1 1] Remover warp
    (Class|MotionWarpingComponent|RemoveWarpTarget (Variables|Default|GetMotionWarping) "enemy")
    ;;;[1 1 1] Unlock rotation
    (Variables|Default|SetLockRotation "0.000000,-999.000000,0.000000")
    ;;;[1 1 1] END THE ATTACK
    (CallFunction|OnAttackEnd 1.0)
    (else
      (Variables|Default|SetAttacking false))))

(event EventTick
  (params (DeltaSeconds :type Float%20%28single-precision%29))
  (|CallParentFunction DeltaSeconds))

(event EventBeginPlay
  (|CallParentFunction))

(event EventAfterAttackFilter
  (params (ID :type Integer))
  ;[0 0 0] Step 2 - Launch the attack
  (Utilities|FlowControl|Sequence
    (:then_0
      (CallFunction|SetPositiononEnemyQueue)
      (switch int ID ; Here you can have an unlimited number of attacks, as long as they are declared in the ‘Attacks’ variable
        (:0
          (CallFunction|ExampleAttack1Close))
        (:1
          (CallFunction|ExampleAttack2Close))
        (:2
          (CallFunction|Long-DistanceAttackExample))
        (:3
          (CallFunction|ExampleAttack6Combo))))
    (:then_1
      (CallFunction|InitializetheCooldownSystemforAttacks))))

(fn ConstructionScript
  (|CallParentFunction))

(fn SetupHitBoxes
  (bind _bpc_combat (Variables|Default|GetBPC_Combat))
  (bind _hitboxes (Variables|/Game/ResidentHorrorFPS/Blueprints/BP_MasterAI/IA/Blueprint/BP/BPC_Combat.BPC_Combat_C|GetHitboxes _bpc_combat))
  ;[0 0 0] Extracting the names of each HitBox
  (Utilities|Map|Add _hitboxes (Variables|Default|GetLLegBOx) "PernaEsquerda")
  (Utilities|Map|Add _hitboxes (Variables|Default|GetRLegBox) "PernaDireita")
  (Utilities|Map|Add _hitboxes (Variables|Default|GetLLegBOx) "LeftArm")
  (Utilities|Map|Add _hitboxes (Variables|Default|GetRLegBox) "RightArm")
  (Utilities|Map|Add _hitboxes (Variables|Default|GetChestBox) "Peito")
  (Utilities|Map|Add _hitboxes (Variables|Default|GetHeadBox) "head")
  ;[0 0 0] Adding damage multipliers for body parts
  ; e.g., If you hit the head, the damage will be 50% higher
  ;        If you hit the legs, the damage will be 50% lower
  (Utilities|Map|Add (Variables|/Game/ResidentHorrorFPS/Blueprints/BP_MasterAI/IA/Blueprint/BP/BPC_Combat.BPC_Combat_C|GetHitboxMultiplier (Variables|Default|GetBPC_Combat)) (Variables|Default|GetHeadBox) 1.5)
  (Utilities|Map|Add (Variables|/Game/ResidentHorrorFPS/Blueprints/BP_MasterAI/IA/Blueprint/BP/BPC_Combat.BPC_Combat_C|GetHitboxMultiplier (Variables|Default|GetBPC_Combat)) (Variables|Default|GetLLegBOx) 0.5)
  (Utilities|Map|Add (Variables|/Game/ResidentHorrorFPS/Blueprints/BP_MasterAI/IA/Blueprint/BP/BPC_Combat.BPC_Combat_C|GetHitboxMultiplier (Variables|Default|GetBPC_Combat)) (Variables|Default|GetRLegBox) 0.5)
  ;[1 0.06809 0] Adding Stun Multipliers
  ; In addition to dealing damage, we’ll add a bit of stun, depending on which part of the body was hit.
  (Utilities|Map|Add (Variables|/Game/ResidentHorrorFPS/Blueprints/BP_MasterAI/IA/Blueprint/BP/BPC_Combat.BPC_Combat_C|GetHitboxSTUNValues (Variables|Default|GetBPC_Combat)) (Variables|Default|GetHeadBox) 2.0))

(fn BPIGetCreatureName
  (return "NewEnumerator1"))

(fn CanAlertOtherEntities
  (return true))

(fn IsPawnDead
  (return false))

(fn ReceiveAIEnemy
  (return self))