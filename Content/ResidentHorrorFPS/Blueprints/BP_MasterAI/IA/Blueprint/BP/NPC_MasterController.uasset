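; AI controller for NPCs that runs BT_AIMaster and decides whom the pawn treats as an enemy.
; Perception events screen targets by death, alertability, combat style, player stealth and creature relationship, allowing AI-versus-AI fights.
; Accepted targets drive blackboard chase state, visibility and melee range; interface events can force or clear them.
; A retriggerable five-second forget timer works around the engine's unreliable perception-forgotten delegate.
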(event OnTargetPerceptionForgotten(AIPerception)
  (params (Actor :type Actor%20Object%20Reference))
  ;[0 0 0] He lost sight of the enemy
  (if (== Actor (Game|Player|GetPlayerPawn 0))
    (bind _return (Class|BPIMasterIAEnemy|BPICanForgetAboutEnemy(Message) (Pawn|GetControlledPawn) Actor))
    (if _return
      (Variables|Default|SetRC true)
      (Utilities|Array|RemoveItem (Variables|/Game/ResidentHorrorFPS/Blueprints/BP_MasterAI/IA/Blueprint/BP/BPC_Combat.BPC_Combat_C|GetActorsAfterMe (Actor|GetComponentbyClass (Variables|Default|GetActorSeen) "/Game/ResidentHorrorFPS/Blueprints/BP_MasterAI/IA/Blueprint/BP/BPC_Combat.BPC_Combat_C")) (Pawn|GetControlledPawn))
      (CallFunction|ForceRemoveEnemy))))

(event OnTargetPerceptionUpdated(AIPerception)
  (params (Actor :type Actor%20Object%20Reference) (Stimulus :type AI%20Stimulus%20Structure))
  (bind _returnvalue (AI|GetBlackboard 0))
  (bind _returnvalue_2 (Utilities|Name|MakeLiteralName "State"))
  (bind _returnvalue_3 (Pawn|GetControlledPawn))
  (bind _returnvalue_4 (Pawn|GetControlledPawn))
  (bind _returnvalue_5 (Utilities|Enum|LiteralenumE_ChaseStatus "NewEnumerator3"))
  (bind _returnvalue_6 (Utilities|Enum|LiteralenumE_ChaseStatus "NewEnumerator1"))
  (bind _returnvalue_7 (Class|BlackboardComponent|GetValueasEnum _returnvalue _returnvalue_2))
  (bind _returnvalue_8 (Actor|GetComponentbyClass _returnvalue_3 "/Game/ResidentHorrorFPS/Blueprints/BP_MasterAI/IA/Blueprint/BP/BPC_Combat.BPC_Combat_C"))
  (bind _returnvalue_9 (Utilities|Enum|ByteToEnumE_ChaseStatus _returnvalue_7))
  ;[0 0 0] Have you found or lost sight of someone?
  (if (Utilities|Struct|BreakAIStimulus Stimulus)
    (Variables|Default|SetC_UpdatedActor Actor :!label _label)
    ;[0 0 0] Is Dead?
    (Variables|Default|SetC_Stimulus Stimulus)
    (bind _return (Class|BPIMasterIAEnemy|IsPawnDead(Message) _returnvalue_4))
    (if _return
      (Variables|Default|SetActorSeen 0)
      (else
        ;[0 0 0] Update my current combat style
        (bind _style (Class|BPIMasterIAEnemy|GetCombatStyle(Message) _returnvalue_4))
        (Variables|Default|SetAICombatStyle _style)
        ;[0 0 0] Is the actor in the picture dead?
        (if (Utilities|DoesObjectImplementInterface (Variables|Default|GetC_UpdatedActor) "/Game/ResidentHorrorFPS/Blueprints/BP_MasterAI/IA/Blueprint/Interfaces/BPI_MasterIAEnemy.BPI_MasterIAEnemy_C")
          (bind _return_2 (Class|BPIMasterIAEnemy|IsPawnDead(Message) (Variables|Default|GetC_UpdatedActor)))
          (if (not _return_2)
            ;[0 0 0] Double-check whether this character can upgrade their vision now
            (if (not (Variables|Default|GetUnableToSee))
              ;[0 0 0] Some AIs will not update their perception of others, such as bosses and so on. These AIs may go unnoticed by minions and so on
              (bind _return_3 (Class|BPIMasterIAEnemy|CanAlertOtherEntities(Message) (Variables|Default|GetC_UpdatedActor)))
              (if _return_3
                ;[0 0 0] AI entities with Neutral behavior will not be triggered by sight. They must be attacked in order to respond.
                (if (and (Utilities|Enum|NotEqual(Enum) (Variables|Default|GetAICombatStyle) "NewEnumerator2") (Utilities|Enum|NotEqual(Enum) (Variables|Default|GetAICombatStyle) "NewEnumerator5"))
                  ;[0 0 0] Is the actor we see the player?
                  (if (== (Variables|Default|GetC_UpdatedActor) (Game|Player|GetPlayerPawn 0))
                    ;[0 0 0] Did you see the player, or did you just lose sight of him?
                    (if (Utilities|Struct|BreakAIStimulus (Variables|Default|GetC_Stimulus))
                      ;[0 0 0] Check to see if the player is hiding in any way, e.g., crouched in tall grass, etc.
                      (bind _return_4 (Class|BPIMasterIAEnemy|ActorinStealth(Message) (Variables|Default|GetC_UpdatedActor)))
                      (if (not _return_4)
                        ;[0.15 0.15 0.15 0.5] Force Target Perception
                        (CallFunction|ForceTargetPerception (Variables|Default|GetC_UpdatedActor)))
                      (else
                        (bind _return_5 (Class|BPIMasterIAEnemy|IsPawnDead(Message) (Pawn|GetControlledPawn) :!label _label_2))
                        (if (not _return_5)
                          (Variables|Default|SetActorSeen (Variables|Default|GetC_UpdatedActor))
                          (Variables|Default|SetC_SucessfullySensed (Utilities|Struct|BreakAIStimulus (Variables|Default|GetC_Stimulus)))
                          (bind _actorseen (Variables|Default|GetActorSeen)
                            (:then
                              (bind _return_6 (Class|BPIMasterIAEnemy|CanAlertOtherEntities(Message) _actorseen))
                              (if _return_6
                                (Utilities|ShouldUpdateEnemyActor (Variables|Default|GetActorSeen) (Variables|Default|GetC_SucessfullySensed))
                                (Utilities|SawEnemy (Variables|Default|GetActorSeen) (Variables|Default|GetC_SucessfullySensed)
                                  (:true
                                    ;[0 0 0] He saw an enemy
                                    (bind _actorseen_2 (Variables|Default|GetActorSeen)
                                      (:then
                                        (bind _return_7 (Class|BPIMasterIAEnemy|IsPawnDead(Message) _actorseen_2))
                                        (if (not _return_7)
                                          (Utilities|FlowControl|Sequence
                                            (:then_0
                                              (if (and (Utilities|Enum|NotEqual(Enum) _returnvalue_9 (Utilities|Enum|LiteralenumE_ChaseStatus "NewEnumerator1")) (Utilities|Enum|NotEqual(Enum) _returnvalue_9 (Utilities|Enum|LiteralenumE_ChaseStatus "NewEnumerator3")))
                                                (AI|Components|Blackboard|SetValueasEnum (AI|GetBlackboard 0) (Utilities|Name|MakeLiteralName "State") (Utilities|Select :Index (Variables|Default|GetAICombatStyle) :NewEnumerator0 _returnvalue_6 :NewEnumerator1 _returnvalue_5 :NewEnumerator2 _returnvalue_6 :NewEnumerator3 _returnvalue_6 :NewEnumerator4 (Utilities|Enum|LiteralenumE_ChaseStatus "NewEnumerator4") :NewEnumerator5 _returnvalue_5))
                                                (Class|BPIMasterIAEnemy|BPICustomSawEnemy(Message) (Pawn|GetControlledPawn))))
                                            (:then_1
                                              (Utilities|IsValid _returnvalue_8
                                                (:Is%20Valid
                                                  (AI|Components|Blackboard|SetValueasBool (AI|GetBlackboard 0) (Utilities|Name|MakeLiteralName "EnemyIsInMeleeRange") (<= (Transformation|GetDistanceTo (Pawn|GetControlledPawn) (Variables|Default|GetActorSeen)) (.Value (Utilities|Map|Find (Variables|/Game/ResidentHorrorFPS/Blueprints/BP_MasterAI/IA/Blueprint/BP/BPC_Combat.BPC_Combat_C|GetCharacterStats _returnvalue_8) "Melee"))))))))))
                                      (:else)))
                                  (:false
                                    ;[0 0 0 0.5] Force Remove Enemy
                                    (bind _actorseen_3 (Variables|Default|GetActorSeen)
                                      (:then
                                        (if (== _actorseen_3 (Game|Player|GetPlayerPawn 0))
                                          (Variables|Default|GetCurrent_EnemyActor
                                            (:then)
                                            (:else
                                              (CallFunction|ForceRemoveEnemy)))))
                                      (:else)))
                                  (:LostSightOfEnemy
                                    (CallFunction|EnemyForgetTimer)
                                    (AI|Components|Blackboard|SetValueasEnum (AI|GetBlackboard 0) (Utilities|Name|MakeLiteralName "NonCombateSyle"))))))
                            (:else)))))
                    (else
                      (goto _label_2))))))))))
    (elif (== Actor (Variables|Default|GetCurrent_EnemyActor))
      (bind _return_8 (Class|BPIMasterIAEnemy|BPICanForgetAboutEnemy(Message) (Pawn|GetControlledPawn)))
      (if _return_8
        (goto _label)))))

(event Custom|ForceTargetPerception
  (params (ActorToBePerceived :type Actor%20Object%20Reference))
  (bind _returnvalue (AI|GetBlackboard 0))
  (bind _returnvalue_2 (Utilities|Name|MakeLiteralName "State"))
  (bind _returnvalue_3 (Pawn|GetControlledPawn))
  (bind _returnvalue_4 (Utilities|Enum|LiteralenumE_ChaseStatus "NewEnumerator3"))
  (bind _returnvalue_5 (Utilities|Enum|LiteralenumE_ChaseStatus "NewEnumerator1"))
  (bind _returnvalue_6 (Class|BlackboardComponent|GetValueasEnum _returnvalue _returnvalue_2))
  (bind _returnvalue_7 (Actor|GetComponentbyClass _returnvalue_3 "/Game/ResidentHorrorFPS/Blueprints/BP_MasterAI/IA/Blueprint/BP/BPC_Combat.BPC_Combat_C"))
  (bind _returnvalue_8 (Utilities|Enum|ByteToEnumE_ChaseStatus _returnvalue_6))
  ;[0 0 0 0.5] ForceTargetPerception
  (bind _return (Class|BPIMasterIAEnemy|IsPawnDead(Message) (Pawn|GetControlledPawn)))
  (if (not _return)
    (Utilities|IsValid ActorToBePerceived
      (:Is%20Valid
        (Utilities|IsValid (AI|GetBlackboard 0) :!label _label
          (:Is%20Valid
            (Utilities|IsValid (Actor|GetComponentbyClass ActorToBePerceived "/Game/ResidentHorrorFPS/Blueprints/BP_MasterAI/IA/Blueprint/BP/BPC_Combat.BPC_Combat_C")
              (:Is%20Valid
                (if (not (|VerificationStateIA))
                  (Variables|Default|SetActorSeen ActorToBePerceived)
                  (Variables|Default|SetC_SucessfullySensed true)
                  (bind _return_2 (Class|BPIMasterIAEnemy|CanAlertOtherEntities(Message) (stale OnTargetPerceptionUpdated(AIPerception) _actorseen)))
                  (if _return_2
                    (Utilities|ShouldUpdateEnemyActor (Variables|Default|GetActorSeen) (Variables|Default|GetC_SucessfullySensed))
                    (Utilities|SawEnemy (Variables|Default|GetActorSeen) (Variables|Default|GetC_SucessfullySensed)
                      (:true
                        ;[0 0 0] He saw an enemy
                        (bind _actorseen (Variables|Default|GetActorSeen)
                          (:then
                            (bind _return_3 (Class|BPIMasterIAEnemy|IsPawnDead(Message) _actorseen))
                            (if (not _return_3)
                              (Utilities|FlowControl|Sequence
                                (:then_0
                                  (if (and (Utilities|Enum|NotEqual(Enum) _returnvalue_8 (Utilities|Enum|LiteralenumE_ChaseStatus "NewEnumerator1")) (Utilities|Enum|NotEqual(Enum) _returnvalue_8 (Utilities|Enum|LiteralenumE_ChaseStatus "NewEnumerator3")))
                                    (AI|Components|Blackboard|SetValueasEnum (AI|GetBlackboard 0) (Utilities|Name|MakeLiteralName "State") (Utilities|Select :Index (Variables|Default|GetAICombatStyle) :NewEnumerator0 _returnvalue_5 :NewEnumerator1 _returnvalue_4 :NewEnumerator2 _returnvalue_5 :NewEnumerator3 _returnvalue_5 :NewEnumerator4 (Utilities|Enum|LiteralenumE_ChaseStatus "NewEnumerator4") :NewEnumerator5 _returnvalue_4))
                                    (Class|BPIMasterIAEnemy|BPICustomSawEnemy(Message) (Pawn|GetControlledPawn))))
                                (:then_1
                                  (Utilities|IsValid _returnvalue_7
                                    (:Is%20Valid
                                      (AI|Components|Blackboard|SetValueasBool (AI|GetBlackboard 0) (Utilities|Name|MakeLiteralName "EnemyIsInMeleeRange") (<= (Transformation|GetDistanceTo (Pawn|GetControlledPawn) (Variables|Default|GetActorSeen)) (.Value (Utilities|Map|Find (Variables|/Game/ResidentHorrorFPS/Blueprints/BP_MasterAI/IA/Blueprint/BP/BPC_Combat.BPC_Combat_C|GetCharacterStats _returnvalue_7) "Melee"))))))))))
                          (:else)))
                      (:false
                        ;[0 0 0 0.5] Force Remove Enemy
                        (bind _actorseen_2 (Variables|Default|GetActorSeen)
                          (:then
                            (if (== _actorseen_2 (Game|Player|GetPlayerPawn 0))
                              (Variables|Default|GetCurrent_EnemyActor
                                (:then)
                                (:else
                                  (CallFunction|ForceRemoveEnemy)))))
                          (:else)))
                      (:LostSightOfEnemy
                        (CallFunction|EnemyForgetTimer)
                        (AI|Components|Blackboard|SetValueasEnum (AI|GetBlackboard 0) (Utilities|Name|MakeLiteralName "NonCombateSyle")))))))))
          (:Is%20Not%20Valid
            (Utilities|FlowControl|Delay 0.2)
            (goto _label)))))))

(event Custom|ForceRemoveEnemy
  (bind _returnvalue (AI|GetBlackboard 0))
  ;[0 0 0] Force Remove Enemy BB
  (Utilities|IsValid _returnvalue
    (:Is%20Valid
      (AI|Components|Blackboard|SetValueasBool _returnvalue (Utilities|Name|MakeLiteralName "CanSeeEnemy") false)
      (AI|Components|Blackboard|SetValueasEnum _returnvalue (Utilities|Name|MakeLiteralName "State") (Utilities|Enum|LiteralenumE_ChaseStatus "NewEnumerator0")))))

(event Custom|ChangeEnemyActor_C
  (params (NewEnemy :type Actor%20Object%20Reference) (Owner :type Actor%20Object%20Reference))
  ;[0 0 0] Force Change Enemy Actor
  (Variables|Default|SetCurrent_EnemyActor NewEnemy)
  (Utilities|FlowControl|Delay 0.6)
  (CallFunction|CheckMeleeRange Owner (Variables|Default|GetCurrent_EnemyActor))
  (AI|SetFocus (Variables|Default|GetCurrent_EnemyActor)))

(event Custom|Enemy%20forget%20timer
  (bind _returnvalue (Pawn|GetControlledPawn))
  ;[0 0 0 0.5] Unreal's AI perception system delegate "on perception forgotten" is not being called due to a bug, so this is a solution to fix that unreal bug.
  (bind _actorseen (Variables|Default|GetActorSeen)
    (:then
      (Utilities|FlowControl|RetriggerableDelay 5.0)
      (Utilities|IsValid (Actor|GetComponentbyClass _actorseen "/Game/ResidentHorrorFPS/Blueprints/BP_MasterAI/IA/Blueprint/BP/BPC_Combat.BPC_Combat_C")
        (:Is%20Valid
          (if (not (Variables|Default|GetC_SucessfullySensed))
            (Utilities|IsValid _returnvalue
              (:Is%20Valid
                (Utilities|Array|RemoveItem (Variables|/Game/ResidentHorrorFPS/Blueprints/BP_MasterAI/IA/Blueprint/BP/BPC_Combat.BPC_Combat_C|GetActorsAfterMe (Actor|GetComponentbyClass _actorseen "/Game/ResidentHorrorFPS/Blueprints/BP_MasterAI/IA/Blueprint/BP/BPC_Combat.BPC_Combat_C")) _returnvalue)
                (CallFunction|ForceRemoveEnemy)))))))
    (:else)))

(event EventBeginPlay
  ;[0 0 0] Begin Play
  (Utilities|FlowControl|Delay 0.5)
  (AI|RunBehaviorTree "/Game/ResidentHorrorFPS/Blueprints/BP_MasterAI/IA/BT_AIMaster.BT_AIMaster")
  (Utilities|IsValid (AI|GetBlackboard 0) :!label _label
    (:Is%20Valid
      (bind _ai (Class|BPIIA|GetAISettings(Message) (Pawn|GetControlledPawn)))
      (AI|Components|Blackboard|SetValueasEnum (AI|GetBlackboard 0) (Utilities|Name|MakeLiteralName "NonCombateSyle") (Utilities|Enum|ByteToEnumE_NonCombatType (.InitialCombatIA (Utilities|Struct|BreakST_AISettings _ai))))
      (Class|BlackboardComponent|SetValueasName (AI|GetBlackboard 0) (Utilities|Name|MakeLiteralName "Name") (Utilities|String|StringToName (Utilities|GetDisplayName (Pawn|GetControlledPawn))))
      (bind _return (Class|BPIMasterIAEnemy|BPIGetCreatureName(Message) (Pawn|GetControlledPawn)))
      (Variables|Default|SetMyCreatureName _return))
    (:Is%20Not%20Valid
      (Utilities|FlowControl|Delay 0.1)
      (goto _label))))

(event EventBPIForceTargetPerception
  (params (Actor :type Actor%20Object%20Reference))
  ;[0 0 0 0.5] Target Perception Enemy
  (CallFunction|ForceTargetPerception Actor)
  (CallFunction|EnemyForgetTimer))

(event EventSetEnemyActor
  (params (Actor :type Actor%20Object%20Reference))
  ;[0 0 0 0.5] Set Enemy Actor
  (Variables|Default|SetCurrent_EnemyActor Actor))

(event EventBPIForceRemoveEnemy
  ;[0 0 0] Remove Enemy Force
  (CallFunction|ForceRemoveEnemy))

(fn ConstructionScript)

(fn CheckMeleeRange
  (params (Owner :type Actor%20Object%20Reference) (OtherActor :type Actor%20Object%20Reference))
  (bind _returnvalue (Actor|GetComponentbyClass OtherActor "/Game/ResidentHorrorFPS/Blueprints/BP_MasterAI/IA/Blueprint/BP/BPC_Combat.BPC_Combat_C"))
  (Utilities|IsValid OtherActor
    (:Is%20Valid
      (Utilities|IsValid _returnvalue
        (:Is%20Valid
          (AI|Components|Blackboard|SetValueasBool (AI|GetBlackboard 0) (Utilities|Name|MakeLiteralName "EnemyIsInMeleeRange") (<= (Math|Vector|Distance(Vector) (Transformation|GetWorldLocation (Variables|/Script/Engine.Actor|GetRootComponent Owner)) (Transformation|GetWorldLocation (Variables|/Script/Engine.Actor|GetRootComponent OtherActor))) (.Value (Utilities|Map|Find (Variables|/Game/ResidentHorrorFPS/Blueprints/BP_MasterAI/IA/Blueprint/BP/BPC_Combat.BPC_Combat_C|GetCharacterStats _returnvalue) "Melee"))))
          (return))
        (:Is%20Not%20Valid
          _)))
    (:Is%20Not%20Valid
      _))
  (return))

(fn GetEnemyActor
  (bind _current_enemyactor (Variables|Default|GetCurrent_EnemyActor))
  (return (Utilities|IsValid _current_enemyactor) _current_enemyactor))