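; BP_DamageCauser is a box volume, labelled as a debug damage causer, that sends damage to overlapping actors implementing BPI_MasterIAEnemy.
; Each actor takes damage on entry via BPIDamageMessage and is tracked in an array until it leaves.
; With DanoContinuo on, a looping one-second timer re-damages tracked actors and clears when the array empties.
; The construction script sizes the box and places a text label above it showing the damage mode.
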(event OnComponentBeginOverlap(Box)
  (params (OverlappedComponent :type Primitive%20Component%20Object%20Reference) (OtherActor :type Actor%20Object%20Reference) (OtherComp :type Primitive%20Component%20Object%20Reference) (OtherBodyIndex :type Integer) (bFromSweep :type Boolean) (SweepResult :type Hit%20Result%20Structure%20%28by%20ref%29))
  ;[0.15 0.15 0.15 0.5] Damage Causer Debug Overlap
  (if (Utilities|DoesObjectImplementInterface OtherActor "/Game/ResidentHorrorFPS/Blueprints/BP_MasterAI/IA/Blueprint/Interfaces/BPI_MasterIAEnemy.BPI_MasterIAEnemy_C")
    (if (not (Utilities|Array|ContainsItem (Variables|Default|GetActorsBeingDamage) OtherActor))
      (Class|BPIMasterIAEnemy|BPIDamage(Message) :self OtherActor :DamageCauser self :Base%20Damage (Variables|Default|GetDamage))
      (Utilities|Array|Add (Variables|Default|GetActorsBeingDamage) OtherActor)
      (if (Variables|Default|GetDano%20Continuo)
        (bind _returnvalue (Utilities|Time|SetTimerbyEvent (delegate Custom|OnTick) 1.0 true))
        (Variables|Default|SetTimerHandle _returnvalue)))))

(event OnComponentEndOverlap(Box)
  (params (OverlappedComponent :type Primitive%20Component%20Object%20Reference) (OtherActor :type Actor%20Object%20Reference) (OtherComp :type Primitive%20Component%20Object%20Reference) (OtherBodyIndex :type Integer))
  (bind _actorsbeingdamage (Variables|Default|GetActorsBeingDamage))
  ;[0.15 0.15 0.15 0.5] Damage Causer Debug end Overlap
  (if (Utilities|Array|ContainsItem _actorsbeingdamage OtherActor)
    (Utilities|Array|RemoveItem _actorsbeingdamage OtherActor)
    (if (Variables|Default|GetDano%20Continuo)
      (if (Utilities|Array|IsEmpty (Variables|Default|GetActorsBeingDamage))
        (Utilities|Time|ClearandInvalidateTimerbyHandle (Variables|Default|GetTimerHandle))))))

(event Custom|OnTick
  ;[0.15 0.15 0.15 0.5] Damage Causer Debug Overlap
  (for _array_element (Variables|Default|GetActorsBeingDamage)
    (Class|BPIMasterIAEnemy|BPIDamage(Message) :self _array_element :DamageCauser self :Base%20Damage (Variables|Default|GetDamage))))

(fn ConstructionScript
  (bind _in_box_extent (Variables|Default|GetIn%20Box%20Extent))
  (bind _textrender (Variables|Default|GetTextRender))
  (bind _relativelocation (Variables|/Script/Engine.SceneComponent|GetRelativeLocation _textrender))
  (Rendering|Components|TextRender|SetText (Variables|Default|GetTextRender) (Utilities|Text|FormatText (select (Variables|Default|GetDano%20Continuo) "Dano Continuo" "Dano único")))
  (Components|Box|SetBoxExtent (Variables|Default|GetBox) _in_box_extent true)
  (Transformation|SetRelativeLocation _textrender (Math|Vector|MakeVector (.x _relativelocation) (.y _relativelocation) (+ (.Z (Math|Vector|BreakVector _in_box_extent)) 25.0)) false false))