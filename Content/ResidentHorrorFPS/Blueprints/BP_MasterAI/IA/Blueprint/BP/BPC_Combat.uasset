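; BPC_Combat is a combat component for the master AI that tracks temporarily blocked attacks by tag and provides a random ID helper.
; CheckBlockTags starts a looping timer, if none is active, that counts down each entry in the BlockedAttacksTags map and removes expired ones.
; The timer clears itself once the map is empty.
; GenerateGUID builds a random string from an alphabet array rather than creating a true GUID.
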(event Custom|CustomEvent
  (bind _blockedattackstags (Variables|Default|GetBlockedAttacksTags))
  (bind _blockedattackstags_2 (Variables|Default|GetBlockedAttacksTags))
  ;[0.15 0.15 0.15 0.5] CheckBlockTags
  (if (Utilities|Map|IsNotEmpty _blockedattackstags)
    (bind _keys (Utilities|Map|Keys _blockedattackstags))
    (for _array_element _keys
      (if (<= (.Value (Utilities|Map|Find _blockedattackstags _array_element)) 0.0)
        (Utilities|Map|Remove _blockedattackstags_2 _array_element)
        (else
          (Utilities|Map|Add _blockedattackstags_2 _array_element (- (.Value (Utilities|Map|Find _blockedattackstags _array_element)) 0.1)))))
    (else
      (Utilities|Time|ClearandInvalidateTimerbyHandle (Variables|Default|GetCheckBlockTagsHandle)))))

(event Custom|CheckBlockTags
  ;[0.15 0.15 0.15 0.5] CheckBlockTags
  (if (not (Utilities|Time|IsTimerActivebyHandle (Variables|Default|GetCheckBlockTagsHandle)))
    (bind _returnvalue (Utilities|Time|SetTimerbyEvent (delegate Custom|CustomEvent) 0.1 true))
    (Variables|Default|SetCheckBlockTagsHandle _returnvalue)))

(fn GenerateGUID
  (for _index (range 1 20)
    (LocalVariables|SetOutString (Utilities|String|Append (LocalVariables|GetOutString) (Utilities|Array|Get(acopy) (LocalVariables|GetAlphabet) (Math|Random|RandomInteger 34)))))
  (return (LocalVariables|GetOutString)))