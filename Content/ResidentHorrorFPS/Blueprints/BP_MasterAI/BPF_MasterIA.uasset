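; BPF_MasterIA is a helper for the master AI that decides whether one creature should attack another.
; Its relationship check scans the rows of the DT_CreaturesRelationship data table for entries whose Me field matches the given creature name.
; It sets ShouldAttack and stops searching once a matching row lists the other creature in EnemyCreatures, keeping hostility rules data-driven.
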(fn BPFCheckCreatureRelationship
  (params (MyCreatureName :type E_CreatureNames%20Enum :default "NewEnumerator0") (CreatureToCheck :type E_CreatureNames%20Enum :default "NewEnumerator0"))
  (bind _outrownames (DataTable|GetDataTableRowNames "/Game/ResidentHorrorFPS/Blueprints/BP_MasterAI/DT_CreaturesRelationship.DT_CreaturesRelationship"))
  (bind _array_element (Utilities|Array|ForEachLoopwithBreak _outrownames :!label _label)
    (:LoopBody
      (bind _returnvalue (Utilities|GetDataTableRow "/Game/ResidentHorrorFPS/Blueprints/BP_MasterAI/DT_CreaturesRelationship.DT_CreaturesRelationship" _array_element)
        (:then
          (if (Utilities|Enum|Equal(Enum) (.Me (Utilities|Struct|BreakST_CreaturesRelationship _returnvalue)) MyCreatureName)
            (if (Utilities|Array|ContainsItem (.EnemyCreatures (Utilities|Struct|BreakST_CreaturesRelationship _returnvalue)) CreatureToCheck)
              (LocalVariables|SetbShouldAttack true)
              (goto _label Break))))))
    (:Completed
      (return (LocalVariables|GetbShouldAttack)))))