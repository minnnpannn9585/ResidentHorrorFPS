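; Blueprint function library of player camera helpers for the ResidentHorrorFPS player.
; YawClamp limits the camera manager's view yaw to 90 degrees either side of the player character's current facing, and ResetYaw restores a near-full-circle range.
; GetUIHud is an empty stub with an unconnected HUD lookup.
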(fn YawClamp
  (bind _player (CallFunction|RHVFPSPlayerRef))
  (bind _player_2 (CallFunction|RHVFPSPlayerRef))
  (bind _returnvalue (Game|GetPlayerCameraManager _player))
  (bind _returnvalue_2 (Game|GetPlayerCharacter _player_2))
  (bind _returnvalue_3 (Transformation|GetActorRotation _returnvalue_2))
  (Variables|/Script/Engine.PlayerCameraManager|SetViewYawMin _returnvalue (- (.yaw _returnvalue_3) 9e+01))
  (Variables|/Script/Engine.PlayerCameraManager|SetViewYawMax _returnvalue (+ (.yaw _returnvalue_3) 9e+01)))

(fn ResetYaw
  (bind _returnvalue (Game|GetPlayerCameraManager 0))
  (Variables|/Script/Engine.PlayerCameraManager|SetViewYawMin _returnvalue 0.0)
  (Variables|/Script/Engine.PlayerCameraManager|SetViewYawMax _returnvalue 359.998993))

(fn GetUIHud)